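; BP_Sector is an actor that represents a sector and creates its rooms when play begins.
; GenerateRooms spawns one BP_Room per count of Size and stores each in the Rooms array.
; Every room spawns at the world origin with collision ignored, so no layout is applied.
; SetRandomSize can randomize Size within a small range, but nothing in this Blueprint calls it.
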(event EventBeginPlay
  (CallFunction|GenerateRooms))

(event EventActorBeginOverlap
  (params (OtherActor :type Actor%20Object%20Reference)))

(event EventTick
  (params (DeltaSeconds :type Float%20%28single-precision%29)))

(fn ConstructionScript)

(fn SetRandomSize
  (Variables|Default|SetSize (Math|Random|RandomIntegerinRange 1 5)))

(fn GenerateRooms
  (for _index (range 0 (- (Variables|Default|GetSize) 1))
    (bind _returnvalue (Game|SpawnActorfromClass "/Game/BP_Room.BP_Room_C" (Math|Transform|MakeTransform "0, 0, 0") "AlwaysSpawn" 0 0))
    (Utilities|Array|Add (Variables|Default|GetRooms) _returnvalue)))