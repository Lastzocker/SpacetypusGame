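; Ammo pickup Blueprint that refills the weapons of the BP_BlutenUndLevelnPawn receiving it.
; Its ItemAction override runs the parent action, casts the receiver to that pawn, then adds a fixed amount of ammo to every entry in its Weapons array.
; The HUD ammo readout updates inside the loop as a non-consume event, so it ends on the last weapon's count.
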(event EventBeginPlay)

(event EventActorBeginOverlap
  (params (OtherActor :type Actor%20Object%20Reference))
  (|CallParentFunction 0))

(event EventTick
  (params (DeltaSeconds :type Float%20%28single-precision%29)))

(event EventItemAction
  (params (Receiver :type Actor%20Object%20Reference))
  (|CallParentFunction Receiver)
  (bind _asbp_bluten_und_leveln_pawn (Utilities|Casting|CastToBP_BlutenUndLevelnPawn Receiver))
  (for _array_element (Variables|/Game/BP_BlutenUndLevelnPawn.BP_BlutenUndLevelnPawn_C|GetWeapons _asbp_bluten_und_leveln_pawn)
    (Default|AddAmmo _array_element 20)
    (Default|SetCurrentAmmo (Variables|/Game/BP_BlutenUndLevelnPawn.BP_BlutenUndLevelnPawn_C|GetHUD _asbp_bluten_und_leveln_pawn) (Variables|/Game/BP_Weapon.BP_Weapon_C|GetAmmo _array_element) false)))

(fn ConstructionScript
  (|CallParentFunction))