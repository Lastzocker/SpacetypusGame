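; BP_LevelGenerator is an actor that spawns a set of BP_Sector actors when play begins.
; GenerateSectors spawns Size sectors, all at the world origin, and stores them in Sectors.
; SetRandomSize can roll Size from 1 to 5, but nothing here calls it.
; FillSectorHUD, also uncalled here, creates a SectorButton per sector; its nodes for adding buttons to the HUD are disconnected.
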(event EventBeginPlay
  (CallFunction|GenerateSectors))

(event EventActorBeginOverlap
  (params (OtherActor :type Actor%20Object%20Reference)))

(event EventTick
  (params (DeltaSeconds :type Float%20%28single-precision%29)))

(fn ConstructionScript)

(fn GenerateSectors
  (for _index (range 0 (- (Variables|Default|GetSize) 1))
    (bind _returnvalue (Game|SpawnActorfromClass "/Game/BP_Sector.BP_Sector_C" (Math|Transform|MakeTransform "0, 0, 0") "AlwaysSpawn" 0 0))
    (Utilities|Array|Add (Variables|Default|GetSectors) _returnvalue)))

(fn SetRandomSize
  (Variables|Default|SetSize (Math|Random|RandomIntegerinRange 1 5)))

(fn FillSectorHUD
  (bind _asbp_bluten_und_leveln_pawn (Utilities|Casting|CastToBP_BlutenUndLevelnPawn (Game|Player|GetPlayerPawn 0)))
  (for _array_element (Variables|Default|GetSectors)
    (bind _returnvalue (UserInterface|CreateWidget "/Game/HUD/SectorButton.SectorButton_C"))))