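; BP_Container is a container actor that opens when its Collision component is hit, then fades out and destroys itself.
; On hit, Open switches off that component's physics and collision and prints a debug string, then FinishOpening turns ContainerMesh into a physics-simulated body with the Ragdoll profile.
; A timeline drives the Fade parameter on a dynamic material created at BeginPlay for the mesh's second material slot, destroying the actor when finished.
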(event OnComponentHit(Collision)
  (params (OtherActor :type Actor%20Object%20Reference) (OtherComp :type Primitive%20Component%20Object%20Reference) (NormalImpulse :type Vector :default "0, 0, 0") (Hit :type Hit%20Result%20Structure%20%28by%20ref%29))
  (CallFunction|Open)
  (CallFunction|FinishOpening)
  (bind _newtrack_0 (Timeline|Timeline_0 Play)
    (:Update
      (Rendering|Material|SetScalarParameterValue (Variables|Default|GetMat) "Fade" _newtrack_0 :!class /Script/Engine.MaterialInstanceDynamic))
    (:Finished
      (Actor|DestroyActor))))

(event EventBeginPlay
  (bind _returnvalue (Rendering|Material|CreateDynamicMaterialInstance (Variables|Default|GetContainerMesh) 1 "/Game/Materials/INST_Container.INST_Container" :!class /Script/Engine.PrimitiveComponent))
  (Variables|Default|SetMat _returnvalue))

(event EventActorBeginOverlap
  (params (OtherActor :type Actor%20Object%20Reference)))

(event EventTick
  (params (DeltaSeconds :type Float%20%28single-precision%29)))

(fn ConstructionScript)

(fn Open
  (bind _collision (Variables|Default|GetCollision))
  (Development|PrintString "Hello")
  (Physics|SetSimulatePhysics _collision false)
  (Collision|SetCollisionProfileName _collision "NoCollision" :!class /Script/Engine.PrimitiveComponent))

(fn FinishOpening
  (bind _containermesh (Variables|Default|GetContainerMesh))
  (Collision|IgnoreActorwhenMoving _containermesh self true)
  (Collision|SetCollisionProfileName _containermesh "Ragdoll" :!class /Script/Engine.PrimitiveComponent)
  (Physics|SetSimulatePhysics _containermesh true))