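; Player controller for the Bluten und Leveln pawn that turns player input into pawn actions.
; Movement and turn axes, plus fire, alt-fire and find-target presses, cast the controlled pawn to BP_BlutenUndLevelnPawn and call its matching function.
; The Interact press instead calls CallInteractionKey on the controller itself, without touching the pawn.
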(event Input|ActionEvents|InputActionFire
  (params (Key :type Key%20Structure :default "AnyKey"))
  (:Pressed
    (bind _asbp_bluten_und_leveln_pawn (Utilities|Casting|CastToBP_BlutenUndLevelnPawn (Pawn|GetControlledPawn)))
    (Class|BlutenUndLevelnPawn|FireShot _asbp_bluten_und_leveln_pawn)))

(event Input|ActionEvents|InputActionFindTarget
  (params (Key :type Key%20Structure :default "AnyKey"))
  (:Pressed
    (bind _asbp_bluten_und_leveln_pawn (Utilities|Casting|CastToBP_BlutenUndLevelnPawn (Pawn|GetControlledPawn)))
    (Class|BlutenUndLevelnPawn|FindTarget _asbp_bluten_und_leveln_pawn)))

(event Input|ActionEvents|InputActionAltFire
  (params (Key :type Key%20Structure :default "AnyKey"))
  (:Pressed
    (bind _asbp_bluten_und_leveln_pawn (Utilities|Casting|CastToBP_BlutenUndLevelnPawn (Pawn|GetControlledPawn)))
    (Default|AltFire _asbp_bluten_und_leveln_pawn)))

(event Input|ActionEvents|InputActionInteract
  (params (Key :type Key%20Structure :default "AnyKey"))
  (:Pressed
    (Default|CallInteractionKey)))

(event Input|AxisEvents|InputAxisMoveForward
  (params (AxisValue :type Float%20%28single-precision%29))
  (bind _asbp_bluten_und_leveln_pawn (Utilities|Casting|CastToBP_BlutenUndLevelnPawn (Pawn|GetControlledPawn)))
  (Class|BlutenUndLevelnPawn|MoveForward _asbp_bluten_und_leveln_pawn AxisValue))

(event Input|AxisEvents|InputAxisMoveRight
  (params (AxisValue :type Float%20%28single-precision%29))
  (bind _asbp_bluten_und_leveln_pawn (Utilities|Casting|CastToBP_BlutenUndLevelnPawn (Pawn|GetControlledPawn)))
  (Class|BlutenUndLevelnPawn|MoveRight _asbp_bluten_und_leveln_pawn AxisValue))

(event Input|AxisEvents|InputAxisTurn
  (params (AxisValue :type Float%20%28single-precision%29))
  (bind _asbp_bluten_und_leveln_pawn (Utilities|Casting|CastToBP_BlutenUndLevelnPawn (Pawn|GetControlledPawn)))
  (Class|BlutenUndLevelnPawn|Turn _asbp_bluten_und_leveln_pawn AxisValue))

(fn ConstructionScript)