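; BP_Weapon is a weapon actor that fires projectiles at the cost of the owning pawn's energy.
; OwningActor falls back to the first player pawn on BeginPlay if unset.
; Fire checks readiness and BP_BlutenUndLevelnPawn energy, deducts the cost, spawns and launches the projectile, and attaches a muzzle flash at the spawn component.
; A one-shot timer enforces the cooldown, with CoolDownFinished re-enabling firing.
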(event EventBeginPlay
  (if (== (Variables|Default|GetOwningActor) 0)
    (Variables|Default|SetOwningActor (Game|Player|GetPlayerPawn 0))))

(event EventActorBeginOverlap
  (params (OtherActor :type Actor%20Object%20Reference)))

(event EventTick
  (params (DeltaSeconds :type Float%20%28single-precision%29)))

(fn ConstructionScript)

(fn Fire
  (params (Velocity :type Vector))
  (bind _shootingenergycost (Variables|Default|GetShootingEnergyCost))
  (bind _projectilespawnlocation (Variables|Default|GetProjectileSpawnLocation))
  (bind _returnvalue (Transformation|GetWorldTransform _projectilespawnlocation))
  (if (Variables|Default|GetCanFire)
    (bind _asbp_bluten_und_leveln_pawn (Utilities|Casting|CastToBP_BlutenUndLevelnPawn (Variables|Default|GetOwningActor)))
    (if (>= (Variables|/Game/BP_BlutenUndLevelnPawn.BP_BlutenUndLevelnPawn_C|GetEnergy _asbp_bluten_und_leveln_pawn) _shootingenergycost)
      (Default|ChangeEnergy _asbp_bluten_und_leveln_pawn (* _shootingenergycost -1.0))
      (Variables|Default|SetCanFire false)
      (Utilities|Time|SetTimerbyEvent (EventDispatchers|CreateEvent :!event CoolDownFinished) (Variables|Default|GetCoolDown))
      (bind _returnvalue_2 (Game|SpawnActorfromClass (Variables|Default|GetProjectile) _returnvalue "Undefined" 0 0))
      (Default|Launch _returnvalue_2 Velocity)
      (Effects|SpawnEmitterAttached "/Game/Effects/Projectiles/FX_MuzzleFlash_Chemical.FX_MuzzleFlash_Chemical" _projectilespawnlocation "None" "0, 0, 0" (.Rotation (Math|Transform|BreakTransform _returnvalue)) "SnapToTarget" false))))

(fn CoolDownFinished
  (Variables|Default|SetCanFire true))