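; Destructible wreck of a destroyed object that drifts, spins and then breaks apart, driven by ConfigData.
; BeginPlay applies the set Velocity and a random Z spin, then spawns an optional immediate BP_Explosion effect.
; Tick damps linear velocity by VelocityDecayFactor.
; After the configured lifetime, radius damage at a randomly offset origin fractures the Destructible and a main BP_Explosion spawns, inheriting its velocity.
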(event EventBeginPlay
  (bind _destructible (Variables|Default|GetDestructible))
  (Physics|SetPhysicsLinearVelocity _destructible (Variables|Default|GetVelocity) false "None")
  (Class|PrimitiveComponent|SetPhysicsAngularVelocity _destructible (Math|Vector|MakeVector 0.0 0.0 (Math|Random|RandomFloatinRange -2e+01 2e+01)) false "None")
  (CallFunction|SpawnImmediateEffect)
  (Utilities|FlowControl|Delay (.Lifetime (Utilities|Struct|BreakSTRUCT_DestructionConfig (Variables|Default|GetConfigData))))
  (CallFunction|DestroyObject))

(event EventActorBeginOverlap
  (params (OtherActor :type Actor%20Object%20Reference)))

(event EventTick
  (params (DeltaSeconds :type Float%20%28single-precision%29))
  (bind _destructible (Variables|Default|GetDestructible))
  (bind _returnvalue (Transformation|GetComponentVelocity _destructible))
  (Physics|SetPhysicsLinearVelocity (Variables|Default|GetDestructible) (- _returnvalue (* _returnvalue (Variables|Default|GetVelocityDecayFactor))) false "None"))

(fn ConstructionScript)

(fn SpawnMainEffect
  (bind _configdata (Variables|Default|GetConfigData))
  (bind (_maineffectemitter _maineffectsound _maineffectintensity) (Utilities|Struct|BreakSTRUCT_DestructionConfig _configdata))
  (Game|SpawnActorfromClass "/Game/Blueprint/BP_Explosion.BP_Explosion_C" (Transformation|GetWorldTransform (Variables|Default|GetDestructible)) "Undefined" 0 true 0.01 (Transformation|GetComponentVelocity (Variables|Default|GetDestructible)) _maineffectemitter _maineffectsound _maineffectintensity))

(fn DestroyObject
  (bind _destructible (Variables|Default|GetDestructible))
  (Class|DestructibleComponent|ApplyRadiusDamage _destructible 1e+02 (+ (Transformation|GetWorldLocation _destructible) (* (Math|Random|RandomUnitVector) 2e+01)) 2e+02 1.5e+02 false)
  (CallFunction|SpawnMainEffect))

(fn SpawnImmediateEffect
  (bind _configdata (Variables|Default|GetConfigData))
  (bind (_maineffectemitter _maineffectsound _maineffectintensity _immediateeffectemitter _immediateeffectsound _immediateeffectintensity) (Utilities|Struct|BreakSTRUCT_DestructionConfig _configdata))
  (Utilities|IsValid _immediateeffectemitter
    (:Is%20Valid
      (Game|SpawnActorfromClass "/Game/Blueprint/BP_Explosion.BP_Explosion_C" (Transformation|GetWorldTransform (Variables|Default|GetDestructible)) "Undefined" 0 true 0.01 (Transformation|GetComponentVelocity (Variables|Default|GetDestructible)) _immediateeffectemitter _immediateeffectsound _immediateeffectintensity))))