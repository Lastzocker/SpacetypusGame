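; Behavior tree task that steers a BP_BlutenUndLevelnPawn one step toward the TargetVector blackboard location and fires its weapon.
; Each execution turns by the sign of the yaw difference (modulo 180), then tests the controller's forward and right axes.
; CheckDirection picks the sign that shortens target distance and line-traces for obstacles, allowing movement only on clear axes.
; It finishes immediately, failing only when a cast fails.
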(event EventReceiveExecute
  (params (OwnerActor :type Actor%20Object%20Reference))
  (if (!= (Variables|Default|GetAIControllerRef) 0)
    (bind _asbp_bluten_und_leveln_pawn (Utilities|Casting|CastToBP_BlutenUndLevelnPawn (Pawn|GetControlledPawn (stale _output_get)) :!label _label)
      (:then
        (Class|BlutenUndLevelnPawn|Turn _asbp_bluten_und_leveln_pawn (* (Math|Float|Sign(Float) (- (Math|Float|%(Float) (.yaw (Transformation|GetActorRotation (Pawn|GetControlledPawn (stale _output_get)))) 1.8e+02) (Math|Float|%(Float) (.yaw (Math|Rotator|FindLookatRotation (Transformation|GetActorLocation (Pawn|GetControlledPawn (stale _output_get))) (Class|BTFunctionLibrary|GetBlackboardValueasVector (Variables|Default|GetTargetVector)))) 1.8e+02))) -1.0))
        (bind (_returnvalue _directionisfree) (CallFunction|CheckDirection (Transformation|GetActorForwardVector (Variables|Default|GetAIControllerRef))))
        (if _directionisfree
          (Class|BlutenUndLevelnPawn|MoveForward _asbp_bluten_und_leveln_pawn _returnvalue))
        (bind (_returnvalue_2 _directionisfree_2) (CallFunction|CheckDirection (Transformation|GetActorRightVector (Variables|Default|GetAIControllerRef))))
        (if _directionisfree_2
          (Class|BlutenUndLevelnPawn|MoveRight _asbp_bluten_und_leveln_pawn _returnvalue_2))
        (Default|FireWeapon _asbp_bluten_und_leveln_pawn 1)
        (AI|BehaviorTree|FinishExecute true))
      (:CastFailed
        (AI|BehaviorTree|FinishExecute false :!label _label_2)))
    (else
      (bind _asbp_aicontroller_simple (Utilities|Casting|CastToBP_AIController_Simple OwnerActor)
        (:then
          (bind _output_get (Variables|Default|SetAIControllerRef _asbp_aicontroller_simple))
          (goto _label))
        (:CastFailed
          (goto _label_2))))))

(fn CheckDirection
  (params (Direction :type Vector))
  (bind _targetvector (Variables|Default|GetTargetVector))
  (bind _aicontrollerref (Variables|Default|GetAIControllerRef))
  (bind _returnvalue (Pawn|GetControlledPawn _aicontrollerref))
  (bind _returnvalue_2 (Class|BTFunctionLibrary|GetBlackboardValueasVector _targetvector))
  (bind _returnvalue_3 (Transformation|GetActorLocation _returnvalue))
  (bind _returnvalue_4 (- _returnvalue_2 _returnvalue_3))
  (bind _returnvalue_5 (+ _returnvalue_3 Direction))
  (bind _returnvalue_6 (Math|Vector|VectorLength _returnvalue_4))
  (bind _returnvalue_7 (- _returnvalue_2 _returnvalue_5))
  (bind _returnvalue_8 (Math|Vector|VectorLength _returnvalue_7))
  (bind _returnvalue_9 (- _returnvalue_6 _returnvalue_8))
  (bind _returnvalue_10 (Math|Float|Sign(Float) _returnvalue_9))
  ;[1 1 1] Check if going in the chosen direction is safe
  (bind _returnvalue_11 (Collision|LineTraceForObjects _returnvalue_3 (+ _returnvalue_3 (* (* Direction _returnvalue_10) (Variables|Default|GetTraceLength))) (Utilities|Array|MakeArray "ObjectTypeQuery4" "ObjectTypeQuery1") false 0 "None"))
  (return _returnvalue_10 (not _returnvalue_11)))