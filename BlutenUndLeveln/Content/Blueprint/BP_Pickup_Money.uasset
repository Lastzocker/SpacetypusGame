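; Money pickup that adds a random cash amount to the player's balance through BP_GameInstance when its inherited ItemAction fires.
; On BeginPlay it rolls the Amount and creates a dynamic material whose Color parameter is driven by that value.
; Larger amounts swap the item mesh to one of two higher-tier gradient cash meshes, so the pickup's look reflects its worth.
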(event EventBeginPlay
  (bind _returnvalue (Math|Random|RandomIntegerinRange 50 400))
  (bind _itemmesh (Variables|Default|GetItemMesh))
  (|CallParentFunction)
  (bind _returnvalue_2 (Rendering|Material|CreateDynamicMaterialInstance (Variables|Default|GetItemMesh) 0 (Rendering|Material|GetMaterial (Variables|Default|GetItemMesh) 0) :!class /Script/Engine.PrimitiveComponent))
  (Variables|Default|SetCashMaterial _returnvalue_2)
  (bind _output_get (Variables|Default|SetAmount (- _returnvalue (Math|Integer|%(Integer) _returnvalue 20))))
  (Rendering|Material|SetVectorParameterValue (Variables|Default|GetCashMaterial) "Color" (Utilities|Struct|MakeLinearColor 1.0 1e+01 (/ (Math|Conversions|ToFloat(Integer) _output_get) 1e+01) 1.0) :!class /Script/Engine.MaterialInstanceDynamic)
  (if (> (Variables|Default|GetAmount) 100)
    (if (> (Variables|Default|GetAmount) 200)
      (Components|StaticMesh|SetStaticMesh _itemmesh "/Game/Meshes/Items/MESH_ItemCash_V3Gradient.MESH_ItemCash_V3Gradient")
      (else
        (Components|StaticMesh|SetStaticMesh _itemmesh "/Game/Meshes/Items/MESH_ItemCash_V2Gradient.MESH_ItemCash_V2Gradient")))))

(event EventActorBeginOverlap
  (params (OtherActor :type Actor%20Object%20Reference)))

(event EventTick
  (params (DeltaSeconds :type Float%20%28single-precision%29))
  (|CallParentFunction 0.0))

(event EventItemAction
  (params (Receiver :type BP%20Bluten%20Und%20Leveln%20Pawn%20Object%20Reference))
  (|CallParentFunction Receiver)
  (bind _asbp_game_instance (Utilities|Casting|CastToBP_GameInstance (Game|GetGameInstance)))
  (Default|AddMoney _asbp_game_instance (Variables|Default|GetAmount)))

(fn ConstructionScript
  (|CallParentFunction))