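; Player ship AI that comments on gameplay through comm-link messages in the gameplay HUD.
; Initialize stores the player and HUD, then binds to the room manager's start and completion events and the pawn's critical hull event.
; Each event, delayed for room events, picks a collection by room type or state from a data table and queues it on the HUD, usually choosing a random line.
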(event Custom|BindAIEvents
  ;[1 1 1] Bind AI Events
  (Utilities|FlowControl|Sequence
    (:then_0
      ;[1 1 1] Room manager
      (Utilities|IsValid (Variables|/Game/Blueprint/BP_BuLPlayerController.BP_BuLPlayerController_C|GetRoomManager (Variables|Default|GetPlayer))
        (:Is%20Valid
          (Utilities|FlowControl|Sequence
            (:then_0
              ;[1 1 1] Room completed event
              (EventDispatchers|BindEventtoRoomCompleted (Variables|/Game/Blueprint/BP_BuLPlayerController.BP_BuLPlayerController_C|GetRoomManager (Variables|Default|GetPlayer)) (delegate Custom|OnRoomCompleted)))
            (:then_1
              ;[1 1 1] Room started event
              (EventDispatchers|BindEventtoRoomStarted (Variables|/Game/Blueprint/BP_BuLPlayerController.BP_BuLPlayerController_C|GetRoomManager (Variables|Default|GetPlayer)) (delegate Custom|OnRoomStarted)))))))
    (:then_1
      (Utilities|FlowControl|Sequence
        (:then_0
          ;[1 1 1] Hull Integrity changed event
          (EventDispatchers|BindEventtoCriticalHullIntegrity (Variables|/Game/Blueprint/BP_BuLPlayerController.BP_BuLPlayerController_C|GetPlayerPawn (Variables|Default|GetPlayer)) (delegate Custom|OnCriticalHullIntegrity)))))))

(event Custom|OnRoomCompleted
  ;[1 1 1] Room completed event
  (Utilities|FlowControl|Delay 2.0)
  (CallFunction|INFORoomCompleted))

(event Custom|OnRoomStarted
  (params (HasBeenCompleted :type Boolean) (RoomType :type ENUM_RoomTypes%20Enum))
  ;[1 1 1] Room started event
  (Utilities|FlowControl|Delay 1.0)
  (CallFunction|INFORoomStart HasBeenCompleted RoomType))

(event Custom|OnCriticalHullIntegrity
  ;[1 1 1] Hull Integrity changed event
  (CallFunction|INFOHullCritical))

(event EventBeginPlay
  (bind _asbp_game_instance (Utilities|Casting|CastToBP_GameInstance (Game|GetGameInstance)))
  (Variables|Default|SetGameInstance _asbp_game_instance))

(event EventTick
  (params (DeltaSeconds :type Float%20%28single-precision%29)))

(fn MessagetoPlayer
  (params (Collection :type Name) (PickRandom :type Boolean))
  (bind _returnvalue (Utilities|GetDataTableRow "/Game/DataTables/DATA_CommLinkMessageCollections.DATA_CommLinkMessageCollections" Collection)
    (:then
      (Default|AddPendingMessageCollection (Variables|Default|GetGameplayHUD) PickRandom _returnvalue))
    (:RowNotFound
      (Development|PrintText "Ship AI: Collection not found"))))

(fn AddPointer)

(fn INFORoomStart
  (params (HasBeenCompleted :type Boolean) (RoomType :type ENUM_RoomTypes%20Enum))
  (CallFunction|MessagetoPlayer "OnRoomEntry" true)
  (if HasBeenCompleted
    (CallFunction|MessagetoPlayer "OnRoomStart_Completed" true)
    (else
      (switch Utilities|FlowControl|Switch|SwitchonENUM_RoomTypes RoomType
        (:NewEnumerator0
          (CallFunction|MessagetoPlayer "OnRoomStart_Empty" true))
        (:NewEnumerator1
          (CallFunction|MessagetoPlayer "OnRoomStart_Battle" true))))))

(fn INFORoomCompleted
  (switch Utilities|FlowControl|Switch|SwitchonENUM_RoomTypes (.RoomType (Utilities|Struct|BreakSTRUCT_RoomData (Variables|/Game/Blueprint/LevelGeneration/BP_RoomManager.BP_RoomManager_C|GetRoomData (Variables|/Game/Blueprint/BP_BuLPlayerController.BP_BuLPlayerController_C|GetRoomManager (Variables|Default|GetPlayer)))))
    (:NewEnumerator1
      (CallFunction|MessagetoPlayer "OnRoomCompleted_Battle" true))))

(fn Initialize
  (params (Player :type BP%20Bu%20L%20Player%20Controller%20Object%20Reference) (GameplayHUD :type HUD%20Gameplay%20Object%20Reference))
  (Variables|Default|SetPlayer Player)
  (Variables|Default|SetGameplayHUD GameplayHUD)
  (CallFunction|BindAIEvents))

(fn INFOHullCritical
  (CallFunction|MessagetoPlayer "OnHullCritical" true))