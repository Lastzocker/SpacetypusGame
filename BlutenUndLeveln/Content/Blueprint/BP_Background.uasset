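; BP_Background is a backdrop actor with a nebula projection plane that follows the player camera's world position.
; BeginPlay waits briefly, caches the camera of the BP_BlutenUndLevelnPawn player pawn, then opens a gate.
; Tick feeds that gate, moving the actor to the camera's location every frame without changing its rotation.
; The construction script sets the plane's visibility from the ShowNebula flag.
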(event EventBeginPlay
  (Utilities|FlowControl|Delay 0.05)
  (bind _asbp_bluten_und_leveln_pawn (Utilities|Casting|CastToBP_BlutenUndLevelnPawn (Game|Player|GetPlayerPawn 0)))
  (Variables|Default|SetTargetCamera (Variables|/Game/Blueprint/BP_BlutenUndLevelnPawn.BP_BlutenUndLevelnPawn_C|GetCamera _asbp_bluten_und_leveln_pawn))
  (Utilities|FlowControl|Gate true) ; enters at Open
)

(event EventActorBeginOverlap
  (params (OtherActor :type Actor%20Object%20Reference)))

(event EventTick
  (params (DeltaSeconds :type Float%20%28single-precision%29))
  (Utilities|FlowControl|Gate true
    (:Exit
      (Transformation|SetActorLocation (Transformation|GetWorldLocation (Variables|Default|GetTargetCamera)) false false))))

(fn ConstructionScript
  (Rendering|SetVisibility (Variables|Default|GetNebulaProjectionPlane) (Variables|Default|GetShowNebula) false))