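; BP_Container is a one-time lootable container that the player opens with the interaction key when within InteractionRadius.
; Opening stops it blocking Pawns, spawns drops through the game mode's DropHandler, and turns the mesh into a ragdoll-profile physics body.
; A timeline then fades the container and scaffolding dynamic materials before destroying the actor.
; OnDetect and OnLostContact animate its marker widget in and out, starting hidden.
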(event Custom|UsedContainer
  (if (<= (Math|Vector|VectorLength (- (Transformation|GetActorLocation) (Transformation|GetActorLocation (Game|Player|GetPlayerPawn 0)))) (Variables|Default|GetInteractionRadius))
    (Utilities|FlowControl|DoOnce false
      (:Completed
        (CallFunction|Open)
        (CallFunction|FinishOpening)
        (bind _newtrack_0 (Timeline|Timeline_0 Play)
          (:Update
            (Rendering|Material|SetScalarParameterValue (Variables|Default|GetContainerMat) "Fade" _newtrack_0 :!class /Script/Engine.MaterialInstanceDynamic))
          (:Finished
            (Actor|DestroyActor)))))))

(event EventBeginPlay
  (bind _containermesh (Variables|Default|GetContainerMesh))
  (bind _returnvalue (Rendering|Material|CreateDynamicMaterialInstance _containermesh 1 "/Game/Materials/INST_Container.INST_Container" :!class /Script/Engine.PrimitiveComponent))
  (Variables|Default|SetContainerMat _returnvalue)
  (bind _returnvalue_2 (Rendering|Material|CreateDynamicMaterialInstance _containermesh 0 "/Game/Materials/INST_Scaffolding_Container.INST_Scaffolding_Container" :!class /Script/Engine.PrimitiveComponent))
  (Variables|Default|SetScaffoldingMat _returnvalue_2)
  (bind _asbp_bu_lplayer_controller (Utilities|Casting|CastToBP_BuLPlayerController (Game|GetPlayerController 0)))
  (EventDispatchers|BindEventtoInteractionKey _asbp_bu_lplayer_controller (delegate Custom|UsedContainer))
  (bind _ashud_container_marker (Utilities|Casting|CastToHUD_ContainerMarker (UserInterface|GetUserWidgetObject (Variables|Default|GetMarkerWidget))))
  (bind _output_get (Variables|Default|SetMarker _ashud_container_marker))
  (Default|PlayHideAnim _output_get))

(event EventTick
  (params (DeltaSeconds :type Float%20%28single-precision%29)))

(event EventOnDetect
  (Default|PlayShowAnim (Variables|Default|GetMarker)))

(event EventOnLostContact
  (Default|PlayHideAnim (Variables|Default|GetMarker)))

(fn ConstructionScript)

(fn Open
  (Collision|SetCollisionResponsetoChannel (Variables|Default|GetCollision) "ECC_Pawn" "ECR_Ignore")
  (bind _asbp_bu_lgame_mode (Utilities|Casting|CastToBP_BuLGameMode (Game|GetGameMode)))
  (Default|SpawnDrop (Variables|/Game/Blueprint/BP_BuLGameMode.BP_BuLGameMode_C|GetDropHandler _asbp_bu_lgame_mode) (Transformation|GetActorLocation) 4))

(fn FinishOpening
  (bind _containermesh (Variables|Default|GetContainerMesh))
  (Collision|IgnoreActorwhenMoving _containermesh self true)
  (Collision|SetCollisionProfileName _containermesh "Ragdoll" :!class /Script/Engine.PrimitiveComponent)
  (Physics|SetSimulatePhysics _containermesh true))