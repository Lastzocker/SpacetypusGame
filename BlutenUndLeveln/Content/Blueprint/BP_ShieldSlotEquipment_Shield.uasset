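; Player ship shield equipment that, while held active, drains energy, grants the owner damage immunities and absorbs hits into an integrity pool, with a plasma damage factor.
; SetWorking toggles damageability, overlaps and immunities, driving timelines that fade and flicker a dynamic sphere material scaled by remaining integrity.
; Tick recharges integrity while the shield is down and reports it to the player controller.
; Breaking or energy depletion disables the shield until integrity or energy recovers.
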(event Custom|GetHit
  (bind _shieldmat (Variables|Default|GetShieldMat))
  (bind _opacity (Timeline|ShieldHitTimeline PlayFromStart)
    (:Update
      (bind (_opacitymodifier _noisemodifier) (CallFunction|GetStability))
      (Rendering|Material|SetScalarParameterValue _shieldmat "TotalOpacity" (+ (* _opacity 15.0) _opacitymodifier) :!class /Script/Engine.MaterialInstanceDynamic)
      (Rendering|Material|SetScalarParameterValue _shieldmat "ShieldNoiseMultiplier" (+ (* _opacity 3e+01) _noisemodifier) :!class /Script/Engine.MaterialInstanceDynamic))))

(event Custom|Activate
  (bind _shieldmat (Variables|Default|GetShieldMat))
  (Effects|SpawnEmitterAttached "/Game/Effects/Special/FX_PlayerShield_Activate.FX_PlayerShield_Activate" (Variables|Default|GetSphere) "None" "0, 0, 0" "0, 0, 0" "SnapToTarget")
  (Rendering|SetVisibility (Variables|Default|GetSphere) true false)
  (bind (_direction _opacity _noise) (Timeline|Timeline_0 Play)
    (:Update
      (bind (_opacitymodifier _noisemodifier) (CallFunction|GetStability))
      (Rendering|Material|SetScalarParameterValue _shieldmat "TotalOpacity" (* _opacity _opacitymodifier) :!class /Script/Engine.MaterialInstanceDynamic)
      (Rendering|Material|SetScalarParameterValue _shieldmat "ShieldNoiseMultiplier" (+ (* 3e+02 _noise) _noisemodifier) :!class /Script/Engine.MaterialInstanceDynamic))
    (:Finished
      (switch Utilities|FlowControl|Switch|SwitchonETimelineDirection _direction
        (:Backward
          (Rendering|SetVisibility (Variables|Default|GetSphere) false false))))))

(event Custom|Deactivate
  (bind _shieldmat (Variables|Default|GetShieldMat))
  (if (Variables|Default|GetIsFunctional)
    (Effects|SpawnEmitterAttached "/Game/Effects/Special/FX_PlayerShield_Deactivate.FX_PlayerShield_Deactivate" (Variables|Default|GetSphere) "None" "0, 0, 0" "0, 0, 0" "SnapToTarget")
    (bind (_direction _opacity _noise) (Timeline|Timeline_0 Reverse)
      (:Update
        (bind (_opacitymodifier _noisemodifier) (CallFunction|GetStability))
        (Rendering|Material|SetScalarParameterValue _shieldmat "TotalOpacity" (* _opacity _opacitymodifier) :!class /Script/Engine.MaterialInstanceDynamic)
        (Rendering|Material|SetScalarParameterValue _shieldmat "ShieldNoiseMultiplier" (+ (* 3e+02 _noise) _noisemodifier) :!class /Script/Engine.MaterialInstanceDynamic))
      (:Finished
        (switch Utilities|FlowControl|Switch|SwitchonETimelineDirection _direction
          (:Backward
            (Rendering|SetVisibility (Variables|Default|GetSphere) false false)))))))

(event Custom|Collapse
  (bind _shieldmat (Variables|Default|GetShieldMat))
  (bind (_direction _opacity _noise) (Timeline|Timeline_0 Reverse)
    (:Update
      (bind (_opacitymodifier _noisemodifier) (CallFunction|GetStability))
      (Rendering|Material|SetScalarParameterValue _shieldmat "TotalOpacity" (* _opacity _opacitymodifier) :!class /Script/Engine.MaterialInstanceDynamic)
      (Rendering|Material|SetScalarParameterValue _shieldmat "ShieldNoiseMultiplier" (+ (* 3e+02 _noise) _noisemodifier) :!class /Script/Engine.MaterialInstanceDynamic))
    (:Finished
      (switch Utilities|FlowControl|Switch|SwitchonETimelineDirection _direction
        (:Backward
          (Rendering|SetVisibility (Variables|Default|GetSphere) false false))))))

(event EventBeginPlay
  (|CallParentFunction))

(event EventTick
  (params (DeltaSeconds :type Float%20%28single-precision%29))
  (bind _maxintegrity (Variables|Default|GetMaxIntegrity))
  (bind _maxintegrity_2 (Variables|Default|GetMaxIntegrity))
  (bind _isactive (Variables|Default|GetIsActive))
  (bind _owningactor (Variables|Default|GetOwningActor))
  (bind _owningactor_2 (Variables|Default|GetOwningActor))
  ;[1 1 1] Tick
  (if (and (Variables|Default|GetIsActive) (Variables|Default|GetIsFunctional))
    (if (not (Variables|/Game/Blueprint/BP_BlutenUndLevelnPawn.BP_BlutenUndLevelnPawn_C|GetHasInfiniteAmmoAndEnergy (Variables|Default|GetOwningActor)))
      (bind _successful (Default|ChangeEnergy (Variables|Default|GetOwningActor) (* (Variables|Default|GetEnergyConsumption) DeltaSeconds -1.0)))
      (if _successful
        (Utilities|FlowControl|DoOnce true :!label _label
          (:Completed
            (CallFunction|SetWorking true)))
        (else
          ;;[1 1 1] Too little energy
          (Variables|Default|SetIsFunctional false)
          (CallFunction|SetWorking false)
          (CallFunction|Collapse)
          (Variables|Default|SetShieldDownFromEnergyLoss true)
          (goto _label Reset))))
    (elif (Variables|Default|GetShieldDownFromEnergyLoss)
      (if (> (/ (Variables|/Game/Blueprint/BP_BlutenUndLevelnPawn.BP_BlutenUndLevelnPawn_C|GetEnergy _owningactor_2) (Variables|/Game/Blueprint/BP_BlutenUndLevelnPawn.BP_BlutenUndLevelnPawn_C|GetMaxEnergy _owningactor_2)) (Variables|Default|GetMinEnergy))
        (Variables|Default|SetIsFunctional true)
        (Default|CallShieldRestored _owningactor)
        (if _isactive
          (Variables|Default|SetShieldDownFromEnergyLoss false)))
      (elif (< (Variables|Default|GetIntegrity) _maxintegrity_2)
        (Variables|Default|SetIntegrity (Math|Float|Min(Float) (Math|Interpolation|FInterptoConstant (Variables|Default|GetIntegrity) _maxintegrity_2 DeltaSeconds (Variables|Default|GetIntegrityInterpSpeed)) (Variables|Default|GetMaxIntegrity)))
        (bind _asbp_bu_lplayer_controller (Utilities|Casting|CastToBP_BuLPlayerController (Pawn|GetController (Variables|Default|GetOwningActor))))
        (Default|SetShieldIntegrity _asbp_bu_lplayer_controller false (/ (Variables|Default|GetIntegrity) _maxintegrity) (Variables|Default|GetIntegrity) _maxintegrity)
        (else
          (Utilities|FlowControl|DoOnce true
            (:Completed
              (Variables|Default|SetIsFunctional true)
              (Default|CallShieldRestored _owningactor)
              (if _isactive
                (CallFunction|SetWorking true)))))))))

(event EventInitialize
  (params (ShipInfo :type STRUCT%20Ship%20Config%20Structure))
  (bind (_shieldmesh _shieldcolor _shieldintegrity _shieldchargerate) (Utilities|Struct|BreakSTRUCT_ShipConfig ShipInfo))
  (bind _sphere (Variables|Default|GetSphere))
  (|CallParentFunction ShipInfo)
  (bind _output_get (Variables|Default|SetMaxIntegrity _shieldintegrity))
  (Variables|Default|SetIntegrity _output_get)
  (Variables|Default|SetIntegrityInterpSpeed _shieldchargerate)
  (Components|StaticMesh|SetStaticMesh (Variables|Default|GetSphere) _shieldmesh)
  (bind _returnvalue (Rendering|Material|CreateDynamicMaterialInstance _sphere 0 (Rendering|Material|GetMaterial _sphere 0) :!class /Script/Engine.PrimitiveComponent))
  (bind _output_get_2 (Variables|Default|SetShieldMat _returnvalue))
  (Rendering|Material|SetVectorParameterValue _output_get_2 "TintColor" _shieldcolor :!class /Script/Engine.MaterialInstanceDynamic)
  (CallFunction|SetWorking false))

(event Game|Damage|EventAnyDamage
  (params (Damage :type Float%20%28single-precision%29) (DamageType :type Damage%20Type%20Object%20Reference) (InstigatedBy :type Controller%20Object%20Reference) (DamageCauser :type Actor%20Object%20Reference))
  (CallFunction|GetHit)
  (bind _zerointegrity (CallFunction|HandleDamage Damage DamageType))
  (if _zerointegrity
    (Variables|Default|SetIsFunctional false)
    (CallFunction|SetWorking false)
    (Development|PrintString "Shield broke")
    (CallFunction|Collapse)
    (Default|CallShieldOverload (Variables|Default|GetOwningActor))
    (Utilities|FlowControl|DoOnce true) ; enters at Reset
  ))

(event EventUse
  ;[1 1 1] Use
  (Variables|Default|SetIsActive true)
  (if (Variables|Default|GetIsFunctional)
    (CallFunction|SetWorking true)))

(event EventRelease
  (bind _owningactor (Variables|Default|GetOwningActor))
  ;[1 1 1] Release
  (Variables|Default|SetIsActive false)
  (if (> (/ (Variables|/Game/Blueprint/BP_BlutenUndLevelnPawn.BP_BlutenUndLevelnPawn_C|GetEnergy _owningactor) (Variables|/Game/Blueprint/BP_BlutenUndLevelnPawn.BP_BlutenUndLevelnPawn_C|GetMaxEnergy _owningactor)) (Variables|Default|GetMinEnergy)) ; Making sure the player can't restart the shield as long as it's under the minimum
    (CallFunction|SetWorking false)
    (else
      ;[1 1 1] Tick
      ;;[1 1 1] Too little energy
      (Variables|Default|SetIsFunctional false)
      (CallFunction|SetWorking false)
      (CallFunction|Collapse)
      (Variables|Default|SetShieldDownFromEnergyLoss true)
      (Utilities|FlowControl|DoOnce true) ; enters at Reset
    )))

(fn ConstructionScript
  (|CallParentFunction))

(fn SetWorking
  (params (IsWorking :type Boolean))
  (bind _owningactor (Variables|Default|GetOwningActor))
  (Utilities|IsValid _owningactor
    (:Is%20Valid
      (|Handleimmunities _owningactor (not IsWorking)))
    (:Is%20Not%20Valid
      _))
  (Variables|Default|SetbCanBeDamaged IsWorking)
  (Variables|/Script/Engine.PrimitiveComponent|SetbGenerateOverlapEvents (Variables|Default|GetSphere) IsWorking)
  (if IsWorking
    (CallFunction|Activate)
    (else
      (CallFunction|Deactivate))))

(fn GetStability
  (bind _integrity (Variables|Default|GetIntegrity))
  (bind _maxintegrity (Variables|Default|GetMaxIntegrity))
  (bind _defaultmaxnoise (Variables|Config|GetDefaultMaxNoise))
  (bind _returnvalue (/ _integrity _maxintegrity))
  (return (Math|Float|Clamp(Float) _returnvalue (Variables|Config|GetDefaultMinOpacity) (Variables|Config|GetDefaultMaxOpacity)) (Math|Float|Clamp(Float) (* (- 1.0 _returnvalue) _defaultmaxnoise) (Variables|Config|GetDefaultMinNoise) _defaultmaxnoise)))

(fn HandleDamage
  (params (Damage :type Float%20%28single-precision%29) (DamageType :type Damage%20Type%20Object%20Reference))
  (bind _maxintegrity (Variables|Default|GetMaxIntegrity))
  (LocalVariables|SetPreviousIntegrity (Variables|Default|GetIntegrity))
  (Utilities|Casting|CastToBP_DamageType_Plasma DamageType
    (:then
      (Variables|Default|SetIntegrity (Math|Float|Max(Float) (- (Variables|Default|GetIntegrity) (* (Variables|Default|GetPlasmaFactor) Damage)) 0.0)))
    (:CastFailed
      (bind _output_get (Variables|Default|SetIntegrity (Math|Float|Max(Float) (- (Variables|Default|GetIntegrity) Damage) 0.0)))))
  (bind _asbp_bu_lplayer_controller (Utilities|Casting|CastToBP_BuLPlayerController (Pawn|GetController (Variables|Default|GetOwningActor)))
    (:then
      (Default|SetShieldIntegrity _asbp_bu_lplayer_controller true (/ (Variables|Default|GetIntegrity) _maxintegrity) (Variables|Default|GetIntegrity) _maxintegrity)
      (Default|UpdateDamageStats _asbp_bu_lplayer_controller (- (LocalVariables|GetPreviousIntegrity) (Variables|Default|GetIntegrity)) true))
    (:CastFailed
      _))
  (return (<= _output_get 0.0)))