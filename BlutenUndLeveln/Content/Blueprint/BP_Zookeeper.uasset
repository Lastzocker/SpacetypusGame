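; BP_Zookeeper tracks the pawns in a room and triggers the room-cleared response when only one remains.
; Shortly after BeginPlay, it counts every BP_BlutenUndLevelnPawn and binds to each one's destruction, decrementing the count per death.
; At one left, it calls Unlock on the first BP_Beacon and plays the HUD's room-cleared sequence.
; The PlayerShip filter is unconnected, so matching pawns stay counted.
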(event Custom|PawnDestroyed
  (bind _output_get (Variables|Default|SetEnemyCount (- (Variables|Default|GetEnemyCount) 1)))
  (if (== _output_get 1)
    (bind _outactors (Actor|GetAllActorsOfClass "/Game/Blueprint/LevelElements/BP_Beacon.BP_Beacon_C"))
    (Default|Unlock (Utilities|Array|Get(acopy) _outactors) false)
    (bind _asbp_bu_lplayer_controller (Utilities|Casting|CastToBP_BuLPlayerController (Game|GetPlayerController 0)))
    (Default|RoomClearedSequence (Variables|/Game/Blueprint/BP_C_PlayerHUD.BP_C_PlayerHUD_C|GetHUD_Main (Variables|/Game/Blueprint/BP_BuLPlayerController.BP_BuLPlayerController_C|GetBP_C_PlayerHUD _asbp_bu_lplayer_controller)))))

(event EventBeginPlay
  (Utilities|FlowControl|Delay 0.2)
  (bind _outactors (Actor|GetAllActorsOfClass "/Game/Blueprint/BP_BlutenUndLevelnPawn.BP_BlutenUndLevelnPawn_C"))
  (for _array_element _outactors
    (EventDispatchers|BindEventtoDestruction _array_element (delegate Custom|PawnDestroyed)))
  (Variables|Default|SetEnemyCount (Utilities|Array|Length _outactors)))

(event EventActorBeginOverlap
  (params (OtherActor :type Actor%20Object%20Reference)))

(event EventTick
  (params (DeltaSeconds :type Float%20%28single-precision%29)))

(fn ConstructionScript)