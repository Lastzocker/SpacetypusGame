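; Player HUD component that builds the gameplay HUD and tracks off-screen targets with direction markers.
; After a startup delay it creates the main screen widget and spawns a ship HUD actor attached to the pawn, hosting reticle, vitals and decorator.
; Each tick, registered targets outside the viewport get markers projected to an inset screen border and rotated toward them; invalid targets are pruned.
; It can also hide all gameplay elements.
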(event EventBeginPlay
  (Components|Tick|SetComponentTickEnabled false)
  (Utilities|FlowControl|Delay 1.0)
  (CallFunction|Initialize)
  (Utilities|FlowControl|Delay 1.0)
  (Default|SetDisplayStatus (Variables|/Game/Blueprint/BP_PlayerShipHUD.BP_PlayerShipHUD_C|GetReticle (Variables|Default|GetShipHUDActor)) true))

(event EventTick
  (params (DeltaSeconds :type Float%20%28single-precision%29))
  (CallFunction|HandleTargets))

(fn Initialize
  (bind _asbp_bluten_und_leveln_pawn (Utilities|Casting|CastToBP_BlutenUndLevelnPawn (Game|Player|GetPlayerPawn 0)))
  (bind _output_get (Variables|Default|SetPlayerPawn _asbp_bluten_und_leveln_pawn))
  (Utilities|FlowControl|Sequence
    (:then_0
      ;[1 1 1] Initialize Main Group
      (bind _returnvalue (UserInterface|CreateWidget "/Game/HUD/HUD_Gameplay.HUD_Gameplay_C"))
      (bind _output_get_2 (Variables|Default|SetHUD_Main _returnvalue))
      (Default|Initialize _output_get_2 _output_get)
      (UserInterface|Viewport|AddtoViewport _returnvalue 0))
    (:then_1
      ;[1 1 1] Intialize Ship Group
      (bind _returnvalue_2 (Game|SpawnActorfromClass "/Game/Blueprint/BP_PlayerShipHUD.BP_PlayerShipHUD_C" (Transformation|GetActorTransform (Variables|Default|GetPlayerPawn)) "Undefined" 0 0))
      (Class|Actor|AttachRootComponenttoActor _returnvalue_2 (Variables|Default|GetPlayerPawn) "None" "SnapToTarget" true)
      (Variables|Default|SetShipHUDActor _returnvalue_2)
      (Utilities|FlowControl|Sequence
        (:then_0
          (Transformation|AddLocalOffset (Variables|/Game/Blueprint/BP_PlayerShipHUD.BP_PlayerShipHUD_C|GetReticleWidget _returnvalue_2) (Math|Vector|MakeVector (Variables|Default|GetReticleOffset) 0.0 0.0) false false))
        (:then_1
          (bind _ashud_ship_vitals (Utilities|Casting|CastToHUD_ShipVitals (UserInterface|GetUserWidgetObject (Variables|/Game/Blueprint/BP_PlayerShipHUD.BP_PlayerShipHUD_C|GetVitals _returnvalue_2))))
          (bind _output_get_3 (Variables|Default|SetHUD_Vitals _ashud_ship_vitals))
          (Default|Initialize _output_get_3 (Variables|Default|GetPlayerPawn)))
        (:then_2
          (bind _ashud_center_group_decorator_1 (Utilities|Casting|CastToHUD_CenterGroupDecorator1 (UserInterface|GetUserWidgetObject (Variables|/Game/Blueprint/BP_PlayerShipHUD.BP_PlayerShipHUD_C|GetDecorator1 _returnvalue_2))))
          (Variables|Default|SetHUD_Decorator _ashud_center_group_decorator_1)
          (Default|Initialize _ashud_center_group_decorator_1))))
    (:then_2
      (Components|Tick|SetComponentTickEnabled true))))

(fn AddTarget
  (params (TargetActor :type Actor%20Object%20Reference) (Icon :type Texture%202D%20Object%20Reference) (IsHostile :type Boolean))
  (bind _returnvalue (UserInterface|CreateWidget "/Game/HUD/HUD_DirectionMarker.HUD_DirectionMarker_C" (Game|GetPlayerController 0)))
  (Default|SetIcon _returnvalue Icon)
  (Default|SetHostile _returnvalue IsHostile)
  (Widget|SetVisibility _returnvalue "Collapsed")
  (UserInterface|Viewport|AddtoViewport _returnvalue 0)
  (Utilities|Array|Add (Variables|Default|GetKnownTargets) (Utilities|Struct|MakeSTRUCT_Target TargetActor _returnvalue false))
  (return _returnvalue))

(fn RemoveTarget
  (params (TargetActor :type Actor%20Object%20Reference))
  (bind _knowntargets (Variables|Default|GetKnownTargets))
  (for _array_element _knowntargets
    (if (== TargetActor (.TargetActor (Utilities|Struct|BreakSTRUCT_Target _array_element)))
      (Widget|RemovefromParent (.TargetDirectionMarker (Utilities|Struct|BreakSTRUCT_Target _array_element)))
      (Utilities|Array|RemoveItem _knowntargets _array_element))))

(fn HandleTargets
  (for _array_element (Variables|Default|GetKnownTargets)
    (Utilities|IsValid (.TargetActor (Utilities|Struct|BreakSTRUCT_Target _array_element))
      (:Is%20Valid
        (bind _isonscreen (CallFunction|GetTargetonScreen (.TargetActor (Utilities|Struct|BreakSTRUCT_Target _array_element))))
        (if _isonscreen ; Is target on screen?
          (Widget|SetVisibility (.TargetDirectionMarker (Utilities|Struct|BreakSTRUCT_Target _array_element)) "Collapsed")
          (else
            (CallFunction|SetDirectionMarkerLocRot (.TargetActor (Utilities|Struct|BreakSTRUCT_Target _array_element)) (.TargetDirectionMarker (Utilities|Struct|BreakSTRUCT_Target _array_element)))
            (Widget|SetVisibility (.TargetDirectionMarker (Utilities|Struct|BreakSTRUCT_Target _array_element)) "Visible"))))
      (:Is%20Not%20Valid
        (Utilities|IsValid (.TargetDirectionMarker (Utilities|Struct|BreakSTRUCT_Target _array_element))
          (:Is%20Valid
            (Widget|RemovefromParent (.TargetDirectionMarker (Utilities|Struct|BreakSTRUCT_Target _array_element)))
            (Utilities|Array|RemoveItem (Variables|Default|GetKnownTargets) _array_element)))))))

(fn SetDirectionMarkerLocRot
  (params (TargetActor :type Actor%20Object%20Reference) (DirectionMarker :type HUD%20Direction%20Marker%20Object%20Reference))
  (bind _returnvalue (Viewport|GetViewportSize))
  (bind _returnvalue_2 (/ _returnvalue 2.0))
  (bind _projectedposition (Class|CVectorUtility|ProjecttoScreenBorder (Transformation|GetActorLocation (Variables|Default|GetPlayerPawn)) (Transformation|GetActorLocation TargetActor) (Game|GetPlayerController 0)))
  (Default|SetDirectionPointerRot DirectionMarker (- _projectedposition _returnvalue_2))
  (Class|UserWidget|SetPositioninViewport DirectionMarker (- (+ (* (- _projectedposition _returnvalue_2) 0.95) _returnvalue_2) "(X=32.000000,Y=32.000000)") true))

(fn GetTargetonScreen
  (params (TargetActor :type Actor%20Object%20Reference))
  (bind _returnvalue (Game|GetPlayerController 0))
  (bind _returnvalue_2 (Transformation|GetActorLocation TargetActor))
  (bind _returnvalue_3 (Viewport|GetViewportSize))
  (bind _screenposition (Class|GameplayStatics|ProjectWorldtoScreen _returnvalue _returnvalue_2))
  (return (and (Math|Float|InRange(Float) (.x _screenposition) 0.0 (.x _returnvalue_3)) (Math|Float|InRange(Float) (.y _screenposition) 0.0 (.y _returnvalue_3)))))

(fn DeactivateGameplayElements
  (Default|HideGameplayElements (Variables|Default|GetHUD_Main))
  (Default|Hide (Variables|Default|GetHUD_Vitals))
  (Default|Hide (Variables|Default|GetHUD_Decorator))
  (Default|SetDisplayStatus (Variables|/Game/Blueprint/BP_PlayerShipHUD.BP_PlayerShipHUD_C|GetReticle (Variables|Default|GetShipHUDActor)) false))