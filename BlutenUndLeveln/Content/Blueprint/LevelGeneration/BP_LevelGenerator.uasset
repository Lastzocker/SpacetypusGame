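; BP_LevelGenerator is an actor that builds a sector of rooms at BeginPlay and lists them on a HUD.
; It spawns a BP_Sector with a random room count, fills it with BP_Room actors and makes it current.
; Each room gets a RoomButton holding a generator reference; LoadRoom opens RoomMap regardless of the room passed.
; GenerateRoomData builds beacon position and random size data, but nothing here calls it.
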(event EventBeginPlay
  (CallFunction|GenerateSector)
  (CallFunction|SetStartSector)
  (bind _returnvalue (UserInterface|CreateWidget "/Game/HUD/LevelGeneratorHUD.LevelGeneratorHUD_C" (Game|GetPlayerController 0)))
  (UserInterface|Viewport|AddtoViewport _returnvalue 0)
  (Variables|Default|SetHUD _returnvalue)
  (CallFunction|FillRoomHUD))

(event EventActorBeginOverlap
  (params (OtherActor :type Actor%20Object%20Reference)))

(event EventTick
  (params (DeltaSeconds :type Float%20%28single-precision%29)))

(fn ConstructionScript)

(fn GenerateSector
  ;[1 1 1] Spawns the Actor and adds it to Sectors Array
  (bind _returnvalue (Game|SpawnActorfromClass "/Game/Blueprint/LevelGeneration/BP_Sector.BP_Sector_C" (Math|Transform|MakeTransform "0, 0, 0") "AlwaysSpawn" 0 (Math|Random|RandomIntegerinRange (Variables|Default|GetMinRooms) (Variables|Default|GetMaxRooms)) 0))
  (Utilities|Array|Add (Variables|Default|GetSectors) _returnvalue)
  (CallFunction|GenerateSectorRooms _returnvalue))

(fn FillRoomHUD
  (for _array_element (Variables|/Game/Blueprint/LevelGeneration/BP_Sector.BP_Sector_C|GetRooms (Variables|Default|GetCurrentSector))
    (bind _returnvalue (UserInterface|CreateWidget "/Game/HUD/RoomButton.RoomButton_C" 0 _array_element self))
    (Rendering|Components|TextRender|SetText (Variables|/Game/HUD/RoomButton.RoomButton_C|GetRoomName _returnvalue) (Utilities|Text|ToText(String) (Utilities|GetDisplayName _array_element)))
    (Class|VerticalBox|AddChildtoVerticalBox (Variables|/Game/HUD/LevelGeneratorHUD.LevelGeneratorHUD_C|GetBox (Variables|Default|GetHUD)) _returnvalue)))

(fn SetStartSector
  (Variables|Default|SetCurrentSector (Utilities|Array|Get(acopy) (Variables|Default|GetSectors))))

(fn GenerateSectorRooms
  (params (Sector :type BP%20Sector%20Object%20Reference))
  (for _index (range 0 (- (Variables|/Game/Blueprint/LevelGeneration/BP_Sector.BP_Sector_C|GetSize Sector) 1))
    (bind _returnvalue (Game|SpawnActorfromClass :Class "/Game/Blueprint/LevelGeneration/BP_Room.BP_Room_C" :SpawnTransform (Math|Transform|MakeTransform "0, 0, 0") :CollisionHandlingOverride "Undefined"))
    (Utilities|Array|Add (Variables|/Game/Blueprint/LevelGeneration/BP_Sector.BP_Sector_C|GetRooms Sector) _returnvalue)))

(fn LoadRoom
  (params (Room :type BP%20Room%20Object%20Reference))
  (Game|OpenLevel(byName) "RoomMap"))

(fn GenerateRoomData
  (bind _position (CallFunction|GetBeaconPosition "0, 0, 0"))
  (bind _randomsize (CallFunction|GetRandomSize))
  (return (Utilities|Struct|MakeRoomData "0, 0, 0" _position "0, 0, 0" _randomsize)))

(fn GetBeaconPosition
  (params (CenterPos :type Vector))
  (bind _returnvalue (Math|Random|RandomFloatinRange -5e+01 -5e+01))
  (return (+ CenterPos (Math|Vector|MakeVector _returnvalue _returnvalue _returnvalue))))

(fn GetRandomSize
  (return (Math|Random|RandomIntegerinRange 100 1000)))