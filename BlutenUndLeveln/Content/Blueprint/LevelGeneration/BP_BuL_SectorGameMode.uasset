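; Game mode for sector level generation that makes sure the game instance holds a selected sector.
; On BeginPlay it casts to BP_GameInstance and calls GenerateRandomSector only if that instance is not yet initialized.
; The function stores new sector data with a small random room count in SelectedSector and sets Initialized, so later BeginPlay calls keep the same sector.
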(event EventBeginPlay
  (bind _asbp_game_instance (Utilities|Casting|CastToBP_GameInstance (Game|GetGameInstance)))
  (if (not (Variables|/Game/Blueprint/BP_GameInstance.BP_GameInstance_C|GetInitialized _asbp_game_instance))
    (CallFunction|GenerateRandomSector)))

(event EventTick
  (params (DeltaSeconds :type Float%20%28single-precision%29)))

(fn ConstructionScript)

(fn GenerateRandomSector
  (bind _asbp_game_instance (Utilities|Casting|CastToBP_GameInstance (Game|GetGameInstance))
    (:then
      (Variables|/Game/Blueprint/BP_GameInstance.BP_GameInstance_C|SetSelectedSector _asbp_game_instance (Utilities|Struct|MakeSTRUCT_SectorData (Math|Random|RandomIntegerinRange 1 5) (Utilities|Array|MakeArray "")))
      (Variables|/Game/Blueprint/BP_GameInstance.BP_GameInstance_C|SetInitialized _asbp_game_instance true))
    (:CastFailed
      _))
  (return))