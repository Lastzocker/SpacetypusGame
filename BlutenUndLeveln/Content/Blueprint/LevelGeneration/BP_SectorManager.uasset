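; BP_SectorManager is an actor that shows the rooms of the selected sector and opens the one that is picked.
; On BeginPlay it reads SelectedSector from BP_GameInstance, adds a LevelGeneratorHUD to the viewport and fills it with a numbered RoomButton per room.
; LoadRoom stores the given room as SelectedRoom on the game instance, which carries it across the OpenLevel call to RoomMap.
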(event EventBeginPlay
  (bind _data (CallFunction|GetSector))
  (Variables|Default|SetSectorData _data)
  (bind _returnvalue (UserInterface|CreateWidget "/Game/HUD/LevelGeneratorHUD.LevelGeneratorHUD_C" (Game|GetPlayerController 0)))
  (UserInterface|Viewport|AddtoViewport _returnvalue 0)
  (Variables|Default|SetHUD _returnvalue)
  (CallFunction|FillRoomHUD))

(event EventActorBeginOverlap
  (params (OtherActor :type Actor%20Object%20Reference)))

(event EventTick
  (params (DeltaSeconds :type Float%20%28single-precision%29)))

(fn ConstructionScript)

(fn FillRoomHUD
  (for (_array_element _array_index) (.RoomDatas (Utilities|Struct|BreakSTRUCT_SectorData (Variables|Default|GetSectorData)))
    (bind _returnvalue (UserInterface|CreateWidget "/Game/HUD/RoomButton.RoomButton_C" 0 _array_element self))
    (Rendering|Components|TextRender|SetText (Variables|/Game/HUD/RoomButton.RoomButton_C|GetRoomName _returnvalue) (Utilities|Text|ToText(String) (Utilities|String|MakeLiteralString (Utilities|String|Append (Utilities|String|MakeLiteralString "Room ") (Utilities|String|ToString(Integer) (+ _array_index 1))))))
    (Class|VerticalBox|AddChildtoVerticalBox (Variables|/Game/HUD/LevelGeneratorHUD.LevelGeneratorHUD_C|GetBox (Variables|Default|GetHUD)) _returnvalue)))

(fn LoadRoom
  (params (RoomData :type STRUCT%20Room%20Data%20Structure))
  (bind _asbp_game_instance (Utilities|Casting|CastToBP_GameInstance (Game|GetGameInstance)))
  (Variables|/Game/Blueprint/BP_GameInstance.BP_GameInstance_C|SetSelectedRoom _asbp_game_instance RoomData)
  (Game|OpenLevel(byName) "RoomMap"))

(fn GetSector
  (bind _asbp_game_instance (Utilities|Casting|CastToBP_GameInstance (Game|GetGameInstance))
    (:then
      _)
    (:CastFailed
      _))
  (return (Variables|/Game/Blueprint/BP_GameInstance.BP_GameInstance_C|GetSelectedSector _asbp_game_instance)))

(fn SetSector
  (params (data :type STRUCT%20Sector%20Data%20Structure))
  (bind _asbp_game_instance (Utilities|Casting|CastToBP_GameInstance (Game|GetGameInstance)))
  (Variables|/Game/Blueprint/BP_GameInstance.BP_GameInstance_C|SetSelectedSector _asbp_game_instance data))