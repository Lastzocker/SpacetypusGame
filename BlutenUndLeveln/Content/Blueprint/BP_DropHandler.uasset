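; BP_DropHandler spawns physics-launched money and weapon pickups at a stored location.
; SpawnDrop rolls weapon chance through the game instance's random function until one weapon drops, otherwise spawning money.
; SpawnWeapon computes a weighted pick from DATA_Weapons but never uses it, spawning pickups with row name None.
; Pickups register in RoomManager's room data when it is valid, though BeginPlay sets that reference to None.
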(event EventBeginPlay
  (bind _asbp_bluten_und_leveln_pawn (Utilities|Casting|CastToBP_BlutenUndLevelnPawn (Pawn|GetControlledPawn (Game|GetPlayerController 0))))
  (Variables|Default|SetRoomManager 0))

(event EventActorBeginOverlap
  (params (OtherActor :type Actor%20Object%20Reference)))

(event EventTick
  (params (DeltaSeconds :type Float%20%28single-precision%29)))

(fn ConstructionScript)

(fn SpawnDrop
  (params (Location :type Vector) (Amount :type Integer))
  (bind _returnvalue (Math|Transform|MakeTransform (Math|Vector|MakeVector (.x Location) (.y Location) 0.0)))
  (bind _returnvalue_2 (Math|Random|RandomUnitVector))
  (bind _roommanager (Variables|Default|GetRoomManager))
  (bind _roomdata (Variables|/Game/Blueprint/LevelGeneration/BP_RoomManager.BP_RoomManager_C|GetRoomData _roommanager))
  (bind (_pickups _pickuptransforms) (Utilities|Struct|BreakSTRUCT_RoomData _roomdata))
  (for _index (range 0 Amount)
    (if (LocalVariables|GetDroppedWeapon)
      (bind _returnvalue_3 (Game|SpawnActorfromClass "/Game/Blueprint/PickUps/BP_Pickup_Money.BP_Pickup_Money_C" _returnvalue "AdjustIfPossibleButAlwaysSpawn" 0 -1 (Variables|Default|GetRoomManager) :!label _label))
      (bind _output_get (LocalVariables|SetItem _returnvalue_3))
      (else
        (bind _asbp_game_instance (Utilities|Casting|CastToBP_GameInstance (Game|GetGameInstance))
          (:then
            (bind _randomfloat (Default|GetRandomFloatinRange _asbp_game_instance 0.0 1.0))
            (if (<= _randomfloat (LocalVariables|GetWeaponDropChance))
              (bind (_successful _pickup) (CallFunction|SpawnWeapon _asbp_game_instance _returnvalue))
              (LocalVariables|SetDroppedWeapon _successful)
              (LocalVariables|SetItem _pickup)
              (else
                (goto _label))))
          (:CastFailed
            (goto _label)))))
    (Physics|AddForce (Variables|/Game/Blueprint/PickUps/BP_PickUp.BP_PickUp_C|GetItemMesh _output_get) (* _returnvalue_2 (Math|Random|RandomFloatinRange 2.5e+04 5e+04)) "None" false)
    (Class|PrimitiveComponent|SetPhysicsAngularVelocity (Variables|/Game/Blueprint/PickUps/BP_PickUp.BP_PickUp_C|GetItemMesh _output_get) (* _returnvalue_2 (Math|Random|RandomFloatinRange 1e+02 3e+02)) false "None")
    (Utilities|IsValid _roommanager
      (:Is%20Valid
        (Utilities|Array|Add _pickups (Utilities|GetClass (LocalVariables|GetItem)))
        (bind _returnvalue_4 (Utilities|Array|Add _pickuptransforms (Transformation|GetActorTransform (LocalVariables|GetItem))))
        (Variables|/Game/Blueprint/PickUps/BP_PickUp.BP_PickUp_C|SetIndexInRoom (LocalVariables|GetItem) _returnvalue_4))
      (:Is%20Not%20Valid
        (Development|PrintString "No room manager")))))

(fn SpawnWeapon
  (params (GameInstance :type BP%20Game%20Instance%20Object%20Reference) (Transform :type Transform))
  (bind _outrownames (DataTable|GetDataTableRowNames "/Game/DataTables/DATA_Weapons.DATA_Weapons"))
  (for _array_element _outrownames
    (bind _returnvalue (Utilities|GetDataTableRow "/Game/DataTables/DATA_Weapons.DATA_Weapons" _array_element)
      (:then
        (if (!= (.DropChance (Utilities|Struct|BreakSTRUCT_Weapon _returnvalue)) 0.0)
          (LocalVariables|SetSumChance (+ (LocalVariables|GetSumChance) (.DropChance (Utilities|Struct|BreakSTRUCT_Weapon _returnvalue))))
          (Utilities|Array|Add (LocalVariables|GetChances) (.DropChance (Utilities|Struct|BreakSTRUCT_Weapon _returnvalue)))
          (Utilities|Array|Add (LocalVariables|GetNames) _array_element)))))
  (bind _randomfloat (Default|GetRandomFloatinRange GameInstance 0.0 (LocalVariables|GetSumChance)))
  (LocalVariables|SetRandom _randomfloat)
  (bind (_array_element_2 _array_index) (Utilities|Array|ForEachLoopwithBreak (LocalVariables|GetChances) :!label _label)
    (:LoopBody
      (if (> (LocalVariables|GetAccumulate) (LocalVariables|GetRandom))
        (LocalVariables|SetIndex (- _array_index 1))
        (goto _label Break)
        (else
          (LocalVariables|SetAccumulate (+ _array_element_2 (LocalVariables|GetAccumulate))))))
    (:Completed
      (bind _returnvalue_2 (Game|SpawnActorfromClass "/Game/Blueprint/PickUps/BP_PickUp_Weapon.BP_PickUp_Weapon_C" Transform "AdjustIfPossibleButAlwaysSpawn" 0 "None" -1 (Variables|Default|GetRoomManager)))
      (return true _returnvalue_2))))