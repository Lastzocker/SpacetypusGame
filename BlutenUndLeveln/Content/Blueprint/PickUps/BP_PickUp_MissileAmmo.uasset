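; Missile ammo pickup that refills part of the receiver's missile supply.
; It overrides the parent's ItemAction event, running the parent logic and then adding missiles equal to a RestorePercentage share of the receiver's MaxMissiles, truncated to a whole number.
; All other behavior is left to the parent pickup class.
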(event EventBeginPlay
  (|CallParentFunction))

(event Collision|EventActorBeginOverlap
  (params (OtherActor :type Actor%20Object%20Reference))
  (|CallParentFunction 0))

(event EventTick
  (params (DeltaSeconds :type Float%20%28single-precision%29)))

(event EventItemAction
  (params (Receiver :type BP%20Bluten%20Und%20Leveln%20Pawn%20Object%20Reference))
  (|CallParentFunction Receiver)
  (Default|AddMissiles Receiver (Math|Float|Truncate (* (Variables|/Game/Blueprint/BP_BlutenUndLevelnPawn.BP_BlutenUndLevelnPawn_C|GetMaxMissiles Receiver) (Variables|Default|GetRestorePercentage)))))

(fn ConstructionScript
  (|CallParentFunction))