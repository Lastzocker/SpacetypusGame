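; Repair pickup that restores part of a ship's hull integrity when its item action fires on the receiver.
; ItemAction extends the parent's handler, repairing the receiver by RestorePercentage of its MaxHullIntegrity.
; For receivers controlled by a BP_BuLPlayerController, it then displays the repair effect through that controller and attaches the collect particle effect to the ship mesh.
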(event EventBeginPlay)

(event EventActorBeginOverlap
  (params (OtherActor :type Actor%20Object%20Reference))
  (|CallParentFunction 0))

(event EventTick
  (params (DeltaSeconds :type Float%20%28single-precision%29)))

(event EventItemAction
  (params (Receiver :type BP%20Bluten%20Und%20Leveln%20Pawn%20Object%20Reference))
  (|CallParentFunction Receiver)
  (Default|Repair Receiver (* (Variables|/Script/BlutenUndLeveln.BlutenUndLevelnPawn|GetMaxHullIntegrity Receiver) (Variables|Default|GetRestorePercentage)))
  (bind _asbp_bu_lplayer_controller (Utilities|Casting|CastToBP_BuLPlayerController (Pawn|GetController Receiver)))
  (Default|DisplayRepairEffect _asbp_bu_lplayer_controller)
  (Effects|SpawnEmitterAttached "/Game/Effects/Interaction/FX_PickUp_Repair_Collect.FX_PickUp_Repair_Collect" (Variables|/Script/BlutenUndLeveln.BlutenUndLevelnPawn|GetShipMeshComponent Receiver) "None" "0, 0, 0" "0, 0, 0" "SnapToTarget"))

(fn ConstructionScript
  (|CallParentFunction))