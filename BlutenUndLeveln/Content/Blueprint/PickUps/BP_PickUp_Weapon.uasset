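; Weapon pickup actor that gives the weapon named by WeaponName to the receiver on its item action.
; On BeginPlay it looks up that row in DATA_Weapons, caches the weapon class and fills a HUD_WeaponMarker widget with name and class.
; The item action re-reads the row and sets it on the receiver's WeaponArrays entry indexed by class.
; Show/hide events animate the marker; invalid names print an error.
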(event EventBeginPlay
  (|CallParentFunction)
  (bind _ashud_weapon_marker (Utilities|Casting|CastToHUD_WeaponMarker (UserInterface|GetUserWidgetObject (Variables|Default|GetMarkerWidget))))
  (bind _output_get (Variables|Default|SetMarker _ashud_weapon_marker))
  (Default|PlayHideAnim _output_get)
  (bind _returnvalue (Utilities|GetDataTableRow "/Game/DataTables/DATA_Weapons.DATA_Weapons" (Variables|Default|GetWeaponName))
    (:then
      (Variables|Default|SetWeaponClass (.WeaponClass (Utilities|Struct|BreakSTRUCT_Weapon _returnvalue)))
      (Default|SetWeapon (Variables|Default|GetMarker) (.Name (Utilities|Struct|BreakSTRUCT_Weapon _returnvalue)) (.WeaponClass (Utilities|Struct|BreakSTRUCT_Weapon _returnvalue))))
    (:RowNotFound
      (Development|PrintText "PickUp: Invalid weapon name" true true "(R=1.000000,G=0.024480,B=0.000000,A=1.000000)"))))

(event EventActorBeginOverlap
  (params (OtherActor :type Actor%20Object%20Reference)))

(event EventTick
  (params (DeltaSeconds :type Float%20%28single-precision%29))
  (|CallParentFunction 0.0))

(event EventItemAction
  (params (Receiver :type BP%20Bluten%20Und%20Leveln%20Pawn%20Object%20Reference))
  (|CallParentFunction Receiver)
  (bind _returnvalue (Utilities|GetDataTableRow "/Game/DataTables/DATA_Weapons.DATA_Weapons" (Variables|Default|GetWeaponName))
    (:then
      (Default|SetWeapon (Utilities|Array|Get(acopy) (Variables|/Game/Blueprint/BP_BlutenUndLevelnPawn.BP_BlutenUndLevelnPawn_C|GetWeaponArrays Receiver) (Math|Conversions|ToInteger(Byte) (Variables|Default|GetWeaponClass))) _returnvalue))
    (:RowNotFound
      (Development|PrintText "PickUp: Invalid weapon name" true true "(R=1.000000,G=0.024480,B=0.000000,A=1.000000)"))))

(event EventHideWidget
  (Default|PlayHideAnim (Variables|Default|GetMarker)))

(event EventShowWidget
  (Default|PlayShowAnim (Variables|Default|GetMarker)))

(fn ConstructionScript
  (|CallParentFunction))