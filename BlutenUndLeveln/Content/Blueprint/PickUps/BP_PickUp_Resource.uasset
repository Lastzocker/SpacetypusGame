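; BP_PickUp_Resource is a resource pickup Blueprint that displays an icon marker through a widget component.
; On BeginPlay it runs the parent logic, caches the widget as a HUD_ResourceMarker and assigns its icon texture.
; ShowWidget and HideWidget toggle the marker's visibility after a validity check; the file adds no overlap, tick or collection logic of its own.
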(event EventBeginPlay
  (|CallParentFunction)
  (bind _ashud_resource_marker (Utilities|Casting|CastToHUD_ResourceMarker (UserInterface|GetUserWidgetObject (Variables|Default|GetMarkerWidget))))
  (Variables|Default|SetMarker _ashud_resource_marker)
  (Default|SetIcon (Variables|Default|GetMarker) (Variables|Default|GetIconTexture)))

(event EventActorBeginOverlap
  (params (OtherActor :type Actor%20Object%20Reference)))

(event EventTick
  (params (DeltaSeconds :type Float%20%28single-precision%29))
  (|CallParentFunction 0.0))

(event EventShowWidget
  (bind _marker (Variables|Default|GetMarker))
  (Utilities|IsValid _marker
    (:Is%20Valid
      (Default|SetMarkerVisible _marker true))))

(event EventHideWidget
  (bind _marker (Variables|Default|GetMarker))
  (Utilities|IsValid _marker
    (:Is%20Valid
      (Default|SetMarkerVisible _marker false))))

(fn ConstructionScript
  (|CallParentFunction))