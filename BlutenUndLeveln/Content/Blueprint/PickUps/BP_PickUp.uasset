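; Base pickup actor that the player pawn collects by touching its mesh, with placeholder widget and gain-value functions.
; On overlap it runs ItemAction for sound and particles, removes itself from the RoomManager by index, hides, then destroys itself after a short delay.
; Detectable interface events toggle the marker widget hooks and play a sound, while Tick keeps the detection collision on the randomly rotated mesh.
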(event OnComponentBeginOverlap(ItemMesh)
  (params (OtherActor :type Actor%20Object%20Reference) (OtherComp :type Primitive%20Component%20Object%20Reference) (OtherBodyIndex :type Integer) (bFromSweep :type Boolean) (SweepResult :type Hit%20Result%20Structure%20%28by%20ref%29))
  (bind _returnvalue (Game|GetPlayerController 0))
  (bind _returnvalue_2 (Pawn|GetControlledPawn _returnvalue))
  ;[1 1 1] Collection
  (if (not (Variables|Default|GetIsCollected))
    (if (== _returnvalue_2 OtherActor)
      (bind _asbp_bluten_und_leveln_pawn (Utilities|Casting|CastToBP_BlutenUndLevelnPawn _returnvalue_2))
      (CallFunction|ItemAction _asbp_bluten_und_leveln_pawn)
      (Variables|Default|SetIsCollected true)
      (CallFunction|ItemCollected))))

(event Custom|ItemCollected
  ;[1 1 1] Collected
  (CallFunction|RemovefromRoomList)
  (CallFunction|HideWidget)
  (CallFunction|DisableGraphics)
  (Utilities|FlowControl|Delay 0.5)
  (Actor|DestroyActor))

(event EventOnDetect
  ;[1 1 1] Detectable interface actions
  (CallFunction|ShowWidget)
  (Variables|Default|SetIsDetected true)
  (Audio|PlaySound2D (Variables|Default|GetDetectionSound)))

(event EventOnLostContact
  ;[1 1 1] Detectable interface actions
  (CallFunction|HideWidget)
  (Variables|Default|SetIsDetected false)
  (Audio|PlaySound2D (Variables|Default|GetDetectionSound)))

(event EventBeginPlay
  (Transformation|SetWorldRotation (Variables|Default|GetItemMesh) (Math|Random|RandomRotator true) false false))

(event EventTick
  (params (DeltaSeconds :type Float%20%28single-precision%29))
  ;[1 1 1] Tick
  (Transformation|SetWorldLocation (Variables|Default|GetDetectionCollision) (Transformation|GetWorldLocation (Variables|Default|GetItemMesh)) false false))

(fn ConstructionScript
  (bind _returnvalue (Transformation|GetActorLocation))
  (Transformation|SetActorLocation (Math|Vector|MakeVector (.x _returnvalue) (.y _returnvalue) 0.0) false false))

(fn ItemAction
  (params (Receiver :type BP%20Bluten%20Und%20Leveln%20Pawn%20Object%20Reference))
  (Audio|PlaySoundatLocation (Variables|Default|GetActionSound) (Transformation|GetActorLocation))
  (Effects|SpawnEmitteratLocation (Variables|Default|GetCollectEffect) (Transformation|GetWorldLocation (Variables|Default|GetMarkerWidget)) (Math|Rotator|MakeRotator 0.0 0.0 (Math|Random|RandomFloatinRange 0.0 3.6e+02)))
  (CallFunction|HideWidget))

(fn ShowWidget)

(fn HideWidget)

(fn GetGainValue
  (return 0))

(fn RemovefromRoomList
  (bind _indexinroom (Variables|Default|GetIndexInRoom))
  (if (== _indexinroom -1)
    (Development|PrintString "Could not remove item from room list!")
    (return)
    (else
      (Default|RemovePickUpbyIndex (Variables|Default|GetRoomManager) _indexinroom))))

(fn DisableGraphics
  (Rendering|SetVisibility (Variables|Default|GetItemMesh) false false)
  (Rendering|SetVisibility (Variables|Default|GetAmbientParticles) false false))

(fn EnableGraphics
  (Rendering|SetVisibility (Variables|Default|GetItemMesh) true false)
  (Rendering|SetVisibility (Variables|Default|GetAmbientParticles) true false))