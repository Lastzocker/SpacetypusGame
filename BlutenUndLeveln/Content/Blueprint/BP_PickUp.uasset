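; BP_PickUp is a base pickup actor with an item marker widget and an empty ItemAction hook.
; Detectable interface events show and hide the marker, and Tick keeps the detection collision on the item mesh's location.
; When the player's pawn overlaps the mesh, it calls ItemAction on that pawn, hides marker and mesh, then destroys itself after a short delay.
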(event OnComponentBeginOverlap(ItemMesh)
  (params (OtherActor :type Actor%20Object%20Reference) (OtherComp :type Primitive%20Component%20Object%20Reference) (OtherBodyIndex :type Integer) (bFromSweep :type Boolean) (SweepResult :type Hit%20Result%20Structure%20%28by%20ref%29))
  (bind _returnvalue (Game|GetPlayerController 0))
  (bind _returnvalue_2 (Pawn|GetControlledPawn _returnvalue))
  ;[1 1 1] Collection
  (if (== _returnvalue_2 OtherActor)
    (bind _asbp_bluten_und_leveln_pawn (Utilities|Casting|CastToBP_BlutenUndLevelnPawn _returnvalue_2))
    (CallFunction|ItemAction _asbp_bluten_und_leveln_pawn)
    (CallFunction|HideWidget)
    (Rendering|SetVisibility (Variables|Default|GetItemMesh) false false)
    (Utilities|FlowControl|Delay 0.5)
    (Actor|DestroyActor)))

(event EventOnDetect
  ;[1 1 1] Detectable interface actions
  (CallFunction|ShowWidget))

(event EventOnLostContact
  ;[1 1 1] Detectable interface actions
  (CallFunction|HideWidget))

(event EventBeginPlay
  ;[1 1 1] BeginPlay
  (bind _ashud_item_marker (Utilities|Casting|CastToHUD_ItemMarker (UserInterface|GetUserWidgetObject (Variables|Default|GetMarkerWidget))))
  (bind _output_get (Variables|Default|SetMarker _ashud_item_marker))
  (Default|PlayHideAnim _output_get)
  (Default|SetIcon (Variables|Default|GetMarker) (Variables|Default|GetIconTexture)))

(event EventTick
  (params (DeltaSeconds :type Float%20%28single-precision%29))
  ;[1 1 1] Tick
  (Transformation|SetWorldLocation (Variables|Default|GetDetectionCollision) (Transformation|GetWorldLocation (Variables|Default|GetItemMesh)) false false))

(fn ConstructionScript)

(fn ItemAction
  (params (Receiver :type BP%20Bluten%20Und%20Leveln%20Pawn%20Object%20Reference)))

(fn ShowWidget
  (Default|PlayShowAnim (Variables|Default|GetMarker)))

(fn HideWidget
  (Default|PlayHideAnim (Variables|Default|GetMarker)))