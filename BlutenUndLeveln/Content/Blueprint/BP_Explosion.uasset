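; BP_Explosion is a self-destroying explosion effect actor that plays a particle effect and can drift through the world.
; On BeginPlay it assigns the MainEffect template to its emitter, activates it, and destroys the actor when the particle system finishes.
; Each tick, Move offsets the location by Velocity without sweeping, optionally damping Velocity by a per-frame decay factor that is not scaled by delta time.
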(event Custom|CustomEvent_0
  (params (PSystem :type Particle%20System%20Component%20Object%20Reference))
  (Actor|DestroyActor))

(event EventBeginPlay
  (bind _maineffectemitter (Variables|Default|GetMainEffectEmitter))
  (Effects|Components|ParticleSystem|SetTemplate _maineffectemitter (Variables|Default|GetMainEffect))
  (Components|Activation|Activate (Variables|Default|GetMainEffectEmitter) false)
  (EventDispatchers|BindEventtoOnSystemFinished _maineffectemitter (delegate Custom|CustomEvent_0)))

(event EventActorBeginOverlap
  (params (OtherActor :type Actor%20Object%20Reference)))

(event EventTick
  (params (DeltaSeconds :type Float%20%28single-precision%29))
  (CallFunction|Move DeltaSeconds))

(fn ConstructionScript)

(fn Move
  (params (DeltaSeconds :type Float%20%28single-precision%29))
  (if (Variables|Default|GetVelocityDecay)
    (Variables|Default|SetVelocity (- (Variables|Default|GetVelocity) (* (Variables|Default|GetVelocity) (Variables|Default|GetVelocityDecayFactor)))))
  (Transformation|SetActorLocation (+ (* (Variables|Default|GetVelocity) DeltaSeconds) (Transformation|GetActorLocation)) false false))