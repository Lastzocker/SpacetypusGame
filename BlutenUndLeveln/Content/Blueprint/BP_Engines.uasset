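; Engine actor for a ship that drives its thruster particle effects and engine sound from the ship's thrust inputs.
; SetupThrusterEffects spawns particle components at mesh sockets named by main, brake, left or right prefix plus index, grouped into one array per direction.
; Each tick HandleThrust eases the four thrust values toward the ship's, which scale particle alpha and feed a clamped engine volume.
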(event EventBeginPlay)

(event EventActorBeginOverlap
  (params (OtherActor :type Actor%20Object%20Reference)))

(event EventTick
  (params (DeltaSeconds :type Float%20%28single-precision%29))
  (Utilities|IsValid (Variables|Default|GetShip)
    (:Is%20Valid
      (CallFunction|HandleThrust)
      (for _array_element (Variables|Default|GetMainThrusters)
        (Effects|Components|ParticleSystem|SetFloatParameter _array_element "InstanceAlphaScaleOverLife" (Variables|Default|GetMainThrust)))
      (for _array_element_2 (Variables|Default|GetBrakeThrusters)
        (Effects|Components|ParticleSystem|SetFloatParameter _array_element_2 "InstanceAlphaScaleOverLife" (Variables|Default|GetBrakeThrust)))
      (for _array_element_3 (Variables|Default|GetLeftThrusters)
        (Effects|Components|ParticleSystem|SetFloatParameter _array_element_3 "InstanceAlphaScaleOverLife" (Variables|Default|GetLeftThrust)))
      (for _array_element_4 (Variables|Default|GetRightThrusters)
        (Effects|Components|ParticleSystem|SetFloatParameter _array_element_4 "InstanceAlphaScaleOverLife" (Variables|Default|GetRightThrust))))))

(fn ConstructionScript)

(fn HandleThrust
  (bind _ship (Variables|Default|GetShip))
  (bind _mainvolumemultiplier (LocalVariables|GetMainVolumeMultiplier))
  (bind _brakevolumemultiplier (LocalVariables|GetBrakeVolumeMultiplier))
  (Utilities|FlowControl|Sequence
    (:then_0
      (bind _output_get (Variables|Default|SetMainThrust (Math|Float|Lerp (Variables|Default|GetMainThrust) (Variables|/Script/BlutenUndLeveln.BlutenUndLevelnPawn|GetForwardThrust _ship) 0.1)))
      (LocalVariables|SetEngineVolume (Math|Float|Clamp(Float) (+ (LocalVariables|GetEngineVolume) (* _output_get _mainvolumemultiplier)) 0.0 _mainvolumemultiplier)))
    (:then_1
      (bind _output_get_2 (Variables|Default|SetBrakeThrust (Math|Float|Lerp (Variables|Default|GetBrakeThrust) (* (Variables|/Script/BlutenUndLeveln.BlutenUndLevelnPawn|GetBackwardThrust _ship) -1.0) 0.1)))
      (LocalVariables|SetEngineVolume (Math|Float|Clamp(Float) (+ (LocalVariables|GetEngineVolume) (* _output_get_2 _brakevolumemultiplier)) 0.0 _brakevolumemultiplier)))
    (:then_2
      (bind _output_get_3 (Variables|Default|SetRightThrust (Math|Float|Lerp (Variables|Default|GetRightThrust) (Variables|/Script/BlutenUndLeveln.BlutenUndLevelnPawn|GetRightThrust _ship) 0.1)))
      (LocalVariables|SetEngineVolume (Math|Float|Clamp(Float) (+ (LocalVariables|GetEngineVolume) _output_get_3) 0.0 1.0)))
    (:then_3
      (bind _output_get_4 (Variables|Default|SetLeftThrust (Math|Float|Lerp (Variables|Default|GetLeftThrust) (* (Variables|/Script/BlutenUndLeveln.BlutenUndLevelnPawn|GetLeftThrust _ship) -1.0) 0.1)))
      (LocalVariables|SetEngineVolume (Math|Float|Clamp(Float) (+ (LocalVariables|GetEngineVolume) _output_get_4) 0.0 1.0)))
    (:then_4
      (Audio|Components|Audio|SetVolumeMultiplier (Variables|Default|GetEngineSound) (LocalVariables|GetEngineVolume) :!class /Script/Engine.AudioComponent))))

(fn SetupThrusterEffects
  (params (ThrusterEffects :type Array%20of%20Particle%20System%20Object%20References))
  (bind _item (Utilities|Array|Get(acopy) ThrusterEffects 2))
  (bind _ship (Variables|Default|GetShip))
  (bind _shipmeshcomponent (Variables|/Script/BlutenUndLeveln.BlutenUndLevelnPawn|GetShipMeshComponent _ship))
  (bind _returnvalue (Transformation|GetAllSocketNames _shipmeshcomponent))
  (bind _returnvalue_2 (Utilities|Array|Length _returnvalue))
  (bind _returnvalue_3 (- _returnvalue_2 1))
  (for _array_element _returnvalue
    (Utilities|FlowControl|Sequence
      (:then_0
        (for _index (range 0 _returnvalue_3)
          (if (Utilities|Enum|Equal(Enum) (Utilities|String|BuildString(Integer) "" "ENG_Main_" _index) (Utilities|String|ToString(Name) _array_element))
            (CallFunction|AddThrusterEffect (Transformation|GetSocketTransform (Variables|/Script/BlutenUndLeveln.BlutenUndLevelnPawn|GetShipMeshComponent (Variables|Default|GetShip)) _array_element "RTS_Actor") (Utilities|Array|Get(acopy) ThrusterEffects) (Variables|Default|GetMainThrusters)))))
      (:then_1
        (for _index_2 (range 0 _returnvalue_3)
          (if (Utilities|Enum|Equal(Enum) (Utilities|String|BuildString(Integer) "" "ENG_Brake_" _index_2) (Utilities|String|ToString(Name) _array_element))
            (CallFunction|AddThrusterEffect (Transformation|GetSocketTransform (Variables|/Script/BlutenUndLeveln.BlutenUndLevelnPawn|GetShipMeshComponent (Variables|Default|GetShip)) _array_element "RTS_Actor") (Utilities|Array|Get(acopy) ThrusterEffects 1) (Variables|Default|GetBrakeThrusters)))))
      (:then_2
        (for _index_3 (range 0 _returnvalue_3)
          (if (Utilities|Enum|Equal(Enum) (Utilities|String|BuildString(Integer) "" "ENG_Left_" _index_3) (Utilities|String|ToString(Name) _array_element))
            (CallFunction|AddThrusterEffect (Transformation|GetSocketTransform (Variables|/Script/BlutenUndLeveln.BlutenUndLevelnPawn|GetShipMeshComponent (Variables|Default|GetShip)) _array_element "RTS_Actor") _item (Variables|Default|GetLeftThrusters)))))
      (:then_3
        (for _index_4 (range 0 _returnvalue_3)
          (if (Utilities|Enum|Equal(Enum) (Utilities|String|BuildString(Integer) "" "ENG_Right_" _index_4) (Utilities|String|ToString(Name) _array_element))
            (CallFunction|AddThrusterEffect (Transformation|GetSocketTransform (Variables|/Script/BlutenUndLeveln.BlutenUndLevelnPawn|GetShipMeshComponent (Variables|Default|GetShip)) _array_element "RTS_Actor") _item (Variables|Default|GetRightThrusters))))))))

(fn AddThrusterEffect
  (params (Transform :type Transform) (Effect :type Particle%20System%20Object%20Reference) (Array :type Array%20of%20Particle%20System%20Component%20Object%20References))
  (bind _returnvalue (AddComponent|AddParticleSystemComponent false Transform))
  (Effects|Components|ParticleSystem|SetTemplate _returnvalue Effect)
  (Utilities|Array|Add Array _returnvalue))