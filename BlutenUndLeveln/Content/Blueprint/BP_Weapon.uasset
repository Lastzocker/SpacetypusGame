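; Weapon actor that fires projectiles with a cooldown, critical hits and optional auto-fire, configured from the LightAuto row of DATA_Weapons on BeginPlay.
; Fire spawns and launches a projectile with rolled critical damage, attaches a muzzle effect and starts the cooldown timer.
; CoolDownFinished re-enables firing and, during auto-fire, refires along the owner's forward vector with random yaw spread plus owner velocity.
; Energy cost and max ammo are only stored here.
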(event EventBeginPlay
  (bind _returnvalue (Utilities|GetDataTableRow "/Game/DataTables/DATA_Weapons.DATA_Weapons" "LightAuto")
    (:then
      (CallFunction|Initialize _returnvalue))))

(event EventActorBeginOverlap
  (params (OtherActor :type Actor%20Object%20Reference)))

(event EventTick
  (params (DeltaSeconds :type Float%20%28single-precision%29)))

(fn ConstructionScript)

(fn Fire
  (params (Velocity :type Vector))
  (bind _projectilespawnlocation (Variables|Default|GetProjectileSpawnLocation))
  (bind _returnvalue (Transformation|GetWorldTransform _projectilespawnlocation))
  (if (Variables|Internal|GetCanFire)
    (Variables|Internal|SetCanFire false)
    (Utilities|Time|SetTimerbyEvent (EventDispatchers|CreateEvent :!event CoolDownFinished) (Variables|Stats|GetCoolDown))
    (bind _returnvalue_2 (Game|SpawnActorfromClass (Variables|Default|GetProjectile) _returnvalue "AlwaysSpawn" 0 (Variables|Default|GetOwningActor) 0))
    (Utilities|IsValid _returnvalue_2
      (:Is%20Valid
        (bind (_iscritical _damage) (CallFunction|EvaluateCritical))
        (Default|Launch _returnvalue_2 Velocity _damage _iscritical)
        (Effects|SpawnEmitterAttached (Variables|Default|GetMuzzleEffect) _projectilespawnlocation "None" "0, 0, 0" (.Rotation (Math|Transform|BreakTransform _returnvalue)) "SnapToTarget" false)))))

(fn CoolDownFinished
  (bind _owningactor (Variables|Default|GetOwningActor))
  (bind _projectilespread (Variables|Stats|GetProjectileSpread))
  (Variables|Internal|SetCanFire true)
  (if (and (Variables|Default|GetCanAutoFire) (Variables|Internal|GetIsAutoFireActive))
    (CallFunction|Fire (+ (Transformation|GetVelocity _owningactor) (* (Math|Vector|RotateVector (Transformation|GetActorForwardVector _owningactor) (Math|Rotator|MakeRotator 0.0 0.0 (Math|Random|RandomFloatinRange (* _projectilespread -1.0) _projectilespread))) (Variables|Stats|GetProjectileVelocity))))))

(fn EvaluateCritical
  (if (<= (Math|Random|RandomFloat) (Variables|Stats|GetCriticalChance))
    (return true (* (Variables|Stats|GetCriticalMultiplier) (Variables|Stats|GetDamage)))
    (else
      (return false (Variables|Stats|GetDamage)))))

(fn Initialize
  (params (WeaponType :type STRUCT%20Weapon%20Structure))
  (bind (_name _mesh _damage _criticalchance _criticalmultiplier _cooldown _projectilevelocity _projectilespread _energyconsumption _weaponclass _maxammo _projectile _muzzleeffect) (Utilities|Struct|BreakSTRUCT_Weapon WeaponType))
  (Components|StaticMesh|SetStaticMesh (Variables|Default|GetWeaponMesh) _mesh)
  (Variables|Stats|SetDamage _damage)
  (Variables|Stats|SetCriticalChance _criticalchance)
  (Variables|Stats|SetCriticalMultiplier _criticalmultiplier)
  (Variables|Stats|SetCoolDown _cooldown)
  (Variables|Stats|SetProjectileVelocity _projectilevelocity)
  (Variables|Stats|SetProjectileSpread _projectilespread)
  (Variables|Stats|SetShootingEnergyCost _energyconsumption)
  (Variables|Stats|SetMaxAmmo _maxammo)
  (Variables|Default|SetProjectile _projectile)
  (Variables|Default|SetMuzzleEffect _muzzleeffect))