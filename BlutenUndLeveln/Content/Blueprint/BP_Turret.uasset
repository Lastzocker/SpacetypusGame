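; BP_Turret is a turret that tracks the player's pawn within engagement range and fires at it in timed bursts.
; A looping timer sets or clears the target and starts a burst on TurretWeaponArray when aim is within tolerance.
; Each tick, the mesh yaws toward an iteratively predicted lead point from relative velocity and projectile speed, with its turn capped per frame rather than scaled by delta time.
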(event Custom|FireBurst
  (CallFunction|FireTurret)
  (Utilities|FlowControl|Delay (Variables|Default|GetBurstDuration))
  (CallFunction|EndFire))

(event EventBeginPlay
  (Utilities|Time|SetTimerbyFunctionName 0 "CheckTarget" (+ (Variables|Default|GetTimeBetweenBursts) (Variables|Default|GetBurstDuration)) true))

(event EventActorBeginOverlap
  (params (OtherActor :type Actor%20Object%20Reference)))

(event EventTick
  (params (DeltaSeconds :type Float%20%28single-precision%29))
  (CallFunction|TurntoTarget))

(fn ConstructionScript)

(fn Initialize)

(fn FireTurret
  (bind _turretweaponarray (Variables|Default|GetTurretWeaponArray))
  (Variables|/Game/Blueprint/BP_WeaponArray.BP_WeaponArray_C|SetIsAutoFireActive _turretweaponarray true)
  (Default|Fire _turretweaponarray))

(fn TurntoTarget
  (bind _turretmesh (Variables|Default|GetTurretMesh))
  (bind _targetactor (Variables|Default|GetTargetActor))
  (bind _returnvalue (Math|Vector|GetForwardVector _turretmesh))
  (Utilities|IsValid (Variables|Default|GetTargetActor)
    (:Is%20Valid
      (bind _predictedaimvector (Class|CVectorUtility|GetAimDirectionIterative (Transformation|GetWorldLocation (Variables|Default|GetTurretMesh)) (Transformation|GetActorLocation _targetactor) (- (Transformation|GetVelocity _targetactor) (Transformation|GetVelocity)) (Math|Vector|MakeVector 0.0 0.0 0.0) (Variables|/Game/Blueprint/BP_WeaponArray.BP_WeaponArray_C|GetProjectileVelocity (Variables|Default|GetTurretWeaponArray)) (Variables|Default|GetIterations) (Variables|Default|GetTimeToTarget)))
      (Transformation|SetWorldRotation _turretmesh (Math|Rotator|MakeRotator 0.0 0.0 (+ (.yaw (Transformation|GetWorldRotation _turretmesh)) (* (* (Math|Float|Sign(Float) (Math|Vector|DotProduct (Math|Vector|CrossProduct _predictedaimvector (Math|Vector|Normalize _returnvalue)) (Math|Vector|GetUpVector _turretmesh))) -1.0) (Math|Float|Min(Float) (Variables|Default|GetTurnRate) (Class|KismetMathLibrary|DegAcos (Math|Vector|DotProduct _returnvalue _predictedaimvector)))))) false false)
      (Variables|Default|SetShouldFire (<= (Class|KismetMathLibrary|DegAcos (Math|Vector|DotProduct _returnvalue _predictedaimvector)) 5.0)))))

(fn CheckTarget
  (bind _returnvalue (Game|GetPlayerController 0))
  (bind _returnvalue_2 (Pawn|GetControlledPawn _returnvalue))
  (if (< (Transformation|GetHorizontalDistanceTo _returnvalue_2) (Variables|Default|GetEngagementRange))
    (Variables|Default|SetTargetActor _returnvalue_2)
    (if (Variables|Default|GetShouldFire)
      (CallFunction|FireBurst))
    (else
      (Variables|Default|SetTargetActor 0))))

(fn EndFire
  (Variables|/Game/Blueprint/BP_WeaponArray.BP_WeaponArray_C|SetIsAutoFireActive (Variables|Default|GetTurretWeaponArray) false))