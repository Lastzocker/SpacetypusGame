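; Player controller for BP_BlutenUndLevelnPawn that forwards movement, turning, targeting and weapon input, with alt-fire using the next weapon slot.
; On BeginPlay it creates the pawn camera, marks a beacon on the HUD and binds pawn integrity, energy, ammo and collision events.
; Collisions drive impulse-scaled camera shake and a timeline-animated post-process distortion.
; Tick lerps the camera toward the pawn's anchor and optionally steers by mouse offset from screen centre.
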(event Custom|Collision
  (params (Impulse :type Float%20%28single-precision%29))
  (bind _returnvalue (/ Impulse 1e+05))
  ;[1 1 1] Collision Event
  (Class|PlayerController|ClientPlayCameraShake "/Game/CollisionShake.CollisionShake_C" _returnvalue "CameraLocal" "0, 0, 0")
  (bind _newtrack_0 (Timeline|DistortBlendTimeline PlayFromStart)
    (:Update
      (Rendering|Material|SetScalarParameterValue (Variables|Default|GetDistortPPMaterial) "Intensity" (* _newtrack_0 _returnvalue) :!class /Script/Engine.MaterialInstanceDynamic))))

(event Custom|UpdateHullIntegrityDisplay
  (params (IsDamageEvent :type Boolean) (NewIntegrity :type Float%20%28single-precision%29))
  ;[1 1 1] HUD Events
  (Default|SetStructuralIntegrity (Variables|/Game/Blueprint/BP_C_PlayerHUD.BP_C_PlayerHUD_C|GetHUD (Variables|Default|GetBP_C_PlayerHUD)) IsDamageEvent NewIntegrity))

(event Custom|UpdateEnergyDisplay
  (params (NewEnergy :type Float%20%28single-precision%29))
  ;[1 1 1] HUD Events
  (Default|SetEnergy (Variables|/Game/Blueprint/BP_C_PlayerHUD.BP_C_PlayerHUD_C|GetHUD (Variables|Default|GetBP_C_PlayerHUD)) NewEnergy))

(event Custom|UpdateAmmoDisplay
  (params (IsConsumeEvent :type Boolean) (CurrentAmmo :type Integer) (MaxAmmo :type Integer))
  (bind _bp_c_playerhud (Variables|Default|GetBP_C_PlayerHUD))
  (bind _hud (Variables|/Game/Blueprint/BP_C_PlayerHUD.BP_C_PlayerHUD_C|GetHUD _bp_c_playerhud))
  ;[1 1 1] HUD Events
  (Default|SetCurrentAmmo _hud CurrentAmmo IsConsumeEvent)
  (Default|SetMaxAmmo _hud MaxAmmo))

(event Custom|ChangeMoneyDisplay
  (params (NewMoney :type Integer) (ReceivedMoney :type Integer))
  ;[1 1 1] HUD Events
  (Default|SetMoney (Variables|/Game/Blueprint/BP_C_PlayerHUD.BP_C_PlayerHUD_C|GetHUD (Variables|Default|GetBP_C_PlayerHUD)) NewMoney ReceivedMoney))

(event EventBeginPlay
  ;[1 1 1] Begin play
  (bind _asbp_bluten_und_leveln_pawn (Utilities|Casting|CastToBP_BlutenUndLevelnPawn (Game|Player|GetPlayerPawn 0)))
  (Variables|Default|SetPlayerPawn _asbp_bluten_und_leveln_pawn)
  (Default|MakeCamera _asbp_bluten_und_leveln_pawn)
  (Variables|Default|SetCameraTransform (Transformation|GetWorldTransform (Variables|/Game/Blueprint/BP_BlutenUndLevelnPawn.BP_BlutenUndLevelnPawn_C|GetCameraAnchor _asbp_bluten_und_leveln_pawn)))
  (bind _outactors (Actor|GetAllActorsOfClass "/Game/Blueprint/LevelElements/BP_Beacon.BP_Beacon_C"))
  (Default|AddTarget (Variables|Default|GetBP_C_PlayerHUD) (Utilities|Array|Get(acopy) _outactors) "/Game/HUD/HUDTextures/TEX_HUD_BeaconMarker.TEX_HUD_BeaconMarker")
  ;[1 1 1] HUD Events
  (EventDispatchers|BindEventtoStructuralIntegrityChanged (Variables|Default|GetPlayerPawn) (delegate Custom|UpdateHullIntegrityDisplay))
  (EventDispatchers|BindEventtoEnergyChanged (Variables|Default|GetPlayerPawn) (delegate Custom|UpdateEnergyDisplay))
  (EventDispatchers|BindEventtoAmmoChanged (Variables|Default|GetPlayerPawn) (delegate Custom|UpdateAmmoDisplay))
  (EventDispatchers|BindEventtoOnCollision (Variables|Default|GetPlayerPawn) (delegate Custom|Collision))
  ;[1 1 1] Setup Postprocessing
  (bind _returnvalue (Rendering|Material|CreateDynamicMaterialInstance "/Game/Materials/PostProcess/INST_PP_Distortion.INST_PP_Distortion" :!class /Script/Engine.KismetMaterialLibrary))
  (Variables|Default|SetDistortPPMaterial _returnvalue)
  (Variables|/Script/Engine.PostProcessComponent|SetSettings (Variables|Default|GetPostProcess) (Utilities|Struct|MakePostProcessSettings (Utilities|Struct|MakeWeightedBlendables (Utilities|Array|MakeArray (Utilities|Struct|MakeWeightedBlendable 1.0 (Variables|Default|GetDistortPPMaterial)))))))

(event EventTick
  (params (DeltaSeconds :type Float%20%28single-precision%29))
  (bind _sizex (HUD|GetViewportSize))
  (bind _returnvalue (/ _sizex 2))
  (bind _returnvalue_2 (Math|Conversions|ToFloat(Integer) _returnvalue))
  ;[1 1 1] Tick
  (bind _asbp_bluten_und_leveln_pawn (Utilities|Casting|CastToBP_BlutenUndLevelnPawn (Game|Player|GetPlayerPawn 0)))
  (if (!= (Variables|/Game/Blueprint/BP_BlutenUndLevelnPawn.BP_BlutenUndLevelnPawn_C|GetCamera _asbp_bluten_und_leveln_pawn) 0) ; Check if player has a camera
    (bind _output_get (Variables|Default|SetCameraTransform (Math|Transform|MakeTransform (Math|Vector|Lerp(Vector) (.location (Variables|Default|GetCameraTransform)) (.location (Transformation|GetWorldTransform (Variables|/Game/Blueprint/BP_BlutenUndLevelnPawn.BP_BlutenUndLevelnPawn_C|GetCameraAnchor _asbp_bluten_und_leveln_pawn))) (Variables|Default|GetCameraLocationSmoothing)) (Math|Rotator|Lerp(Rotator) (.rotation (Variables|Default|GetCameraTransform)) (.rotation (Transformation|GetWorldTransform (Variables|/Game/Blueprint/BP_BlutenUndLevelnPawn.BP_BlutenUndLevelnPawn_C|GetCameraAnchor _asbp_bluten_und_leveln_pawn))) (Variables|Default|GetCameraRotationSmoothing) true) "1,1,1")))
    (Transformation|SetWorldTransform (Variables|/Game/Blueprint/BP_BlutenUndLevelnPawn.BP_BlutenUndLevelnPawn_C|GetCamera _asbp_bluten_und_leveln_pawn) _output_get false false)
    ;[1 1 1] Mouse Control
    (if (Variables|Default|GetMouseControl)
      (Class|BlutenUndLevelnPawn|Turn (Variables|Default|GetPlayerPawn) (/ (- (.LocationX (Game|Player|GetMousePosition)) _returnvalue_2) _returnvalue_2)))))

(event Input|ActionEvents|InputActionFire
  (params (Key :type Key%20Structure :default "AnyKey"))
  (bind _returnvalue (Pawn|GetControlledPawn))
  ;[1 1 1] Inputs
  (:Pressed
    (bind _asbp_bluten_und_leveln_pawn (Utilities|Casting|CastToBP_BlutenUndLevelnPawn _returnvalue))
    (Default|FireWeaponArray _asbp_bluten_und_leveln_pawn (Variables|/Game/Blueprint/BP_BlutenUndLevelnPawn.BP_BlutenUndLevelnPawn_C|GetActiveWeaponSlot _asbp_bluten_und_leveln_pawn)))
  (:Released
    (bind _asbp_bluten_und_leveln_pawn_2 (Utilities|Casting|CastToBP_BlutenUndLevelnPawn _returnvalue))
    (Default|ReleaseFireButton _asbp_bluten_und_leveln_pawn_2 (Variables|/Game/Blueprint/BP_BlutenUndLevelnPawn.BP_BlutenUndLevelnPawn_C|GetActiveWeaponSlot _asbp_bluten_und_leveln_pawn_2))))

(event Input|ActionEvents|InputActionFindTarget
  (params (Key :type Key%20Structure :default "AnyKey"))
  ;[1 1 1] Inputs
  (:Pressed
    (bind _asbp_bluten_und_leveln_pawn (Utilities|Casting|CastToBP_BlutenUndLevelnPawn (Pawn|GetControlledPawn)))
    (Class|BlutenUndLevelnPawn|FindTarget _asbp_bluten_und_leveln_pawn)))

(event Input|ActionEvents|InputActionSwitchWeapon
  (params (Key :type Key%20Structure :default "AnyKey"))
  (bind _bp_c_playerhud (Variables|Default|GetBP_C_PlayerHUD))
  (bind _hud (Variables|/Game/Blueprint/BP_C_PlayerHUD.BP_C_PlayerHUD_C|GetHUD _bp_c_playerhud))
  ;[1 1 1] Inputs
  (:Pressed
    (bind _asbp_bluten_und_leveln_pawn (Utilities|Casting|CastToBP_BlutenUndLevelnPawn (Pawn|GetControlledPawn)))
    (bind _nextweaponslot (Default|GetNextWeaponArray _asbp_bluten_und_leveln_pawn))
    (Variables|/Game/Blueprint/BP_BlutenUndLevelnPawn.BP_BlutenUndLevelnPawn_C|SetActiveWeaponSlot _asbp_bluten_und_leveln_pawn _nextweaponslot)
    (Default|SetCurrentAmmo _hud 0 false)
    (Default|SetMaxAmmo _hud)))

(event Input|ActionEvents|InputActionAltFire
  (params (Key :type Key%20Structure :default "AnyKey"))
  (bind _returnvalue (Pawn|GetControlledPawn))
  ;[1 1 1] Inputs
  (:Pressed
    (bind _asbp_bluten_und_leveln_pawn (Utilities|Casting|CastToBP_BlutenUndLevelnPawn _returnvalue))
    (bind _nextweaponslot (Default|GetNextWeaponArray _asbp_bluten_und_leveln_pawn))
    (Default|FireWeaponArray _asbp_bluten_und_leveln_pawn _nextweaponslot))
  (:Released
    (bind _asbp_bluten_und_leveln_pawn_2 (Utilities|Casting|CastToBP_BlutenUndLevelnPawn _returnvalue))
    (bind _nextweaponslot_2 (Default|GetNextWeaponArray _asbp_bluten_und_leveln_pawn_2))
    (Default|ReleaseFireButton _asbp_bluten_und_leveln_pawn_2 _nextweaponslot_2)))

(event Input|ActionEvents|InputActionInteract
  (params (Key :type Key%20Structure :default "AnyKey"))
  ;[1 1 1] Inputs
  (:Pressed
    (Default|CallInteractionKey)))

(event Input|AxisEvents|InputAxisMoveForward
  (params (AxisValue :type Float%20%28single-precision%29))
  ;[1 1 1] Inputs
  (bind _asbp_bluten_und_leveln_pawn (Utilities|Casting|CastToBP_BlutenUndLevelnPawn (Pawn|GetControlledPawn)))
  (Class|BlutenUndLevelnPawn|MoveForward _asbp_bluten_und_leveln_pawn AxisValue))

(event Input|AxisEvents|InputAxisMoveRight
  (params (AxisValue :type Float%20%28single-precision%29))
  ;[1 1 1] Inputs
  (bind _asbp_bluten_und_leveln_pawn (Utilities|Casting|CastToBP_BlutenUndLevelnPawn (Pawn|GetControlledPawn)))
  (Class|BlutenUndLevelnPawn|MoveRight _asbp_bluten_und_leveln_pawn AxisValue))

(event Input|AxisEvents|InputAxisTurn
  (params (AxisValue :type Float%20%28single-precision%29))
  ;[1 1 1] Inputs
  (if (not (Variables|Default|GetMouseControl))
    (bind _asbp_bluten_und_leveln_pawn (Utilities|Casting|CastToBP_BlutenUndLevelnPawn (Pawn|GetControlledPawn)))
    (Class|BlutenUndLevelnPawn|Turn _asbp_bluten_und_leveln_pawn AxisValue)))

(fn ConstructionScript)