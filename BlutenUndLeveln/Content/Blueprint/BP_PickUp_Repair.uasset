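; BP_PickUp_Repair is a pickup that restores hull integrity to whoever receives it.
; Its ItemAction runs the parent behavior, then calls Repair on the receiver with a RestorePercentage share of its MaxHullIntegrity.
; GetGainValue separately returns RestorePercentage scaled by the game instance's RepairGainMultiplier, truncated to an integer.
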(event EventBeginPlay)

(event EventActorBeginOverlap
  (params (OtherActor :type Actor%20Object%20Reference))
  (|CallParentFunction 0))

(event EventTick
  (params (DeltaSeconds :type Float%20%28single-precision%29)))

(event EventItemAction
  (params (Receiver :type BP%20Bluten%20Und%20Leveln%20Pawn%20Object%20Reference))
  (|CallParentFunction Receiver)
  (Default|Repair Receiver (* (Variables|/Script/BlutenUndLeveln.BlutenUndLevelnPawn|GetMaxHullIntegrity Receiver) (Variables|Default|GetRestorePercentage))))

(fn ConstructionScript
  (|CallParentFunction))

(fn GetGainValue
  (bind _asbp_game_instance (Utilities|Casting|CastToBP_GameInstance (Game|GetGameInstance))
    (:then
      _)
    (:CastFailed
      _))
  (return (Math|Float|Truncate (* (Variables|Default|GetRestorePercentage) (Variables|/Game/Blueprint/BP_GameInstance.BP_GameInstance_C|GetRepairGainMultiplier _asbp_game_instance)))))