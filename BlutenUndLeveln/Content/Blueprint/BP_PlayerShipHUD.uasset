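; Player ship HUD actor that shows a reticle, vitals and decorator around the ship and reports sensor contacts.
; Every tick it rotates the reticle by the actor's yaw relative to the camera and places vitals and decorator at different XY blends between camera and ship for a parallax effect.
; Sensor overlaps send detect messages through a gate opened shortly after BeginPlay, while end overlaps send lost-contact messages ungated.
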(event OnComponentBeginOverlap(SensorDetectionRange)
  (params (OtherActor :type Actor%20Object%20Reference) (OtherComp :type Primitive%20Component%20Object%20Reference) (OtherBodyIndex :type Integer) (bFromSweep :type Boolean) (SweepResult :type Hit%20Result%20Structure%20%28by%20ref%29))
  (Utilities|FlowControl|Gate true
    (:Exit
      (Class|INTERFACEDetectable|OnDetect(Message) OtherActor))))

(event OnComponentEndOverlap(SensorDetectionRange)
  (params (OtherActor :type Actor%20Object%20Reference) (OtherComp :type Primitive%20Component%20Object%20Reference) (OtherBodyIndex :type Integer))
  (Class|INTERFACEDetectable|OnLostContact(Message) OtherActor))

(event EventBeginPlay
  (bind _ashud_reticle (Utilities|Casting|CastToHUD_Reticle (UserInterface|GetUserWidgetObject (Variables|Default|GetReticleWidget))))
  (Variables|Default|SetReticle _ashud_reticle)
  (bind _asbp_bu_lplayer_controller (Utilities|Casting|CastToBP_BuLPlayerController (Game|GetPlayerController 0)))
  (Variables|Default|SetPlayerControllerReference _asbp_bu_lplayer_controller)
  (Utilities|FlowControl|Delay 0.1)
  (Utilities|FlowControl|Gate true) ; enters at Open
)

(event EventActorBeginOverlap
  (params (OtherActor :type Actor%20Object%20Reference)))

(event EventTick
  (params (DeltaSeconds :type Float%20%28single-precision%29))
  (Class|Widget|SetRenderAngle (Variables|Default|GetReticle) (- (.yaw (Transformation|GetActorRotation)) (.yaw (.rotation (Variables|/Game/Blueprint/BP_BuLPlayerController.BP_BuLPlayerController_C|GetCameraTransform (Variables|Default|GetPlayerControllerReference))))))
  (CallFunction|HandleShipGroup))

(fn ConstructionScript)

(fn HandleShipGroup
  (bind _returnvalue (Transformation|GetActorLocation))
  (bind _playercontrollerreference (Variables|Default|GetPlayerControllerReference))
  (bind _cameratransform (Variables|/Game/Blueprint/BP_BuLPlayerController.BP_BuLPlayerController_C|GetCameraTransform _playercontrollerreference))
  (Transformation|SetWorldLocation (Variables|Default|GetVitals) (Math|Vector|MakeVector (Math|Float|Lerp (.x (.location _cameratransform)) (.x _returnvalue) 0.7) (Math|Float|Lerp (.y (.location _cameratransform)) (.y _returnvalue) 0.7) 0.0) false false)
  (Transformation|SetWorldLocation (Variables|Default|GetDecorator1) (Math|Vector|MakeVector (Math|Float|Lerp (.x (.location _cameratransform)) (.x _returnvalue) 0.8) (Math|Float|Lerp (.y (.location _cameratransform)) (.y _returnvalue) 0.8) 0.0) false false))