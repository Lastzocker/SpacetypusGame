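; Shield-slot camo equipment that cloaks the owning ship by hiding it from view while active, at an energy cost.
; Use hides the ship mesh, without propagating to its child components, and each weapon array actor, and Release shows them again.
; While active, Tick drains the owner's energy scaled by delta time and calls Release when the energy change fails.
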(event EventBeginPlay
  (|CallParentFunction))

(event EventActorBeginOverlap
  (params (OtherActor :type Actor%20Object%20Reference)))

(event EventTick
  (params (DeltaSeconds :type Float%20%28single-precision%29))
  (if (Variables|Default|GetIsActive)
    (bind _successful (Default|ChangeEnergy (Variables|Default|GetOwningActor) (* (Variables|Default|GetEnergyConsumption) DeltaSeconds -1.0)))
    (if (not _successful)
      (CallFunction|Release))))

(event EventUse
  (bind _owningactor (Variables|Default|GetOwningActor))
  (Development|SetHiddeninGame (Variables|/Script/BlutenUndLeveln.BlutenUndLevelnPawn|GetShipMeshComponent _owningactor) true false)
  (Variables|Default|SetIsActive true)
  (for _array_element (Variables|/Game/Blueprint/BP_BlutenUndLevelnPawn.BP_BlutenUndLevelnPawn_C|GetWeaponArrays _owningactor)
    (Rendering|SetActorHiddenInGame _array_element true)))

(event EventRelease
  (bind _owningactor (Variables|Default|GetOwningActor))
  (Development|SetHiddeninGame (Variables|/Script/BlutenUndLeveln.BlutenUndLevelnPawn|GetShipMeshComponent _owningactor) false false)
  (Variables|Default|SetIsActive false)
  (for _array_element (Variables|/Game/Blueprint/BP_BlutenUndLevelnPawn.BP_BlutenUndLevelnPawn_C|GetWeaponArrays _owningactor)
    (Rendering|SetActorHiddenInGame _array_element false)))

(fn ConstructionScript
  (|CallParentFunction))