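; Weapon array actor that fires all of a ship's guns of one weapon class as a group.
; Initialize builds weapon meshes and muzzle arrows from named sockets on the parent mesh, then loads stats from DATA_Weapons; swaps must match that class.
; Fire shoots muzzles together or alternately, dividing cooldown by weapon count when alternating, with optional auto-refire.
; Each shot adds spread and a critical roll; only the player's ship pays ammo or energy, unless unlimited.
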(event EventBeginPlay)

(event Collision|EventActorBeginOverlap
  (params (OtherActor :type Actor%20Object%20Reference)))

(event EventTick
  (params (DeltaSeconds :type Float%20%28single-precision%29)))

(fn ConstructionScript)

(fn Fire
  (bind _returnvalue (Transformation|GetActorForwardVector))
  (bind _projectilevelocity (Variables|Stats|GetProjectileVelocity))
  (bind _owningship (Variables|Default|GetOwningShip))
  (bind _returnvalue_2 (* _returnvalue _projectilevelocity))
  (bind _returnvalue_3 (Transformation|GetVelocity _owningship))
  (bind _returnvalue_4 (+ _returnvalue_3 _returnvalue_2))
  (if (Variables|Internal|GetCanFire)
    (Variables|Internal|SetCanFire false)
    (Variables|Default|SetFireSoundPlayed false)
    (Utilities|Time|SetTimerbyEvent (EventDispatchers|CreateEvent :!event CoolDownFinished) (Variables|Internal|GetVirtualCooldown))
    (if (Variables|Config|GetAlternatingFire) ; Fire alternating or synchronized?
      (CallFunction|LaunchProjectile (Utilities|Array|Get(acopy) (Variables|Internal|GetArrayMuzzlePositions) (Variables|Internal|GetCurrentMuzzleIndex)) _returnvalue_4)
      (if (< (Variables|Internal|GetCurrentMuzzleIndex) (- (Variables|Default|GetWeaponCount) 1))
        (Math|Integer|IncrementInt (Variables|Internal|GetCurrentMuzzleIndex))
        (else
          (Variables|Internal|SetCurrentMuzzleIndex 0)))
      (else
        (for _array_element (Variables|Internal|GetArrayMuzzlePositions)
          (CallFunction|LaunchProjectile _array_element _returnvalue_4))))))

(fn CoolDownFinished
  (Variables|Internal|SetCanFire true)
  (if (and (Variables|Config|GetCanAutoFire) (Variables|Internal|GetIsAutoFireActive))
    (CallFunction|Fire)))

(fn EvaluateCritical
  (if (<= (Math|Random|RandomFloat) (Variables|Stats|GetCriticalChance))
    (return true (* (Variables|Stats|GetCriticalMultiplier) (Variables|Stats|GetDamage)))
    (else
      (return false (Variables|Stats|GetDamage)))))

(fn Initialize
  (params (WeaponTypeRowName :type Name) (OwningShip :type BP%20Bluten%20Und%20Leveln%20Pawn%20Object%20Reference) (ParentMesh :type Static%20Mesh%20Component%20Object%20Reference) (IsTurretArray :type Boolean))
  (Variables|Default|SetOwningShip OwningShip)
  (bind _returnvalue (Utilities|GetDataTableRow "/Game/DataTables/DATA_Weapons.DATA_Weapons" WeaponTypeRowName)
    (:then
      (CallFunction|SetupMuzzles ParentMesh (.WeaponClass (Utilities|Struct|BreakSTRUCT_Weapon _returnvalue)) IsTurretArray)
      (Variables|Default|SetArrayWeaponClass (.WeaponClass (Utilities|Struct|BreakSTRUCT_Weapon _returnvalue)))
      (CallFunction|SetWeapon WeaponTypeRowName))
    (:RowNotFound
      (Development|PrintText "WeaponArray: Invalid weapon type" true true "(R=1.000000,G=0.000000,B=0.000000,A=1.000000)"))))

(fn SetupMuzzles
  (params (ParentMesh :type Static%20Mesh%20Component%20Object%20Reference) (WeaponClass :type ENUM_WeaponClasses%20Enum) (IsTurretArray :type Boolean))
  (bind _returnvalue (Transformation|GetAllSocketNames ParentMesh))
  (if IsTurretArray
    (LocalVariables|SetSearchString "WPN_")
    (else
      (switch Utilities|FlowControl|Switch|SwitchonENUM_WeaponClasses WeaponClass
        (:NewEnumerator0
          (LocalVariables|SetSearchString "WPN_Projectile_"))
        (:NewEnumerator2
          (LocalVariables|SetSearchString "WPN_Plasma_"))
        (:NewEnumerator1
          (LocalVariables|SetSearchString "WPN_Laser_"))
        (:NewEnumerator3
          (LocalVariables|SetSearchString "WPN_Missile_")))))
  (for _array_element _returnvalue
    (for _index (range 0 (- (Utilities|Array|Length _returnvalue) 1))
      (if (Utilities|Name|Equal(Name) _array_element (Utilities|String|StringToName (Utilities|String|BuildString(Integer) "" (LocalVariables|GetSearchString) _index)))
        (bind _returnvalue_2 (AddComponent|AddStaticMeshComponent false (Transformation|GetSocketTransform ParentMesh _array_element "RTS_Actor")))
        (Utilities|Array|Add (Variables|Internal|GetArrayWeaponMeshes) _returnvalue_2)
        (bind _returnvalue_3 (AddComponent|AddArrowComponent false (Transformation|GetSocketTransform _returnvalue_2 "MUZZLE" "RTS_Actor")))
        (Utilities|Array|Add (Variables|Internal|GetArrayMuzzlePositions) _returnvalue_3)
        (Variables|Default|SetWeaponCount (+ (Variables|Default|GetWeaponCount) 1))))))

(fn LaunchProjectile
  (params (Muzzle :type Scene%20Component%20Object%20Reference) (Velocity :type Vector))
  (bind _returnvalue (Transformation|GetWorldTransform Muzzle))
  (bind _owningship (Variables|Default|GetOwningShip))
  (bind _owningship_2 (Variables|Default|GetOwningShip))
  (bind _projectilespread (Variables|Stats|GetProjectileSpread))
  ;[1 1 1] Check if shooting is possible
  (if (not (Variables|/Game/Blueprint/BP_BlutenUndLevelnPawn.BP_BlutenUndLevelnPawn_C|GetHasInfiniteAmmoAndEnergy _owningship_2))
    (if (== (Game|Player|GetPlayerPawn 0) _owningship_2)
      (if (> (Variables|Stats|GetMaxAmmo) 0)
        (bind _successful (Default|HandleAmmo _owningship_2))
        (if _successful
          (bind _returnvalue_2 (Game|SpawnActorfromClass (Variables|Default|GetProjectile) (Math|Transform|MakeTransform (Math|Vector|MakeVector (.x (.location _returnvalue)) (.y (.location _returnvalue)) 0.0) (.rotation _returnvalue) "1,1,1") "AlwaysSpawn" 0 _owningship (Variables|Default|GetArrayWeaponClass) _owningship :!label _label))
          (Utilities|IsValid _returnvalue_2
            (:Is%20Valid
              (bind (_iscritical _damage) (CallFunction|EvaluateCritical))
              (Default|Launch _returnvalue_2 (Math|Vector|RotateVector Velocity (Math|Rotator|MakeRotator 0.0 0.0 (Math|Random|RandomFloatinRange (* _projectilespread -1.0) _projectilespread))) _damage _iscritical)
              (bind _asbp_bu_lplayer_controller (Utilities|Casting|CastToBP_BuLPlayerController (Pawn|GetController (Variables|Default|GetOwningShip)))
                (:then
                  (Default|UpdateShotsFired _asbp_bu_lplayer_controller (Variables|Default|GetArrayWeaponClass)))
                (:CastFailed
                  _))
              (Effects|SpawnEmitterAttached (Variables|Default|GetMuzzleEffect) Muzzle "None" "0, 0, 0" "0, 0,0.000000" "SnapToTarget")
              (if (not (Variables|Default|GetFireSoundPlayed))
                (Audio|PlaySoundatLocation (Variables|Default|GetMuzzleSound) (Transformation|GetWorldLocation Muzzle) "0, 0, 0" 0.6 (Variables|Default|GetSoundPitch))
                (Variables|Default|SetFireSoundPlayed true)))))
        (else
          (bind _successful_2 (Default|ChangeEnergy _owningship_2 (Variables|Stats|GetShootingEnergyCost)))
          (if _successful_2
            (goto _label))))
      (else
        (goto _label)))
    (else
      (goto _label))))

(fn SetAlternatingFire
  (params (Value :type Boolean))
  (if Value
    (Variables|Internal|SetVirtualCooldown (/ (Variables|Stats|GetCoolDown) (Math|Conversions|ToFloat(Integer) (Variables|Default|GetWeaponCount))))
    (Variables|Config|SetAlternatingFire true)
    (else
      (Variables|Internal|SetVirtualCooldown (Variables|Stats|GetCoolDown))
      (Variables|Config|SetAlternatingFire false))))

(fn SetWeapon
  (params (WeaponTypeRowName :type Name))
  (bind _returnvalue (Utilities|GetDataTableRow "/Game/DataTables/DATA_Weapons.DATA_Weapons" WeaponTypeRowName)
    (:then
      (Variables|Default|SetWeaponTypeRowName WeaponTypeRowName)
      (if (Utilities|Enum|Equal(Enum) (.WeaponClass (Utilities|Struct|BreakSTRUCT_Weapon _returnvalue)) (Variables|Default|GetArrayWeaponClass))
        (for (_array_element _array_index) (Variables|Internal|GetArrayWeaponMeshes)
          (Components|StaticMesh|SetStaticMesh _array_element (.Mesh (Utilities|Struct|BreakSTRUCT_Weapon _returnvalue)))
          (Transformation|SetRelativeTransform (Utilities|Array|Get(acopy) (Variables|Internal|GetArrayMuzzlePositions) _array_index) (Transformation|GetSocketTransform _array_element "MUZZLE" "RTS_Actor") false false))
        (Variables|Default|SetWeaponTypeDisplayName (.Name (Utilities|Struct|BreakSTRUCT_Weapon _returnvalue)))
        (Variables|Stats|SetDamage (.Damage (Utilities|Struct|BreakSTRUCT_Weapon _returnvalue)))
        (Variables|Stats|SetCriticalChance (.CriticalChance (Utilities|Struct|BreakSTRUCT_Weapon _returnvalue)))
        (Variables|Stats|SetCriticalMultiplier (.CriticalMultiplier (Utilities|Struct|BreakSTRUCT_Weapon _returnvalue)))
        (Variables|Stats|SetCoolDown (.Cooldown (Utilities|Struct|BreakSTRUCT_Weapon _returnvalue)))
        (Variables|Stats|SetProjectileVelocity (.ProjectileVelocity (Utilities|Struct|BreakSTRUCT_Weapon _returnvalue)))
        (Variables|Stats|SetProjectileSpread (.ProjectileSpread (Utilities|Struct|BreakSTRUCT_Weapon _returnvalue)))
        (Variables|Stats|SetShootingEnergyCost (* (.EnergyConsumption (Utilities|Struct|BreakSTRUCT_Weapon _returnvalue)) -1.0))
        (Variables|Stats|SetMaxAmmo (.MaxAmmo (Utilities|Struct|BreakSTRUCT_Weapon _returnvalue)))
        (Variables|Default|SetProjectile (.Projectile (Utilities|Struct|BreakSTRUCT_Weapon _returnvalue)))
        (Variables|Default|SetMuzzleEffect (.MuzzleEffect (Utilities|Struct|BreakSTRUCT_Weapon _returnvalue)))
        (Variables|Default|SetMuzzleSound (.MuzzleSound (Utilities|Struct|BreakSTRUCT_Weapon _returnvalue)))
        (Variables|Default|SetSoundPitch (.SoundPitch (Utilities|Struct|BreakSTRUCT_Weapon _returnvalue)))
        (bind _output_get (Variables|Config|SetAlternatingFire (.Alternating (Utilities|Struct|BreakSTRUCT_Weapon _returnvalue))))
        (Default|AdjustAmmotoNewMaxAmmo (Variables|Default|GetOwningShip) (Variables|Stats|GetMaxAmmo) (Utilities|Enum|Equal(Enum) (Variables|Default|GetArrayWeaponClass) "NewEnumerator3"))
        (Default|CallWeaponChanged (Variables|Default|GetOwningShip) (.Name (Utilities|Struct|BreakSTRUCT_Weapon _returnvalue)) (.WeaponClass (Utilities|Struct|BreakSTRUCT_Weapon _returnvalue)))
        (if _output_get
          (Variables|Internal|SetVirtualCooldown (/ (Variables|Stats|GetCoolDown) (Math|Conversions|ToFloat(Integer) (Variables|Default|GetWeaponCount))))
          (else
            (Variables|Internal|SetVirtualCooldown (Variables|Stats|GetCoolDown))))
        (else
          (Development|PrintText "!Incombatible weapon class" true true "(R=1.000000,G=0.000000,B=0.030019,A=1.000000)"))))
    (:RowNotFound
      (Development|PrintText "WeaponArray: Invalid weapon type" true true "(R=1.000000,G=0.000000,B=0.000000,A=1.000000)"))))