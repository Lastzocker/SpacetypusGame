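; Player ship pawn that manages hull integrity, regenerating energy and two attached weapons spawned at BeginPlay, alongside HUD and minimap widgets.
; Damage, including impulse-scaled collision hits, lowers hull and starts timed invulnerability; death only prints.
; Weapons fire along the forward vector with random spread plus inherited velocity.
; Predictive targeting (precise or iterative) with debug drawing exists, but it and minimap marker updates are disconnected from execution.
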(event OnComponentHit(ShipMeshComponent)
  (params (OtherActor :type Actor%20Object%20Reference) (OtherComp :type Primitive%20Component%20Object%20Reference) (NormalImpulse :type Vector) (Hit :type Hit%20Result%20Structure%20%28by%20ref%29))
  (bind _returnvalue (Math|Vector|VectorLength NormalImpulse))
  (bind _collisiondamagedivisor (Variables|Gameplay|GetCollisionDamageDivisor))
  (bind _returnvalue_2 (/ _returnvalue _collisiondamagedivisor))
  (if (> _returnvalue (Variables|Gameplay|GetCollisionDamageThreshold))
    (Development|PrintString (Utilities|String|ToString(Float) _returnvalue_2))
    (Game|Damage|ApplyDamage self _returnvalue_2 0 0)))

(event Custom|InvulnTimer
  (Variables|Default|SetbCanBeDamaged true)
  (Development|PrintString "invulnerability over"))

(event EventBeginPlay
  (bind _returnvalue (Transformation|GetActorTransform))
  (bind _weapons (Variables|Default|GetWeapons))
  (bind _returnvalue_2 (UserInterface|CreateWidget "/Game/HUD/GameplayHUD.GameplayHUD_C"))
  (Variables|Default|SetHUD _returnvalue_2)
  (UserInterface|Viewport|AddtoViewport _returnvalue_2 0)
  (bind _returnvalue_3 (UserInterface|CreateWidget "/Game/HUD/Minimap.Minimap_C"))
  (bind _output_get (Variables|Default|SetMinimap _returnvalue_3))
  (UserInterface|Viewport|AddtoViewport _output_get 0)
  (bind _returnvalue_4 (UserInterface|CreateWidget "/Game/HUD/MinimapMarker.MinimapMarker_C"))
  (bind _output_get_2 (Variables|Default|SetMinimapMarker _returnvalue_4))
  (UserInterface|Viewport|AddtoViewport _output_get_2 0)
  (Variables|Gameplay|SetEnergy (Variables|Gameplay|GetMaxEnergy))
  (bind _returnvalue_5 (Game|SpawnActorfromClass (Variables|Default|GetWeapon1) _returnvalue "Undefined" 0 self 0))
  (Utilities|Array|Add _weapons _returnvalue_5)
  (bind _returnvalue_6 (Game|SpawnActorfromClass (Variables|Default|GetWeapon2) _returnvalue "Undefined" 0 self 0))
  (Utilities|Array|Add _weapons _returnvalue_6)
  (Class|Actor|AttachRootComponenttoActor _returnvalue_6 self "None" "SnapToTarget" true))

(event Game|Damage|EventAnyDamage
  (params (Damage :type Float%20%28single-precision%29) (DamageType :type Damage%20Type%20Object%20Reference) (InstigatedBy :type Controller%20Object%20Reference) (DamageCauser :type Actor%20Object%20Reference))
  (if (Variables|Default|GetbCanBeDamaged)
    (Variables|Default|SetbCanBeDamaged false)
    (Utilities|Time|SetTimerbyEvent (delegate Custom|InvulnTimer) (Variables|Gameplay|GetInvulnTime))
    (bind _output_get (Variables|Default|SetHullIntegrity (- (Variables|Default|GetHullIntegrity) Damage)))
    (Default|SetStructuralIntegrity (Variables|Default|GetHUD) true (/ (Variables|Default|GetHullIntegrity) (Variables|Default|GetMaxHullIntegrity)))
    (if (<= _output_get 0.0)
      (Development|PrintString "dead :("))))

(event EventTick
  (params (DeltaSeconds :type Float%20%28single-precision%29))
  (bind _energy (Variables|Gameplay|GetEnergy))
  (bind _maxenergy (Variables|Gameplay|GetMaxEnergy))
  (|CallParentFunction DeltaSeconds)
  (if (< _energy _maxenergy)
    (CallFunction|ChangeEnergy (- (Math|Interpolation|FInterptoConstant _energy _maxenergy DeltaSeconds (Variables|Default|GetEnergyInterpSpeed)) _energy))))

(fn ConstructionScript)

(fn GetTargetingSolutionPrecise
  (params (TargetActor :type Actor%20Object%20Reference))
  (bind (_predictedaimvector _predictedtargetrelativeposition _timetotarget) (Class|CVectorUtility|GetAimDirectionPrecise (Transformation|GetActorLocation) (Transformation|GetActorLocation TargetActor) (- (Transformation|GetVelocity TargetActor) (Transformation|GetVelocity)) (Variables|Default|GetProjectileSpeed)))
  (return _predictedaimvector _predictedtargetrelativeposition _timetotarget))

(fn DebugDisplayTargetingSolution
  (params (TargetActor :type Actor%20Object%20Reference) (PredictedAimVector :type Vector) (PredictedTargetRelativePosition :type Vector) (TimeToTarget :type Float%20%28single-precision%29))
  (bind _returnvalue (Transformation|GetActorLocation TargetActor))
  (bind _returnvalue_2 (Transformation|GetActorLocation))
  (if (Math|Vector|NotEqual(Vector) PredictedAimVector "0, 0, 0" 0.0001)
    (bind _radialoffsetvector (Class|CVectorUtility|GetTargetRadialOffsetVector PredictedAimVector (Transformation|GetActorLocation) _returnvalue))
    (Rendering|Debug|DrawDebugLine _returnvalue_2 (+ _returnvalue_2 (* PredictedAimVector (* TimeToTarget (Variables|Default|GetProjectileSpeed)))) "(R=0.085000,G=0.000000,B=0.000000,A=0.300000)" 0.0 9.0)
    (Rendering|Debug|DrawDebugLine _returnvalue_2 (+ _returnvalue_2 (* PredictedAimVector 1e+02)) "(R=1.000000,G=0.000000,B=0.000000,A=1.000000)" 0.0 1e+01)
    (Rendering|Debug|DrawDebugLine _returnvalue PredictedTargetRelativePosition "(R=1.000000,G=0.411957,B=0.000000,A=1.000000)" 0.0 1e+01)
    (Rendering|Debug|DrawDebugLine _returnvalue _radialoffsetvector "(R=1.000000,G=0.707986,B=0.000000,A=1.000000)" 0.0 1e+01)
    (Development|PrintString (Utilities|String|BuildString(Float) "" "Time to target: " TimeToTarget "s") true true "(R=0.000000,G=0.660000,B=1.000000,A=1.000000)" 0.0)
    (else
      (Development|PrintString "No valid solution" true true "(R=0.000000,G=0.660000,B=1.000000,A=1.000000)" 0.0))))

(fn GetTargetingSolutionIterative
  (params (TargetActor :type Actor%20Object%20Reference) (Iterations :type Integer))
  (bind _projectiletimetotarget (Variables|Default|GetProjectileTimeToTarget))
  (bind (_predictedaimvector _predictedtargetrelativeposition) (Class|CVectorUtility|GetAimDirectionIterative (Transformation|GetActorLocation) (Transformation|GetActorLocation TargetActor) (- (Transformation|GetVelocity) (Transformation|GetVelocity)) (+ "0, 0, 0" "0, 0, 0") (Variables|Default|GetProjectileSpeed) Iterations _projectiletimetotarget))
  (return _predictedaimvector _predictedtargetrelativeposition _projectiletimetotarget))

(fn TestLineIntersection
  (bind _a1 (LocalVariables|Geta1))
  (bind _a2 (LocalVariables|Geta2))
  (bind _b1 (LocalVariables|Getb1))
  (bind _b2 (LocalVariables|Getb2))
  (bind _intersectionpoint (Class|CVectorUtility|LineLineIntersection _a1 _a2 _b1 _b2))
  (Rendering|Debug|DrawDebugLine (Math|Conversions|ToVector(Vector2D) _a1) (Math|Conversions|ToVector(Vector2D) _a2) "(R=1.000000,G=0.000000,B=0.000000,A=1.000000)" 0.0 5.0)
  (Rendering|Debug|DrawDebugLine (Math|Conversions|ToVector(Vector2D) _b1) (Math|Conversions|ToVector(Vector2D) _b2) "(R=1.000000,G=0.000000,B=0.000000,A=1.000000)" 0.0 5.0)
  (Rendering|Debug|DrawDebugPoint (Math|Conversions|ToVector(Vector2D) _intersectionpoint) 1e+01 "(R=1.000000,G=0.000000,B=0.000000,A=1.000000)" 0.0))

(fn FireWeapon
  (params (WeaponSlot :type Integer))
  (Default|Fire (Utilities|Array|Get(acopy) (Variables|Default|GetWeapons) WeaponSlot) (+ (Transformation|GetVelocity) (* (+ (Transformation|GetActorForwardVector) (* (Math|Random|RandomUnitVector) 0.03)) 1.55e+03))))

(fn Repair
  (params (RepairAmount :type Float%20%28single-precision%29))
  (bind _output_get (Variables|Default|SetHullIntegrity (Math|Float|Min(Float) (+ RepairAmount (Variables|Default|GetHullIntegrity)) (Variables|Default|GetMaxHullIntegrity))))
  (Default|SetStructuralIntegrity (Variables|Default|GetHUD) false _output_get))

(fn ChangeEnergy
  (params (Change :type Float%20%28single-precision%29))
  (bind _output_get (Variables|Gameplay|SetEnergy (Math|Float|Min(Float) (+ Change (Variables|Gameplay|GetEnergy)) (Variables|Gameplay|GetMaxEnergy))))
  (Default|SetEnergy (Variables|Default|GetHUD) (/ _output_get (Variables|Gameplay|GetMaxEnergy))))

(fn GetNextWeapon
  (bind _activeweaponslot (Variables|Default|GetActiveWeaponSlot))
  (bind _weapons (Variables|Default|GetWeapons))
  (bind _returnvalue (Utilities|Array|Length _weapons))
  (bind _returnvalue_2 (+ _activeweaponslot 1))
  (bind _returnvalue_3 (Math|Integer|%(Integer) _returnvalue_2 _returnvalue))
  (return (Utilities|Array|Get(acopy) _weapons _returnvalue_3) _returnvalue_3))