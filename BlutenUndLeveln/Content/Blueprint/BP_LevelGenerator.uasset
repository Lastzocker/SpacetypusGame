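; BP_LevelGenerator is an actor that builds a level's sector and room data at BeginPlay and lists the rooms on the HUD.
; It spawns a BP_Sector with a random size within configured limits, then fills it with that many BP_Room actors, all spawned at the origin.
; The first sector becomes current, and each of its rooms gets a RoomButton in the player pawn's LevelGeneratorHUD.
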(event EventBeginPlay
  (CallFunction|GenerateSector)
  (CallFunction|SetStartSector)
  (CallFunction|FillRoomHUD))

(event EventActorBeginOverlap
  (params (OtherActor :type Actor%20Object%20Reference)))

(event EventTick
  (params (DeltaSeconds :type Float%20%28single-precision%29)))

(fn ConstructionScript)

(fn GenerateSector
  ;[1 1 1] Spawns the Actor and adds it to Sectors Array
  (bind _returnvalue (Game|SpawnActorfromClass "/Game/Blueprint/BP_Sector.BP_Sector_C" (Math|Transform|MakeTransform "0, 0, 0") "AlwaysSpawn" 0 (Math|Random|RandomIntegerinRange (Variables|Default|GetMinRooms) (Variables|Default|GetMaxRooms)) 0))
  (Utilities|Array|Add (Variables|Default|GetSectors) _returnvalue)
  (CallFunction|GenerateSectorRooms _returnvalue))

(fn FillRoomHUD
  (bind _asbp_bluten_und_leveln_pawn (Utilities|Casting|CastToBP_BlutenUndLevelnPawn (Game|Player|GetPlayerPawn 0)))
  (for _array_element (Variables|/Game/Blueprint/BP_Sector.BP_Sector_C|GetRooms (Variables|Default|GetCurrentSector))
    (bind _returnvalue (UserInterface|CreateWidget "/Game/HUD/RoomButton.RoomButton_C"))
    (Rendering|Components|TextRender|SetText (Variables|/Game/HUD/RoomButton.RoomButton_C|GetRoomName _returnvalue) (Utilities|Text|ToText(String) (Utilities|GetDisplayName _array_element)))
    (Class|VerticalBox|AddChildtoVerticalBox (Variables|/Game/HUD/LevelGeneratorHUD.LevelGeneratorHUD_C|GetBox (Variables|/Game/HUD/GameplayHUD.GameplayHUD_C|GetLevelGeneratorHUD (Variables|/Game/Blueprint/BP_BlutenUndLevelnPawn.BP_BlutenUndLevelnPawn_C|GetHUD _asbp_bluten_und_leveln_pawn))) _returnvalue)))

(fn SetStartSector
  (Variables|Default|SetCurrentSector (Utilities|Array|Get(acopy) (Variables|Default|GetSectors))))

(fn GenerateSectorRooms
  (params (Sector :type BP%20Sector%20Object%20Reference))
  (for _index (range 0 (- (Variables|/Game/Blueprint/BP_Sector.BP_Sector_C|GetSize Sector) 1))
    (bind _returnvalue (Game|SpawnActorfromClass "/Game/Blueprint/BP_Room.BP_Room_C" (Math|Transform|MakeTransform "0, 0, 0") "Undefined" 0 0))
    (Utilities|Array|Add (Variables|/Game/Blueprint/BP_Sector.BP_Sector_C|GetRooms Sector) _returnvalue)))