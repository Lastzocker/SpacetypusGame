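; BP_MainMenuScene is the main menu backdrop Blueprint that slowly orbits or pans the player camera.
; On BeginPlay it attaches the PlayerCamera actor to CameraRoot, keeping its world position, then sets the root to a fixed starting yaw.
; Each Tick adds delta time to CameraRoot's yaw, giving a steady frame-rate-independent turn that carries the attached camera with it.
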(event EventBeginPlay
  (Class|Actor|AttachRootComponentto (Variables|Default|GetPlayerCamera) (Variables|Default|GetCameraRoot) "None" "KeepWorldPosition" true)
  (Transformation|SetWorldRotation (Variables|Default|GetCameraRoot) (Math|Rotator|MakeRotator 0.0 0.0 7e+01) false false))

(event Collision|EventActorBeginOverlap
  (params (OtherActor :type Actor%20Object%20Reference)))

(event EventTick
  (params (DeltaSeconds :type Float%20%28single-precision%29))
  (bind _cameraroot (Variables|Default|GetCameraRoot))
  (Transformation|SetWorldRotation _cameraroot (Math|Rotator|MakeRotator 0.0 0.0 (+ (* DeltaSeconds 1.0) (.yaw (Transformation|GetWorldRotation _cameraroot)))) false false))

(fn ConstructionScript)