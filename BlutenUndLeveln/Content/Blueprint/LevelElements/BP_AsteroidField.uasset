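; BP_AsteroidField is a level actor that fills a flat disc-sized area around itself with BP_AsteroidObject actors on BeginPlay.
; The asteroid count comes from the circle area of Radius divided by AverageSpace squared.
; Index-driven Perlin noise using the GameInstance seed sets X/Y offsets at the actor's height, and its random stream sets rotation.
; Each asteroid gets a mesh from AsteroidMeshes via unseeded random selection.
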(event EventBeginPlay
  (CallFunction|CreateField))

(event EventActorBeginOverlap
  (params (OtherActor :type Actor%20Object%20Reference)))

(event EventTick
  (params (DeltaSeconds :type Float%20%28single-precision%29)))

(fn ConstructionScript)

(fn CreateField
  (bind _returnvalue (Transformation|GetActorLocation))
  (bind _asbp_game_instance (Utilities|Casting|CastToBP_GameInstance (Game|GetGameInstance)))
  (LocalVariables|SetSeed (Variables|/Game/Blueprint/BP_GameInstance.BP_GameInstance_C|GetCustomRandomSeed _asbp_game_instance))
  (LocalVariables|SetStream (Variables|/Game/Blueprint/BP_GameInstance.BP_GameInstance_C|GetCustomRandomStream _asbp_game_instance))
  (for _index (range 1 (Math|Float|Truncate (|(((pi*r)*r)/(a*a)) 3.1415 (Variables|Default|GetRadius) (Variables|Default|GetAverageSpace))))
    (CallFunction|SpawnRandomAsteroid (Math|Transform|MakeTransform (Math|Vector|MakeVector (+ (.x _returnvalue) (* (Variables|Default|GetRadius) (Class|CPerlinNoiseUtility|PerlinGetValuePrecise (Math|Conversions|ToFloat(Integer) (* _index 15)) 8.0 67.0 10.649 2.0 "QUALITY_BEST" 6 0.657 (LocalVariables|GetSeed)))) (+ (.y _returnvalue) (* (Variables|Default|GetRadius) (Class|CPerlinNoiseUtility|PerlinGetValuePrecise 18.0 (Math|Conversions|ToFloat(Integer) (* _index 15)) 59.0 15.67 3.0 "QUALITY_BEST" 6 0.657 (LocalVariables|GetSeed)))) (.z _returnvalue)) (Class|KismetMathLibrary|RandomRotatorfromStream true (LocalVariables|GetStream)) "1,1,1.000000"))))

(fn SpawnRandomAsteroid
  (params (Transform :type Transform))
  (bind _asteroidmeshes (Variables|Default|GetAsteroidMeshes))
  (bind _returnvalue (Game|SpawnActorfromClass "/Game/Blueprint/LevelElements/BP_AsteroidObject.BP_AsteroidObject_C" (Math|Transform|MakeTransform (.location Transform) (.rotation Transform) "1,1,1") "AdjustIfPossibleButAlwaysSpawn" 0 0))
  (Components|StaticMesh|SetStaticMesh (Variables|/Game/Blueprint/LevelElements/BP_AsteroidObject.BP_AsteroidObject_C|GetStaticMesh _returnvalue) (Utilities|Array|Get(acopy) _asteroidmeshes (Math|Random|RandomIntegerinRange 0 (- (Utilities|Array|Length _asteroidmeshes) 1)))))