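; Beacon level element with a slowly rollable mesh, detection-driven markers and an interaction trigger.
; Construction and BeginPlay flatten the actor's height and place the mesh at Depth; BeginPlay also orients it near the first directional light's rotation with random jitter, and Tick spins its roll.
; BeginPlay creates a HUD_Beacon and caches both widgets.
; OnDetect and OnLostContact show or hide marker and interaction zone; player pawn overlap toggles marker info.
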(event OnComponentBeginOverlap(InteractionTrigger)
  (params (OtherActor :type Actor%20Object%20Reference) (OtherComp :type Primitive%20Component%20Object%20Reference) (OtherBodyIndex :type Integer) (bFromSweep :type Boolean) (SweepResult :type Hit%20Result%20Structure%20%28by%20ref%29))
  (Utilities|Casting|CastToBP_BlutenUndLevelnPawn OtherActor)
  (Default|PlayShowInfoAnim (Variables|Default|GetMarker)))

(event OnComponentEndOverlap(InteractionTrigger)
  (params (OtherActor :type Actor%20Object%20Reference) (OtherComp :type Primitive%20Component%20Object%20Reference) (OtherBodyIndex :type Integer))
  (Utilities|Casting|CastToBP_BlutenUndLevelnPawn OtherActor)
  (Default|PlayHideInfoAnim (Variables|Default|GetMarker)))

(event EventBeginPlay
  (bind _returnvalue (Transformation|GetActorLocation))
  (bind _returnvalue_2 (Transformation|GetActorLocation))
  (bind _returnvalue_3 (Math|Random|RandomFloatinRange -2e+01 2e+01))
  (Transformation|SetWorldLocation (Variables|Default|GetBeaconMesh) (Math|Vector|MakeVector (.x _returnvalue) (.y _returnvalue) (Variables|Default|GetDepth)) false false)
  (Transformation|SetActorLocation (Math|Vector|MakeVector (.x _returnvalue_2) (.y _returnvalue_2) 0.0) false false)
  (bind _outactors (Actor|GetAllActorsOfClass "/Script/Engine.DirectionalLight")) ; Get first directional light in the level
  (Transformation|SetWorldRotation (Variables|Default|GetBeaconMesh) (Math|Rotator|MakeRotator (+ (.roll (Transformation|GetWorldRotation (Variables|/Script/Engine.Light|GetLightComponent (Utilities|Array|Get(acopy) _outactors)))) _returnvalue_3) (+ (.pitch (Transformation|GetWorldRotation (Variables|/Script/Engine.Light|GetLightComponent (Utilities|Array|Get(acopy) _outactors)))) _returnvalue_3) (+ (.yaw (Transformation|GetWorldRotation (Variables|/Script/Engine.Light|GetLightComponent (Utilities|Array|Get(acopy) _outactors)))) _returnvalue_3)) false false)
  (bind _returnvalue_4 (UserInterface|CreateWidget "/Game/HUD/HUD_Beacon.HUD_Beacon_C" (Game|GetPlayerController 0)))
  (Variables|/Game/HUD/HUD_Beacon.HUD_Beacon_C|SetBeacon _returnvalue_4 self)
  (UserInterface|Viewport|AddtoViewport _returnvalue_4 0)
  (bind _ashud_beacon_marker (Utilities|Casting|CastToHUD_BeaconMarker (UserInterface|GetUserWidgetObject (Variables|Default|GetMarkerWidget))))
  (Variables|Default|SetMarker _ashud_beacon_marker)
  (bind _ashud_interaction_zone (Utilities|Casting|CastToHUD_InteractionZone (UserInterface|GetUserWidgetObject (Variables|Default|GetInteractionZoneWidget))))
  (Variables|Default|SetInteractionZone _ashud_interaction_zone))

(event EventActorBeginOverlap
  (params (OtherActor :type Actor%20Object%20Reference)))

(event EventTick
  (params (DeltaSeconds :type Float%20%28single-precision%29))
  (bind _beaconmesh (Variables|Default|GetBeaconMesh))
  (bind _relativerotation (Variables|/Script/Engine.SceneComponent|GetRelativeRotation _beaconmesh))
  (Transformation|SetRelativeRotation _beaconmesh (Math|Rotator|MakeRotator (+ (* DeltaSeconds (Variables|Default|GetRotationSpeed)) (.roll _relativerotation)) (.pitch _relativerotation) (.yaw _relativerotation)) false false))

(event EventOnDetect
  (Default|PlayShowAnim (Variables|Default|GetMarker))
  (Default|PlayShowAnim (Variables|Default|GetInteractionZone)))

(event EventOnLostContact
  (Default|PlayHideAnim (Variables|Default|GetMarker))
  (Default|PlayHideAnim (Variables|Default|GetInteractionZone)))

(fn ConstructionScript
  (bind _returnvalue (Transformation|GetActorLocation))
  (bind _returnvalue_2 (Transformation|GetActorLocation))
  (Transformation|SetWorldLocation (Variables|Default|GetBeaconMesh) (Math|Vector|MakeVector (.x _returnvalue) (.y _returnvalue) (Variables|Default|GetDepth)) false false)
  (Transformation|SetActorLocation (Math|Vector|MakeVector (.x _returnvalue_2) (.y _returnvalue_2) 0.0) false false))