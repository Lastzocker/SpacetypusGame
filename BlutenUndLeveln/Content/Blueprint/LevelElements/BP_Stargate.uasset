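; BP_Stargate is a level element actor with three parts that spin continuously.
; On Tick, each part's relative yaw advances by delta time times its own constant rate, with Part1 fastest and Part3 slowest, while pitch and roll stay unchanged.
; The construction script is empty and there is no overlap or gameplay logic, so the file shows only this rotation.
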(event EventBeginPlay)

(event EventActorBeginOverlap
  (params (OtherActor :type Actor%20Object%20Reference)))

(event EventTick
  (params (DeltaSeconds :type Float%20%28single-precision%29))
  (bind _part1 (Variables|Default|GetPart1))
  (bind _part2 (Variables|Default|GetPart2))
  (bind _part3 (Variables|Default|GetPart3))
  (bind _relativerotation (Variables|/Script/Engine.SceneComponent|GetRelativeRotation _part3))
  (bind _relativerotation_2 (Variables|/Script/Engine.SceneComponent|GetRelativeRotation _part1))
  (bind _relativerotation_3 (Variables|/Script/Engine.SceneComponent|GetRelativeRotation _part2))
  (Utilities|FlowControl|Sequence
    (:then_0
      (Transformation|SetRelativeRotation _part1 (Math|Rotator|MakeRotator (.roll _relativerotation_2) (.pitch _relativerotation_2) (+ (* DeltaSeconds 2.0) (.yaw _relativerotation_2))) false false))
    (:then_1
      (Transformation|SetRelativeRotation _part2 (Math|Rotator|MakeRotator (.roll _relativerotation_3) (.pitch _relativerotation_3) (+ (* DeltaSeconds 1.0) (.yaw _relativerotation_3))) false false))
    (:then_2
      (Transformation|SetRelativeRotation _part3 (Math|Rotator|MakeRotator (.roll _relativerotation) (.pitch _relativerotation) (+ (* DeltaSeconds 0.5) (.yaw _relativerotation))) false false))))

(fn ConstructionScript)