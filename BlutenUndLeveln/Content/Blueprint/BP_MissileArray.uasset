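; BP_MissileArray is a ship weapon that fires missile projectiles from a given muzzle.
; LaunchProjectile requires a positive MaxAmmo and a successful HandleMissiles call on OwningShip, unless the ship has infinite ammo and energy.
; It spawns the projectile, launches it with random yaw spread and critical-evaluated damage, then plays muzzle effect and sound.
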(event EventBeginPlay
  (|CallParentFunction))

(event EventActorBeginOverlap
  (params (OtherActor :type Actor%20Object%20Reference)))

(event EventTick
  (params (DeltaSeconds :type Float%20%28single-precision%29)))

(event EventLaunchProjectile
  (params (Muzzle :type Scene%20Component%20Object%20Reference) (Velocity :type Vector))
  (bind _owningship (Variables|Default|GetOwningShip))
  (bind _owningship_2 (Variables|Default|GetOwningShip))
  (bind _projectilespread (Variables|Default|GetProjectileSpread))
  ;[1 1 1] Check if shooting is possible
  (if (not (Variables|/Game/Blueprint/BP_BlutenUndLevelnPawn.BP_BlutenUndLevelnPawn_C|GetHasInfiniteAmmoAndEnergy _owningship_2))
    (if (> (Variables|Default|GetMaxAmmo) 0)
      (bind _successful (Default|HandleMissiles _owningship_2))
      (if _successful
        (bind _returnvalue (Game|SpawnActorfromClass (Variables|Default|GetProjectile) (Transformation|GetWorldTransform Muzzle) "AlwaysSpawn" 0 _owningship _owningship :!label _label))
        (Utilities|IsValid _returnvalue
          (:Is%20Valid
            (bind (_iscritical _damage) (CallFunction|EvaluateCritical))
            (Default|Launch _returnvalue (Math|Vector|RotateVector Velocity (Math|Rotator|MakeRotator 0.0 0.0 (Math|Random|RandomFloatinRange (* _projectilespread -1.0) _projectilespread))) _damage _iscritical)
            (Effects|SpawnEmitterAttached (Variables|Default|GetMuzzleEffect) Muzzle "None" "0, 0, 0" "0, 0, 0" "SnapToTarget")
            (Audio|PlaySoundatLocation (Variables|Default|GetMuzzleSound) (Transformation|GetWorldLocation Muzzle) "0, 0, 0" 0.05 (Variables|Default|GetSoundPitch))))))
    (else
      (goto _label))))

(fn ConstructionScript
  (|CallParentFunction))