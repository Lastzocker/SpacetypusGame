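; BP_C_PlayerTarget is a component that marks its owning actor as a target on the player's HUD.
; Enable and disable functions add or remove the owner through the HUD component on player controller 0, optionally enabling on BeginPlay and always disabling on EndPlay.
; Targets can start unknown with a generic, non-hostile icon until SetKnown applies the real icon and hostility to the stored marker.
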(event EventBeginPlay
  (if (Variables|Config|GetStartEnabled)
    (CallFunction|EnableTarget)))

(event EventTick
  (params (DeltaSeconds :type Float%20%28single-precision%29)))

(event EventEndPlay
  (params (EndPlayReason :type EEndPlayReason%20Enum :default "Destroyed"))
  (CallFunction|DisableTarget))

(fn DisableTarget
  (if (Variables|Default|GetIsEnabled)
    (Variables|Default|SetIsEnabled false)
    (bind _asbp_bu_lplayer_controller (Utilities|Casting|CastToBP_BuLPlayerController (Game|GetPlayerController 0)))
    (Default|RemoveTarget (Variables|/Game/Blueprint/BP_BuLPlayerController.BP_BuLPlayerController_C|GetBP_C_PlayerHUD _asbp_bu_lplayer_controller) (Components|GetOwner))))

(fn EnableTarget
  (bind _returnvalue (Components|GetOwner))
  (if (not (Variables|Default|GetIsEnabled))
    (Variables|Default|SetIsEnabled true)
    (bind _asbp_bu_lplayer_controller (Utilities|Casting|CastToBP_BuLPlayerController (Game|GetPlayerController 0)))
    (if (Variables|Config|GetStartUnknown)
      (bind _targetdirectionmarker (Default|AddTarget (Variables|/Game/Blueprint/BP_BuLPlayerController.BP_BuLPlayerController_C|GetBP_C_PlayerHUD _asbp_bu_lplayer_controller) _returnvalue "/Game/HUD/HUDTextures/Icons/TEX_HUD_Icon_UnknownObject_64.TEX_HUD_Icon_UnknownObject_64" false))
      (Variables|Config|SetMarker _targetdirectionmarker)
      (else
        (bind _targetdirectionmarker_2 (Default|AddTarget (Variables|/Game/Blueprint/BP_BuLPlayerController.BP_BuLPlayerController_C|GetBP_C_PlayerHUD _asbp_bu_lplayer_controller) _returnvalue (Variables|Config|GetIcon) (Variables|Config|GetIsHostile)))
        (Variables|Config|SetMarker _targetdirectionmarker_2)))))

(fn SetKnown
  (bind _marker (Variables|Config|GetMarker))
  (Default|SetIcon _marker (Variables|Config|GetIcon))
  (Default|SetHostile _marker (Variables|Config|GetIsHostile)))