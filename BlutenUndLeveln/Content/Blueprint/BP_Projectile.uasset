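; BP_Projectile is a launchable kinetic projectile that ignores collision with the player's ship, spawns hit effects and destroys itself on overlap.
; Launch sets the ProjectileMovement velocity, and the mesh overlap triggers Hit.
; An optional short forward trace refines the effect location and orients it along the inverted reflection vector, falling back to the actor transform.
; Critical hits get their own emitter; otherwise a failed trace selects ricochet over standard impact.
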(event OnComponentBeginOverlap(StaticMesh)
  (params (OtherActor :type Actor%20Object%20Reference) (OtherComp :type Primitive%20Component%20Object%20Reference) (OtherBodyIndex :type Integer) (bFromSweep :type Boolean) (SweepResult :type Hit%20Result%20Structure%20%28by%20ref%29))
  (CallFunction|Hit))

(event EventBeginPlay
  (bind _returnvalue (Game|Player|GetPlayerPawn 0))
  (Collision|IgnoreActorwhenMoving (Variables|Default|GetStaticMesh) _returnvalue true)
  (bind _asbluten_und_leveln_pawn (Utilities|Casting|CastToBlutenUndLevelnPawn _returnvalue))
  (Collision|IgnoreActorwhenMoving (Variables|/Script/BlutenUndLeveln.BlutenUndLevelnPawn|GetShipMeshComponent _asbluten_und_leveln_pawn) self true))

(event EventActorBeginOverlap
  (params (OtherActor :type Actor%20Object%20Reference)))

(event EventTick
  (params (DeltaSeconds :type Float%20%28single-precision%29)))

(fn ConstructionScript)

(fn Launch
  (params (Velocity :type Vector))
  (Variables|/Script/Engine.MovementComponent|SetVelocity (Variables|Default|GetProjectileMovement) Velocity))

(fn Hit
  (bind _superficial (CallFunction|FindHitLocRot))
  (CallFunction|DisplayHitFX _superficial)
  (Actor|DestroyActor))

(fn DisplayHitFX
  (params (Alternative :type Boolean))
  (bind _effectlocation (Variables|Default|GetEffectLocation))
  (bind _effectrotation (Variables|Default|GetEffectRotation))
  (if (Variables|Default|GetIsCritical)
    (Effects|SpawnEmitteratLocation "/Game/Effects/Projectiles/FX_Impact_Kinetic_Critical.FX_Impact_Kinetic_Critical" _effectlocation _effectrotation)
    (elif Alternative
      (Effects|SpawnEmitteratLocation "/Game/Effects/Projectiles/FX_Ricochet_Kinetic_Standard.FX_Ricochet_Kinetic_Standard" _effectlocation _effectrotation)
      (else
        (Effects|SpawnEmitteratLocation "/Game/Effects/Projectiles/FX_Impact_Kinetic_Standard.FX_Impact_Kinetic_Standard" _effectlocation _effectrotation)))))

(fn FindAccurateHitResult
  (bind _returnvalue (Transformation|GetActorLocation))
  (bind (_outhit _returnvalue_2) (Collision|LineTraceByChannel _returnvalue (+ _returnvalue (* (Transformation|GetActorForwardVector) 1e+02)) "TraceTypeQuery1" false 0 "None"))
  (return _outhit _returnvalue_2))

(fn FindHitLocRot
  (if (Variables|Default|GetGetAccurateHitResult) ; Whether to check for accurate Hit-Information
    (bind (_hitresult _hitfound) (CallFunction|FindAccurateHitResult))
    (if _hitfound ; Hit something?
      (bind _reflectedvector (Class|CVectorUtility|GetReflectionVector (Transformation|GetActorForwardVector) (.ImpactNormal (Collision|BreakHitResult _hitresult))))
      (Variables|Default|SetEffectLocation (.ImpactPoint (Collision|BreakHitResult _hitresult)))
      (Variables|Default|SetEffectRotation (Math|Conversions|RotationFromXVector (* _reflectedvector -1.0)))
      (else
        (Variables|Default|SetEffectLocation (Transformation|GetActorLocation) :!label _label)
        (Variables|Default|SetEffectRotation (Math|Conversions|RotationFromXVector (Transformation|GetActorForwardVector)))))
    (else
      (goto _label)))
  (return (not _hitfound)))