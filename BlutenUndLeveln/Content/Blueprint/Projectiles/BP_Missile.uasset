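; Homing missile projectile that launches with physics, then after a start delay fires its engine and accelerates until burnout.
; Player missiles seek the nearest other ship, others seek the player, steering by iterative lead prediction and optionally losing lock on overshoot.
; Overlaps filter out same-side ships, then apply direct or radial damage with hit effects.
; Gates control thrust and tracking, shutting down before delayed destruction; self-destruct spawns an explosion.
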(event OnComponentBeginOverlap(ProjectileMesh)
  (params (OtherActor :type Actor%20Object%20Reference) (OtherComp :type Primitive%20Component%20Object%20Reference) (OtherBodyIndex :type Integer) (bFromSweep :type Boolean) (SweepResult :type Hit%20Result%20Structure%20%28by%20ref%29))
  ;[1 1 1] Hit
  (CallFunction|Hit OtherActor))

(event Custom|Deactivate
  ;[1 1 1] Deactivate
  (Variables|/Script/Engine.PrimitiveComponent|SetbGenerateOverlapEvents (Variables|Default|GetProjectileMesh) false)
  (Components|Activation|Deactivate (Variables|Default|GetFX_RocketEngine_Small))
  (Rendering|SetVisibility (Variables|Default|GetProjectileMesh) false false)
  (Variables|Default|SetHasExploded true)
  (Utilities|FlowControl|Sequence
    (:then_0
      ;[1 1 1] Tick
      (Utilities|FlowControl|Gate false) ; enters at Close
    )
    (:then_1
      (Utilities|FlowControl|Delay 1.0)
      (Actor|DestroyActor))))

(event EventBeginPlay
  ;[1 1 1] BeginPlay
  (|CallParentFunction)
  (Variables|Default|SetPositionAtLaunch (Transformation|GetWorldLocation (Variables|Default|GetProjectileMesh)))
  (Components|Activation|Deactivate (Variables|Default|GetProjectileMovement))
  (CallFunction|FindTarget)
  (Utilities|FlowControl|Delay (Variables|Default|GetStartDelay))
  (if (not (Variables|Default|GetHasExploded))
    (Components|Activation|Activate (Variables|Default|GetFX_RocketEngine_Small) false)
    (Utilities|FlowControl|Sequence
      (:then_0
        ;[1 1 1] Tick
        (Utilities|FlowControl|Gate true) ; enters at Open
      )
      (:then_1
        (Utilities|FlowControl|Delay (Variables|Default|GetBurnTime))
        (if (not (Variables|Default|GetHasExploded))
          (Components|Activation|Deactivate (Variables|Default|GetFX_RocketEngine_Small))
          (Utilities|FlowControl|Gate true) ; enters at Close
        )))))

(event EventTick
  (params (DeltaSeconds :type Float%20%28single-precision%29))
  ;[1 1 1] Tick
  (Utilities|FlowControl|Gate false
    (:Exit
      (if (Variables|Default|GetIsDumb)
        _
        (else
          (CallFunction|TrackTarget)))
      (Utilities|FlowControl|Gate true
        (:Exit
          (CallFunction|Accelerate DeltaSeconds))))))

(event EventLaunch
  (params (Velocity :type Vector) (Damage :type Float%20%28single-precision%29) (IsCritical :type Boolean))
  ;[1 1 1] Launch
  (|CallParentFunction Velocity Damage IsCritical)
  (Physics|SetSimulatePhysics (Variables|Default|GetProjectileMesh) true)
  (Physics|SetPhysicsLinearVelocity (Variables|Default|GetProjectileMesh) Velocity false "None"))

(event EventHit
  (params (HitActor :type Actor%20Object%20Reference))
  (bind _returnvalue (Game|Player|GetPlayerPawn 0))
  (bind _areaofeffectradius (Variables|Default|GetAreaOfEffectRadius))
  (bind _projectiledamage (Variables|Default|GetProjectileDamage))
  ;[1 1 1] Hit
  (Utilities|Casting|CastToBP_BlutenUndLevelnPawn HitActor
    (:then
      (if (Math|Boolean|NotEqual(Boolean) (!= (Variables|Default|GetOwningActor) _returnvalue) (!= _returnvalue HitActor))
        (bind _superficial (CallFunction|FindHitLocRot :!label _label))
        (CallFunction|DisplayHitFX _superficial HitActor)
        (if (Variables|Default|GetHasAreaOfEffect)
          (Class|GameplayStatics|ApplyRadialDamagewithFalloff _projectiledamage (/ _projectiledamage 4.0) (Transformation|GetWorldLocation (Variables|Default|GetProjectileMesh)) (/ _areaofeffectradius 4.0) _areaofeffectradius 2.0 (Variables|Default|GetDamageType) 0 0 0 "ECC_GameTraceChannel3")
          (else
            (Game|Damage|ApplyDamage HitActor (Variables|Default|GetProjectileDamage) (Game|GetInstigatorController) 0 (Variables|Default|GetDamageType))))
        (CallFunction|Deactivate)
        (Physics|SetPhysicsLinearVelocity (Variables|Default|GetProjectileMesh) "0.000000, 0, 0" false "None")))
    (:CastFailed
      (goto _label))))

(event EventSelfdestruct
  (bind _projectilemesh (Variables|Default|GetProjectileMesh))
  ;[1 1 1] Selfdestruct
  (if (not (Variables|Default|GetHasExploded))
    (bind _aspawn (Utilities|Casting|CastToPawn (Variables|Default|GetOwningActor)))
    (Game|SpawnActorfromClass "/Game/Blueprint/BP_Explosion.BP_Explosion_C" (Math|Transform|MakeTransform (Transformation|GetWorldLocation _projectilemesh) (Transformation|GetWorldRotation _projectilemesh) "1,1,1") "Undefined" 0 true 0.02 (Transformation|GetComponentVelocity _projectilemesh) (Variables|Default|GetHitFX_Standard) _aspawn)
    (CallFunction|Deactivate)))

(fn ConstructionScript
  (|CallParentFunction))

(fn Accelerate
  (params (DeltaSeconds :type Float%20%28single-precision%29))
  (bind _projectilemesh (Variables|Default|GetProjectileMesh))
  (Physics|SetPhysicsLinearVelocity (Variables|Default|GetProjectileMesh) (+ (- (Transformation|GetComponentVelocity _projectilemesh) (* (Transformation|GetComponentVelocity _projectilemesh) (Variables|Default|GetFlightDamping))) (* (Math|Vector|GetForwardVector _projectilemesh) (* DeltaSeconds (Variables|Default|GetAcceleration)))) false "None"))

(fn TrackTarget
  (bind _targetactor (Variables|Default|GetTargetActor))
  (bind _projectilemesh (Variables|Default|GetProjectileMesh))
  (bind _projectilemesh_2 (Variables|Default|GetProjectileMesh))
  (bind _returnvalue (Transformation|GetComponentVelocity _projectilemesh))
  (if (not (Variables|Default|GetTargetLost))
    (Utilities|IsValid (Variables|Default|GetTargetActor)
      (:Is%20Valid
        (bind _predictedaimvector (Class|CVectorUtility|GetAimDirectionIterative (Transformation|GetWorldLocation _projectilemesh) (Transformation|GetActorLocation _targetactor) (- (Transformation|GetVelocity _targetactor) _returnvalue) (Math|Vector|MakeVector 0.0 0.0 0.0) (Math|Float|Max(Float) (Math|Vector|VectorLength _returnvalue) 1.5e+03) (LocalVariables|GetIterations) (Variables|Default|GetTimeToTarget)))
        (Transformation|SetWorldRotation _projectilemesh_2 (Math|Rotator|Lerp(Rotator) (Transformation|GetWorldRotation _projectilemesh_2) (Math|Conversions|RotationFromXVector _predictedaimvector) (Variables|Default|GetTurnLerpFactor) true) false false)
        (if (Variables|Default|GetLoosesTargetOnOvershoot)
          (Variables|Default|SetTargetLost (< (- (Math|Vector|VectorLength (- (Transformation|GetActorLocation (Variables|Default|GetTargetActor)) (Variables|Default|GetPositionAtLaunch))) (Math|Vector|VectorLength (- (Transformation|GetWorldLocation (Variables|Default|GetProjectileMesh)) (Variables|Default|GetPositionAtLaunch)))) 0.0))))
      (:Is%20Not%20Valid
        (CallFunction|FindTarget)))))

(fn FindTarget
  (bind _returnvalue (Game|GetPlayerController 0))
  (bind _projectilemesh (Variables|Default|GetProjectileMesh))
  (bind _returnvalue_2 (Transformation|GetWorldLocation _projectilemesh))
  (bind _returnvalue_3 (Pawn|GetControlledPawn _returnvalue))
  (bind _asbp_bluten_und_leveln_pawn (Utilities|Casting|CastToBP_BlutenUndLevelnPawn (Variables|Default|GetOwningActor))
    (:then
      (if (Variables|/Game/Blueprint/BP_BlutenUndLevelnPawn.BP_BlutenUndLevelnPawn_C|GetIsPlayerShip _asbp_bluten_und_leveln_pawn) ; If owner is the player, get the closest target, otherwise just target the player
        (bind _outactors (Actor|GetAllActorsOfClass "/Game/Blueprint/BP_BlutenUndLevelnPawn.BP_BlutenUndLevelnPawn_C"))
        (bind _asbp_bluten_und_leveln_pawn_2 (Utilities|Casting|CastToBP_BlutenUndLevelnPawn (Variables|Default|GetOwningActor))
          (:then
            (Utilities|Array|RemoveItem _outactors _asbp_bluten_und_leveln_pawn_2))
          (:CastFailed
            _))
        (for (_array_element _array_index) _outactors
          (Utilities|IsValid (Variables|Default|GetTargetActor)
            (:Is%20Valid
              (if (< (Math|Vector|VectorLength (- (Transformation|GetActorLocation _array_element) _returnvalue_2)) (Math|Vector|VectorLength (- (Transformation|GetActorLocation (Variables|Default|GetTargetActor)) _returnvalue_2)))
                (Variables|Default|SetTargetActor _array_element)))
            (:Is%20Not%20Valid
              (Variables|Default|SetTargetActor (Utilities|Array|Get(acopy) _outactors _array_index)))))
        (Utilities|IsValid (Variables|Default|GetTargetActor)
          (:Is%20Not%20Valid
            (Development|PrintText "No Target Found")
            (Variables|Default|SetIsDumb true)))
        (else
          (Variables|Default|SetTargetActor _returnvalue_3 :!label _label))))
    (:CastFailed
      (Utilities|IsValid _returnvalue_3
        (:Is%20Valid
          (goto _label))
        (:Is%20Not%20Valid
          (Variables|Default|SetIsDumb true))))))