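; Weapon projectile for ship combat that damages what it overlaps, then destroys itself, or fades its material brightness out after its lifetime.
; Pawn and shield hits count only between player and non-player sides; player hits are reported to the controller by weapon class.
; An optional forward trace refines impact location and reflected effect rotation, with effects varying for rock, critical, untraced or standard hits.
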(event OnComponentBeginOverlap(ProjectileMesh)
  (params (OtherActor :type Actor%20Object%20Reference) (OtherComp :type Primitive%20Component%20Object%20Reference) (OtherBodyIndex :type Integer) (bFromSweep :type Boolean) (SweepResult :type Hit%20Result%20Structure%20%28by%20ref%29))
  ;[1 1 1] On Hit
  (CallFunction|ProjectileHit OtherActor))

(event Custom|Selfdestruct
  ;[1 1 1] Fade out and destroy projectile
  (bind _size (Timeline|Timeline_0 PlayFromStart)
    (:Update
      (Rendering|Material|SetScalarParameterValue (Variables|Default|GetProjectileMat) "Brightness" (* _size (Variables|Default|GetBrightness)) :!class /Script/Engine.MaterialInstanceDynamic))
    (:Finished
      (Actor|DestroyActor))))

(event EventBeginPlay
  (bind _projectilemesh (Variables|Default|GetProjectileMesh))
  (bind _owningactor (Variables|Default|GetOwningActor))
  (Utilities|IsValid (Variables|Default|GetOwningActor)
    (:Is%20Valid
      (Collision|IgnoreActorwhenMoving (Variables|Default|GetProjectileMesh) _owningactor true)
      (bind _asbluten_und_leveln_pawn (Utilities|Casting|CastToBlutenUndLevelnPawn _owningactor))
      (Collision|IgnoreActorwhenMoving (Variables|/Script/BlutenUndLeveln.BlutenUndLevelnPawn|GetShipMeshComponent _asbluten_und_leveln_pawn) self true)
      (bind _returnvalue (Rendering|Material|CreateDynamicMaterialInstance _projectilemesh 0 (Rendering|Material|GetMaterial _projectilemesh 0) :!class /Script/Engine.PrimitiveComponent))
      (bind _output_get (Variables|Default|SetProjectileMat _returnvalue))
      (bind _returnvalue_2 (Rendering|Material|GetScalarParameterValue _output_get "Brightness" :!class /Script/Engine.MaterialInstanceDynamic))
      (Variables|Default|SetBrightness _returnvalue_2)
      (Utilities|FlowControl|Delay (Variables|Default|GetLifetime))
      (CallFunction|Selfdestruct))
    (:Is%20Not%20Valid
      (Development|PrintText "!Projectile owner not assigned" true true "(R=1.000000,G=0.000000,B=0.000000,A=1.000000)" 4.0))))

(event EventActorBeginOverlap
  (params (OtherActor :type Actor%20Object%20Reference)))

(fn ConstructionScript)

(fn Launch
  (params (Velocity :type Vector) (Damage :type Float%20%28single-precision%29) (IsCritical :type Boolean))
  (Variables|/Script/Engine.MovementComponent|SetVelocity (Variables|Default|GetProjectileMovement) Velocity)
  (Variables|Default|SetProjectileDamage Damage)
  (Variables|Default|SetIsCritical IsCritical))

(fn ProjectileHit
  (params (HitActor :type Actor%20Object%20Reference))
  (bind _returnvalue (Game|Player|GetPlayerPawn 0))
  (bind _returnvalue_2 (Game|Player|GetPlayerPawn 0))
  (Utilities|Casting|CastToBP_BlutenUndLevelnPawn HitActor
    (:then
      ;[1 1 1] Hit Actor is Pawn
      (if (Math|Boolean|NotEqual(Boolean) (!= (Variables|Default|GetOwningActor) _returnvalue_2) (!= _returnvalue_2 HitActor))
        (LocalVariables|SetSuccessfulHit true)
        (bind _superficial (CallFunction|FindHitLocRot :!label _label))
        (CallFunction|DisplayHitFX _superficial HitActor)
        (Game|Damage|ApplyDamage HitActor (Variables|Default|GetProjectileDamage) (Game|GetInstigatorController) 0 (Variables|Default|GetDamageType))
        (if (and (LocalVariables|GetSuccessfulHit) (== (Variables|Default|GetOwningActor) (Game|Player|GetPlayerPawn 0)))
          (bind _asbp_bu_lplayer_controller (Utilities|Casting|CastToBP_BuLPlayerController (Game|GetPlayerController 0))
            (:then
              (Default|UpdateHits _asbp_bu_lplayer_controller (Variables|Default|GetOriginWeaponClass)))
            (:CastFailed
              _)))
        (Actor|DestroyActor)))
    (:CastFailed
      (bind _asbp_shield_slot_equipment_shield (Utilities|Casting|CastToBP_ShieldSlotEquipment_Shield HitActor)
        (:then
          ;[1 1 1] Hit Actor is Shield
          (if (Math|Boolean|NotEqual(Boolean) (== (Variables|Default|GetOwningActor) _returnvalue) (== _returnvalue (Variables|/Game/Blueprint/BP_ShieldSlotEquipment.BP_ShieldSlotEquipment_C|GetOwningActor _asbp_shield_slot_equipment_shield)))
            (LocalVariables|SetSuccessfulHit true)
            (goto _label)))
        (:CastFailed
          (goto _label))))))

(fn DisplayHitFX
  (params (Alternative :type Boolean) (HitActor :type Actor%20Object%20Reference))
  (bind _effectlocation (Variables|Default|GetEffectLocation))
  (bind _effectrotation (Variables|Default|GetEffectRotation))
  (Utilities|IsValid HitActor
    (:Is%20Valid
      (if (Actor|ActorHasTag HitActor "Rock")
        (Effects|SpawnEmitteratLocation (Variables|Default|GetHitFX_Rock) _effectlocation _effectrotation)
        (CallFunction|PlayHitSound (Variables|Default|GetImpactSoundRock))
        (else
          (if (Variables|Default|GetIsCritical)
            (Effects|SpawnEmitteratLocation (Variables|Default|GetHitFX_Critical) _effectlocation _effectrotation)
            (elif Alternative
              (Effects|SpawnEmitteratLocation (Variables|Default|GetHitFX_Alternative) _effectlocation _effectrotation)
              (else
                (Effects|SpawnEmitteratLocation (Variables|Default|GetHitFX_Standard) _effectlocation _effectrotation))))
          (CallFunction|PlayHitSound (Variables|Default|GetImpactSound)))))))

(fn FindAccurateHitResult
  (bind _projectilemesh (Variables|Default|GetProjectileMesh))
  (bind _returnvalue (Transformation|GetWorldLocation _projectilemesh))
  (bind (_outhit _returnvalue_2) (Collision|LineTraceByChannel _returnvalue (+ _returnvalue (* (Math|Vector|GetForwardVector _projectilemesh) 1e+02)) "TraceTypeQuery1" false 0 "None"))
  (return _outhit _returnvalue_2))

(fn FindHitLocRot
  (bind _projectilemesh (Variables|Default|GetProjectileMesh))
  (if (Variables|Default|GetGetAccurateHitResult) ; Whether to check for accurate Hit-Information
    (bind (_hitresult _hitfound) (CallFunction|FindAccurateHitResult))
    (if _hitfound ; Hit something?
      (bind _reflectedvector (Class|CVectorUtility|GetReflectionVector (Math|Vector|GetForwardVector (Variables|Default|GetProjectileMesh)) (.ImpactNormal (Collision|BreakHitResult _hitresult))))
      (Variables|Default|SetEffectLocation (.ImpactPoint (Collision|BreakHitResult _hitresult)))
      (Variables|Default|SetEffectRotation (Math|Conversions|RotationFromXVector (* _reflectedvector -1.0)))
      (else
        (Variables|Default|SetEffectLocation (Transformation|GetWorldLocation _projectilemesh) :!label _label)
        (Variables|Default|SetEffectRotation (Math|Conversions|RotationFromXVector (Math|Vector|GetForwardVector _projectilemesh)))))
    (else
      (goto _label)))
  (return (not _hitfound)))

(fn PlayHitSound
  (params (Sound :type Sound%20Cue%20Object%20Reference))
  (Utilities|IsValid Sound
    (:Is%20Valid
      (Audio|PlaySoundatLocation Sound (Transformation|GetWorldLocation (Variables|Default|GetProjectileMesh)) "0, 0, 0" 0.3))
    (:Is%20Not%20Valid
      (Audio|PlaySoundatLocation (Variables|Default|GetImpactSound) "0, 0, 0" "0, 0, 0" 0.3))))