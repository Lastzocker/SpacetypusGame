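; BP_Projectile_LightLaser is a light laser projectile that hits instantly using a line trace.
; Launch stores the damage and traces along the forward vector for world static, world dynamic, physics body and pawn objects.
; On a hit, it teleports to the impact point and passes the hit actor to ProjectileHit.
; The trace draws a one-frame debug line, and a miss triggers no further logic here.
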(event EventBeginPlay
  (|CallParentFunction))

(event EventActorBeginOverlap
  (params (OtherActor :type Actor%20Object%20Reference))
  (|CallParentFunction 0))

(event EventTick
  (params (DeltaSeconds :type Float%20%28single-precision%29)))

(event EventLaunch
  (params (Velocity :type Vector :default "0, 0, 0") (Damage :type Float%20%28single-precision%29) (IsCritical :type Boolean))
  (bind _returnvalue (Transformation|GetActorLocation))
  (Variables|Default|SetProjectileDamage Damage)
  (bind (_outhit _returnvalue_2) (Collision|LineTraceForObjects _returnvalue (+ _returnvalue (* (Transformation|GetActorForwardVector) (Variables|Default|GetTraceLength))) (Utilities|Array|MakeArray "ObjectTypeQuery1" "ObjectTypeQuery2" "ObjectTypeQuery4" "ObjectTypeQuery3") false 0 "ForOneFrame"))
  (if _returnvalue_2
    (Transformation|SetActorLocation (.Location (Collision|BreakHitResult _outhit)) false true)
    (CallFunction|ProjectileHit (.HitActor (Collision|BreakHitResult _outhit)))))

(fn ConstructionScript
  (|CallParentFunction))