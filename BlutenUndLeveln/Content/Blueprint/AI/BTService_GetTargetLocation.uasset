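; Behavior tree service that updates the AI's TargetLocation blackboard key and triggers the AI when its target comes near.
; Each tick writes either the target's location or, with predictive targeting, the pawn's targeting solution for weapon slot 0.
; Until triggered, a visible target within TriggerDistance fires the simple controller's damage reaction, or sets Triggered for other controllers.
; A gate opened on activation closes if an untriggered AI's target is dead, halting updates.
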(event EventTick
  (params (OwnerActor :type Actor%20Object%20Reference) (DeltaSeconds :type Float%20%28single-precision%29))
  (bind _aicontrollerref (Variables|Default|GetAIControllerRef))
  (bind _target (Variables|Default|GetTarget))
  (bind _targetlocation (Variables|Default|GetTargetLocation))
  (bind _returnvalue (AI|BehaviorTree|GetBlackboardValueasActor _target))
  (bind _returnvalue_2 (Pawn|GetControlledPawn _aicontrollerref))
  (bind _returnvalue_3 (Transformation|GetActorLocation _returnvalue))
  (Utilities|FlowControl|Gate true :!label _label
    (:Exit
      (if (Variables|Default|GetUsePredictiveTargeting)
        (bind _asbp_bluten_und_leveln_pawn (Utilities|Casting|CastToBP_BlutenUndLevelnPawn _returnvalue_2))
        (bind _predictedtargetrelativeposition (Default|GetTargetingSolutionPrecise _asbp_bluten_und_leveln_pawn _returnvalue))
        (AI|BehaviorTree|SetBlackboardValueasVector _targetlocation _predictedtargetrelativeposition)
        (else
          (AI|BehaviorTree|SetBlackboardValueasVector _targetlocation _returnvalue_3)))
      (if (not (Class|BTFunctionLibrary|GetBlackboardValueasBool (Variables|Default|GetTriggered)))
        (bind _asbp_bluten_und_leveln_pawn_2 (Utilities|Casting|CastToBP_BlutenUndLevelnPawn _returnvalue))
        (if (> (Variables|/Script/BlutenUndLeveln.BlutenUndLevelnPawn|GetHullIntegrity _asbp_bluten_und_leveln_pawn_2) 0.0) ; Stop doing stuff once the player is dead
          (if (and (not (Variables|/Script/Engine.SceneComponent|GetbHiddenInGame (Variables|/Script/BlutenUndLeveln.BlutenUndLevelnPawn|GetShipMeshComponent _asbp_bluten_und_leveln_pawn_2))) (<= (Math|Vector|VectorLength (- _returnvalue_3 (Transformation|GetActorLocation _returnvalue_2))) (Variables|Default|GetTriggerDistance)))
            (bind _asbp_aicontroller_simple (Utilities|Casting|CastToBP_AIController_Simple (Variables|Default|GetAIControllerRef))
              (:then
                (Default|TookDamageCopy _asbp_aicontroller_simple true 0.0 0.0))
              (:CastFailed
                (Class|BTFunctionLibrary|SetBlackboardValueasBool (Variables|Default|GetTriggered) true))))
          (else
            (goto _label Close)))))))

(event EventReceiveActivation
  (params (OwnerActor :type Actor%20Object%20Reference))
  (bind _target (Variables|Default|GetTarget))
  (bind _targetlocation (Variables|Default|GetTargetLocation))
  (bind _returnvalue (AI|BehaviorTree|GetBlackboardValueasActor _target))
  (bind _returnvalue_2 (Transformation|GetActorLocation _returnvalue))
  (bind _asaicontroller (Utilities|Casting|CastToAIController OwnerActor))
  (Variables|Default|SetAIControllerRef _asaicontroller)
  (Utilities|FlowControl|Gate true) ; enters at Open
)