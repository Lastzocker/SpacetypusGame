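; Behavior tree task that steers an AI-controlled BP_BlutenUndLevelnPawn to face the blackboard TargetVector location.
; Each tick it uses the cached AI controller and calls the pawn's Turn with a direction, skipping angles of five degrees or less.
; GetTurnDirection derives left or right from the cross product projected on the pawn's up vector, and the angle from the dot product's arccosine.
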(event EventTick
  (params (OwnerActor :type Actor%20Object%20Reference) (DeltaSeconds :type Float%20%28single-precision%29))
  (if (!= (Variables|Default|GetAIController) 0)
    _
    (else
      (bind _asaicontroller (Utilities|Casting|CastToAIController OwnerActor))
      (bind _output_get (Variables|Default|SetAIController _asaicontroller))))
  (bind (_direction _angle) (CallFunction|GetTurnDirection))
  (if (> _angle 5.0) ; Don't turn for minimal angles
    (bind _asbp_bluten_und_leveln_pawn (Utilities|Casting|CastToBP_BlutenUndLevelnPawn (Pawn|GetControlledPawn _output_get)))
    (Class|BlutenUndLevelnPawn|Turn _asbp_bluten_und_leveln_pawn _direction)))

(fn GetTurnDirection
  (bind _targetvector (Variables|Default|GetTargetVector))
  (bind _aicontroller (Variables|Default|GetAIController))
  (bind _returnvalue (Pawn|GetControlledPawn _aicontroller))
  (bind _returnvalue_2 (Class|BTFunctionLibrary|GetBlackboardValueasVector _targetvector))
  (bind _returnvalue_3 (Transformation|GetActorForwardVector _returnvalue))
  (bind _returnvalue_4 (Transformation|GetActorLocation _returnvalue))
  (bind _returnvalue_5 (Math|Vector|Normalize _returnvalue_3))
  (bind _returnvalue_6 (- _returnvalue_2 _returnvalue_4))
  (bind _returnvalue_7 (Math|Vector|Normalize _returnvalue_6))
  (bind _returnvalue_8 (Math|Vector|DotProduct _returnvalue_7 _returnvalue_5))
  (bind _returnvalue_9 (Class|KismetMathLibrary|DegAcos _returnvalue_8))
  (if (< (Math|Vector|DotProduct (Math|Vector|CrossProduct _returnvalue_7 _returnvalue_5) (Transformation|GetActorUpVector _returnvalue)) 0.0)
    (return 1.0 _returnvalue_9)
    (else
      (return -1.0 _returnvalue_9))))