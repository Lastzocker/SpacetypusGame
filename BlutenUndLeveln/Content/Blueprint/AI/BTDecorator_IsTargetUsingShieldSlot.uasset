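; Behavior tree decorator that checks whether the AI's target is using a shield slot with an active, working shield.
; It reads the Target blackboard actor and casts it to BP_BlutenUndLevelnPawn, failing if the cast fails.
; It passes only when a shield slot class comparison matches and the pawn's shield reports both Active and Functional.
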(fn PerformConditionCheck
  (params (OwnerActor :type Actor%20Object%20Reference))
  (bind _asbp_bluten_und_leveln_pawn (Utilities|Casting|CastToBP_BlutenUndLevelnPawn (AI|BehaviorTree|GetBlackboardValueasActor (Variables|Default|GetTarget)))
    (:then
      (return (Math|Boolean|ANDBoolean (== 0 (Variables|Default|GetShieldSlotClass)) (.Active (Default|GetIsShieldActive _asbp_bluten_und_leveln_pawn)) (.functional (Default|GetIsShieldActive _asbp_bluten_und_leveln_pawn)))))
    (:CastFailed
      (return false))))