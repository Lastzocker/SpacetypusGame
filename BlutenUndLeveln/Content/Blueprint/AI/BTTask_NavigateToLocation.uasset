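; Behavior tree task that steers the AI-controlled BP_BlutenUndLevelnPawn toward a blackboard target vector every tick, without navmesh pathfinding or finishing itself.
; Dot and cross products drive turning, skipping small angle differences.
; The target offset is split into forward and sideways inputs, scaled by the pawn's directional multipliers and normalized, with CheckDirection supplying signs.
; Line traces along each movement axis suppress that axis's input when blocked.
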(event EventTick
  (params (OwnerActor :type Actor%20Object%20Reference) (DeltaSeconds :type Float%20%28single-precision%29))
  (if (!= (Variables|Default|GetAIControllerRef) 0)
    _
    (else
      (bind _asbp_aicontroller_simple (Utilities|Casting|CastToBP_AIController_Simple OwnerActor))
      (bind _output_get (Variables|Default|SetAIControllerRef _asbp_aicontroller_simple))))
  (bind _asbp_bluten_und_leveln_pawn (Utilities|Casting|CastToBP_BlutenUndLevelnPawn (Pawn|GetControlledPawn _output_get)))
  (if (> (Class|KismetMathLibrary|DegAcos (Math|Vector|DotProduct (Math|Vector|Normalize (- (Class|BTFunctionLibrary|GetBlackboardValueasVector (Variables|Default|GetTargetVector)) (Transformation|GetActorLocation _asbp_bluten_und_leveln_pawn))) (Math|Vector|Normalize (Transformation|GetActorForwardVector _asbp_bluten_und_leveln_pawn)))) 5.0) ; Don't rotate for minimal angle differences
    (bind _newparam (CallFunction|GetTurnDirection))
    (Class|BlutenUndLevelnPawn|Turn _asbp_bluten_und_leveln_pawn _newparam))
  ;[1 1 1] Magic
  (bind _returnvalue (CallFunction|CheckDirection (Transformation|GetActorForwardVector _asbp_bluten_und_leveln_pawn)))
  (if (< _returnvalue 0.0)
    (Variables|Default|Setforwardfactor (* (* (Math|Vector|VectorLength (- (Class|BTFunctionLibrary|GetBlackboardValueasVector (Variables|Default|GetTargetVector)) (Transformation|GetActorLocation _asbp_bluten_und_leveln_pawn))) (Math|Vector|DotProduct (Math|Vector|Normalize (- (Class|BTFunctionLibrary|GetBlackboardValueasVector (Variables|Default|GetTargetVector)) (Transformation|GetActorLocation _asbp_bluten_und_leveln_pawn))) (Math|Vector|Normalize (Transformation|GetActorForwardVector _asbp_bluten_und_leveln_pawn)))) _returnvalue))
    (else
      (Variables|Default|Setforwardfactor (/ (* (* (Math|Vector|VectorLength (- (Class|BTFunctionLibrary|GetBlackboardValueasVector (Variables|Default|GetTargetVector)) (Transformation|GetActorLocation _asbp_bluten_und_leveln_pawn))) (Math|Vector|DotProduct (Math|Vector|Normalize (- (Class|BTFunctionLibrary|GetBlackboardValueasVector (Variables|Default|GetTargetVector)) (Transformation|GetActorLocation _asbp_bluten_und_leveln_pawn))) (Math|Vector|Normalize (Transformation|GetActorForwardVector _asbp_bluten_und_leveln_pawn)))) _returnvalue) (Variables|/Script/BlutenUndLeveln.BlutenUndLevelnPawn|GetBackwardsMultiplier _asbp_bluten_und_leveln_pawn)))))
  (bind _returnvalue_2 (CallFunction|CheckDirection (Transformation|GetActorRightVector _asbp_bluten_und_leveln_pawn)))
  (bind _output_get_2 (Variables|Default|Setsidefactor (/ (* _returnvalue_2 (* (Math|Vector|VectorLength (- (Class|BTFunctionLibrary|GetBlackboardValueasVector (Variables|Default|GetTargetVector)) (Transformation|GetActorLocation _asbp_bluten_und_leveln_pawn))) (Math|Trig|Sin(Degrees) (Class|KismetMathLibrary|DegAcos (Math|Vector|DotProduct (Math|Vector|Normalize (- (Class|BTFunctionLibrary|GetBlackboardValueasVector (Variables|Default|GetTargetVector)) (Transformation|GetActorLocation _asbp_bluten_und_leveln_pawn))) (Math|Vector|Normalize (Transformation|GetActorForwardVector _asbp_bluten_und_leveln_pawn))))))) (Variables|/Script/BlutenUndLeveln.BlutenUndLevelnPawn|GetSidewaysMultiplier _asbp_bluten_und_leveln_pawn))))
  (bind _output_get_3 (Variables|Default|Setmax (Math|Float|Max(Float) (Math|Float|Absolute(Float) _output_get_2) (Math|Float|Absolute(Float) (Variables|Default|Getforwardfactor)))))
  (Variables|Default|Setforwardfactor (* _returnvalue (Math|Float|NormalizetoRange (Variables|Default|Getforwardfactor) 0.0 _output_get_3)))
  (Variables|Default|Setsidefactor (Math|Float|NormalizetoRange (Variables|Default|Getsidefactor) 0.0 _output_get_3))
  (bind _returnvalue_3 (Collision|LineTraceForObjects (Transformation|GetActorLocation _asbp_bluten_und_leveln_pawn) (+ (Transformation|GetActorLocation _asbp_bluten_und_leveln_pawn) (* (Transformation|GetActorForwardVector _asbp_bluten_und_leveln_pawn) (* (Variables|Default|GetTraceLength) (Math|Float|Sign(Float) (Variables|Default|Getforwardfactor))))) (Utilities|Array|MakeArray "ObjectTypeQuery1" "ObjectTypeQuery4" "ObjectTypeQuery3") false (Utilities|Array|MakeArray _asbp_bluten_und_leveln_pawn) "None"))
  (if _returnvalue_3
    _
    (else
      (Class|BlutenUndLevelnPawn|MoveForward _asbp_bluten_und_leveln_pawn (Variables|Default|Getforwardfactor))))
  (bind _returnvalue_4 (Collision|LineTraceForObjects (Transformation|GetActorLocation _asbp_bluten_und_leveln_pawn) (+ (Transformation|GetActorLocation _asbp_bluten_und_leveln_pawn) (* (Transformation|GetActorRightVector _asbp_bluten_und_leveln_pawn) (* (Variables|Default|GetTraceLength) (Math|Float|Sign(Float) (Variables|Default|Getsidefactor))))) (Utilities|Array|MakeArray "ObjectTypeQuery1" "ObjectTypeQuery4" "ObjectTypeQuery3") false (Utilities|Array|MakeArray _asbp_bluten_und_leveln_pawn) "None"))
  (if (not _returnvalue_4)
    (Class|BlutenUndLevelnPawn|MoveRight _asbp_bluten_und_leveln_pawn (Variables|Default|Getsidefactor))))

(fn CheckDirection
  (params (Direction :type Vector))
  (bind _targetvector (Variables|Default|GetTargetVector))
  (bind _aicontrollerref (Variables|Default|GetAIControllerRef))
  (bind _returnvalue (Pawn|GetControlledPawn _aicontrollerref))
  (bind _returnvalue_2 (Class|BTFunctionLibrary|GetBlackboardValueasVector _targetvector))
  (bind _returnvalue_3 (Transformation|GetActorLocation _returnvalue))
  (return (Math|Float|Sign(Float) (- (Math|Vector|VectorLength (- _returnvalue_2 _returnvalue_3)) (Math|Vector|VectorLength (- _returnvalue_2 (+ _returnvalue_3 Direction)))))))

(fn GetTurnDirection
  (bind _aicontrollerref (Variables|Default|GetAIControllerRef))
  (bind _returnvalue (Pawn|GetControlledPawn _aicontrollerref))
  (if (< (Math|Vector|DotProduct (Math|Vector|CrossProduct (Math|Vector|Normalize (- (Class|BTFunctionLibrary|GetBlackboardValueasVector (Variables|Default|GetTargetVector)) (Transformation|GetActorLocation _returnvalue))) (Math|Vector|Normalize (Transformation|GetActorForwardVector _returnvalue))) (Transformation|GetActorUpVector _returnvalue)) 0.0)
    (return 1.0)
    (else
      (return -1.0))))