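; Behavior tree decorator that passes when the AI's controlled pawn is closer to a target location than an acceptable distance.
; It compares the length of the vector between the pawn and the TargetLocation blackboard value against AcceptableDistance.
; The AI controller is cast from the owner actor and cached on first use, and the check fails if that cast fails.
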(fn PerformConditionCheck
  (params (OwnerActor :type Actor%20Object%20Reference))
  (if (not (== (Variables|Default|GetAIController) 0))
    _
    (else
      (bind _asaicontroller (Utilities|Casting|CastToAIController OwnerActor)
        (:then
          (bind _output_get (Variables|Default|SetAIController _asaicontroller)))
        (:CastFailed
          (return false)))))
  (return (< (Math|Vector|VectorLength (- (Transformation|GetActorLocation (Pawn|GetControlledPawn _output_get)) (Class|BTFunctionLibrary|GetBlackboardValueasVector (Variables|Default|GetTargetLocation)))) (Variables|Default|GetAcceptableDistance))))