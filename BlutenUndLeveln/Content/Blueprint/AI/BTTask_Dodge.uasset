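; Behavior tree task that makes an AI-controlled BlutenUndLeveln pawn dodge in reaction to nearby hits on its blackboard Target.
; Each tick, it sphere-traces WorldStatic objects around the pawn, overwriting the stored location per matching hit and dividing it by a never-reset hit count.
; GetDodgeDirection derives forward/right components from that point, signed by CheckDirection's distance comparison.
; The pawn dodges along the weaker axis, if that dodge is available.
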(event EventTick
  (params (OwnerActor :type Actor%20Object%20Reference) (DeltaSeconds :type Float%20%28single-precision%29))
  (if (== (Variables|Default|GetAIC) 0)
    (bind _asaicontroller (Utilities|Casting|CastToAIController OwnerActor))
    (bind _output_get (Variables|Default|SetAIC _asaicontroller)))
  (bind (_outhits _returnvalue) (Collision|MultiSphereTraceForObjects (Transformation|GetActorLocation (Pawn|GetControlledPawn _output_get)) (Transformation|GetActorLocation (Pawn|GetControlledPawn _output_get)) (Variables|Default|GetCheckRadius) (Utilities|Array|MakeArray "ObjectTypeQuery1") false 0 "None"))
  (if _returnvalue
    (for _array_element _outhits
      (if (== (.HitActor (Collision|BreakHitResult _array_element)) (AI|BehaviorTree|GetBlackboardValueasActor (Variables|Default|GetTarget)))
        (Variables|Default|SetTotalHitLocations (Math|Conversions|ToVector2D(Vector) (+ (.Location (Collision|BreakHitResult _array_element)) (- (.Location (Collision|BreakHitResult _array_element)) (Transformation|GetActorLocation (Pawn|GetControlledPawn _output_get))))))
        (Math|Integer|IncrementInt (Variables|Default|GetNumHits))))
    (bind _asbp_bluten_und_leveln_pawn (Utilities|Casting|CastToBP_BlutenUndLevelnPawn (Pawn|GetControlledPawn _output_get)))
    (bind _output_get_2 (Variables|Default|SetForward (.Forward (CallFunction|GetDodgeDirection _asbp_bluten_und_leveln_pawn))))
    (bind _output_get_3 (Variables|Default|SetRight (.Right (CallFunction|GetDodgeDirection _asbp_bluten_und_leveln_pawn))))
    (if (> (Math|Float|Absolute(Float) _output_get_3) (Math|Float|Absolute(Float) _output_get_2)) ; dodge forward/back if projectiles in that direction are closer and vice versa
      (if (Variables|/Game/Blueprint/BP_BlutenUndLevelnPawn.BP_BlutenUndLevelnPawn_C|GetCanDodgeForward _asbp_bluten_und_leveln_pawn)
        (Default|DodgeForward _asbp_bluten_und_leveln_pawn (Math|Float|Sign(Float) (Variables|Default|GetForward))))
      (elif (Variables|/Game/Blueprint/BP_BlutenUndLevelnPawn.BP_BlutenUndLevelnPawn_C|GetCanDodgeRight _asbp_bluten_und_leveln_pawn)
        (Default|DodgeRight _asbp_bluten_und_leveln_pawn (Math|Float|Sign(Float) (Variables|Default|GetRight)))))))

(fn GetDodgeDirection
  (params (Actor :type Actor%20Object%20Reference))
  (bind _returnvalue (Transformation|GetActorForwardVector Actor))
  (bind _totalhitlocations (Variables|Default|GetTotalHitLocations))
  (bind _numhits (Variables|Default|GetNumHits))
  (bind _returnvalue_2 (Math|Conversions|ToFloat(Integer) _numhits))
  (bind _returnvalue_3 (Math|Vector|Normalize _returnvalue))
  (bind _returnvalue_4 (/ _totalhitlocations _returnvalue_2))
  (bind _returnvalue_5 (Math|Conversions|ToVector(Vector2D) _returnvalue_4))
  (bind _returnvalue_6 (Math|Vector|VectorLength _returnvalue_5))
  (bind _returnvalue_7 (Math|Vector|Normalize _returnvalue_5))
  (bind _returnvalue_8 (Math|Vector|DotProduct _returnvalue_7 _returnvalue_3))
  (return (* (* _returnvalue_6 _returnvalue_8) (CallFunction|CheckDirection _returnvalue _returnvalue_5)) (* (* _returnvalue_6 (Math|Trig|Sin(Degrees) (Class|KismetMathLibrary|DegAcos _returnvalue_8))) (CallFunction|CheckDirection (Transformation|GetActorRightVector Actor) _returnvalue_5))))

(fn CheckDirection
  (params (Direction :type Vector) (TargetAbsLocation :type Vector))
  (bind _aic (Variables|Default|GetAIC))
  (bind _returnvalue (Pawn|GetControlledPawn _aic))
  (bind _returnvalue_2 (Transformation|GetActorLocation _returnvalue))
  (return (Math|Float|Sign(Float) (- (Math|Vector|VectorLength (- TargetAbsLocation _returnvalue_2)) (Math|Vector|VectorLength (- TargetAbsLocation (+ _returnvalue_2 Direction)))))))