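; Behavior tree task that makes an AI-controlled BP_BlutenUndLevelnPawn fire its weapon in timed bursts.
; Tick alternates between a shoot window and a wait window, releasing the fire button when shooting ends.
; During the shoot window it fires weapon array 0 only while facing the blackboard TargetVector within a small angle and a line trace, ignoring itself and Target, finds no obstruction.
; The graph never finishes the task itself.
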(event EventTick
  (params (OwnerActor :type Actor%20Object%20Reference) (DeltaSeconds :type Float%20%28single-precision%29))
  (if (Variables|Default|GetCanShoot)
    (if (< (Variables|Default|GetTime) (Variables|Default|GetShootTime))
      (if (== (Variables|Default|GetAIC) 0)
        (bind _asaicontroller (Utilities|Casting|CastToAIController OwnerActor))
        (bind _output_get (Variables|Default|SetAIC _asaicontroller)))
      (bind _asbp_bluten_und_leveln_pawn (Utilities|Casting|CastToBP_BlutenUndLevelnPawn (Pawn|GetControlledPawn _output_get)))
      (bind _returnvalue (Collision|LineTraceForObjects (Transformation|GetActorLocation _asbp_bluten_und_leveln_pawn) (Class|BTFunctionLibrary|GetBlackboardValueasVector (Variables|Default|GetTargetVector)) (Utilities|Array|MakeArray "ObjectTypeQuery1" "ObjectTypeQuery4" "ObjectTypeQuery3") false (Utilities|Array|MakeArray (Pawn|GetControlledPawn (Variables|Default|GetAIC)) (AI|BehaviorTree|GetBlackboardValueasActor (Variables|Default|GetTarget))) "ForDuration"))
      (if (and (<= (Class|KismetMathLibrary|DegAcos (Math|Vector|DotProduct (Math|Vector|Normalize (- (Class|BTFunctionLibrary|GetBlackboardValueasVector (Variables|Default|GetTargetVector)) (Transformation|GetActorLocation (Pawn|GetControlledPawn _output_get)))) (Math|Vector|Normalize (Transformation|GetActorForwardVector (Pawn|GetControlledPawn _output_get))))) 5.0) (not _returnvalue)) ; Don't rotate for minimal angle differences
        (Default|FireWeaponArray _asbp_bluten_und_leveln_pawn))
      (Variables|Default|SetTime (+ (Variables|Default|GetTime) DeltaSeconds))
      (else
        (Default|ReleaseFireButton _asbp_bluten_und_leveln_pawn)
        (Variables|Default|SetTime 0.0 :!label _label)
        (Variables|Default|SetCanShoot (not (Variables|Default|GetCanShoot)))))
    (elif (< (Variables|Default|GetTime) (Variables|Default|GetWaitTime))
      (Variables|Default|SetTime (+ (Variables|Default|GetTime) DeltaSeconds))
      (else
        (goto _label)))))