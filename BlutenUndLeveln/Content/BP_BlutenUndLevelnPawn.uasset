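; Pawn that serves as a test bed for lead-target aiming, with a gameplay HUD and minimap.
; Each tick it computes a precise or iterative intercept for TargetActor, draws it as debug lines and places the target's minimap marker.
; The HUD border icon is pinned at zero, ignoring the screen-border projection, and marker range hiding is unwired.
; AltFire launches a test projectile with random spread plus the pawn's velocity.
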(event EventBeginPlay
  (bind _returnvalue (UserInterface|CreateWidget "/Game/HUD/GameplayHUD.GameplayHUD_C"))
  (Variables|Default|SetHUD _returnvalue)
  (UserInterface|Viewport|AddtoViewport _returnvalue 0)
  (bind _returnvalue_2 (UserInterface|CreateWidget "/Game/HUD/Minimap.Minimap_C"))
  (bind _output_get (Variables|Default|SetMinimap _returnvalue_2))
  (UserInterface|Viewport|AddtoViewport _output_get 0)
  (bind _returnvalue_3 (UserInterface|CreateWidget "/Game/HUD/MinimapMarker.MinimapMarker_C"))
  (bind _output_get_2 (Variables|Default|SetMinimapMarker _returnvalue_3))
  (UserInterface|Viewport|AddtoViewport _output_get_2 0))

(event EventTick
  (params (DeltaSeconds :type Float%20%28single-precision%29))
  (bind _returnvalue (Game|GetPlayerController 0))
  (bind _targetactor (Variables|Default|GetTargetActor))
  (bind (_sizex _sizey) (HUD|GetViewportSize _returnvalue))
  (|CallParentFunction DeltaSeconds)
  (Rendering|Debug|DrawDebugSphere (+ (Transformation|GetActorLocation) (* (Transformation|GetActorForwardVector) 3e+02)) 1e+01 12 "(R=1.000000,G=0.000000,B=0.000000,A=1.000000)" 0.0)
  (Utilities|IsValid (Variables|Default|GetTargetActor)
    (:Is%20Valid
      (Utilities|FlowControl|Sequence
        (:then_0
          ;[1 1 1] Targeting
          (if (Variables|Targeting|GetUseIterativeTargeting)
            (bind (_predictedaimvector _predictedtargetrelativeposition _timetotarget) (CallFunction|GetTargetingSolutionIterative _targetactor 1))
            (CallFunction|DebugDisplayTargetingSolution _targetactor _predictedaimvector _predictedtargetrelativeposition _timetotarget)
            (else
              (bind (_predictedaimvector_2 _predictedtargetrelativeposition_2 _timetotarget_2) (CallFunction|GetTargetingSolutionPrecise _targetactor))
              (CallFunction|DebugDisplayTargetingSolution _targetactor _predictedaimvector_2 _predictedtargetrelativeposition_2 _timetotarget_2))))
        (:then_1
          ;[1 1 1] TargetBorderIcon
          (Class|CVectorUtility|ProjecttoScreenBorder (Transformation|GetActorLocation) (Transformation|GetActorLocation (Variables|Default|GetTargetActor)) (Game|GetPlayerController 0))
          (Default|SetIconPosition (Variables|Default|GetHUD)))
        (:then_2
          (bind (_mapposition _inrange) (Class|CVectorUtility|ConverttoMapSpace (Transformation|GetActorLocation (Variables|Default|GetTargetActor)) (Transformation|GetActorLocation) (- (Math|Vector2D|MakeVector2D (Math|Conversions|ToFloat(Integer) _sizex) (Math|Conversions|ToFloat(Integer) _sizey)) "(X=150.000000,Y=150.000000)") (+ 0.0 128.0) (+ 0.0 2e+01) _returnvalue))
          (Class|UserWidget|SetPositioninViewport (Variables|Default|GetMinimapMarker) _mapposition true))))))

(fn ConstructionScript)

(fn GetTargetingSolutionPrecise
  (params (TargetActor :type Actor%20Object%20Reference))
  (bind (_predictedaimvector _predictedtargetrelativeposition _timetotarget) (Class|CVectorUtility|GetAimDirectionPrecise (Transformation|GetActorLocation) (Transformation|GetActorLocation TargetActor) (- (Transformation|GetVelocity TargetActor) (Transformation|GetVelocity)) (Variables|Default|GetProjectileSpeed)))
  (return _predictedaimvector _predictedtargetrelativeposition _timetotarget))

(fn DebugDisplayTargetingSolution
  (params (TargetActor :type Actor%20Object%20Reference) (PredictedAimVector :type Vector) (PredictedTargetRelativePosition :type Vector) (TimeToTarget :type Float%20%28single-precision%29))
  (bind _returnvalue (Transformation|GetActorLocation TargetActor))
  (bind _returnvalue_2 (Transformation|GetActorLocation))
  (if (Math|Vector|NotEqual(Vector) PredictedAimVector "0, 0, 0" 0.0001)
    (bind _radialoffsetvector (Class|CVectorUtility|GetTargetRadialOffsetVector PredictedAimVector (Transformation|GetActorLocation) _returnvalue))
    (Rendering|Debug|DrawDebugLine _returnvalue_2 (+ _returnvalue_2 (* PredictedAimVector (* TimeToTarget (Variables|Default|GetProjectileSpeed)))) "(R=0.085000,G=0.000000,B=0.000000,A=0.300000)" 0.0 9.0)
    (Rendering|Debug|DrawDebugLine _returnvalue_2 (+ _returnvalue_2 (* PredictedAimVector 1e+02)) "(R=1.000000,G=0.000000,B=0.000000,A=1.000000)" 0.0 1e+01)
    (Rendering|Debug|DrawDebugLine _returnvalue PredictedTargetRelativePosition "(R=1.000000,G=0.411957,B=0.000000,A=1.000000)" 0.0 1e+01)
    (Rendering|Debug|DrawDebugLine _returnvalue _radialoffsetvector "(R=1.000000,G=0.707986,B=0.000000,A=1.000000)" 0.0 1e+01)
    (Development|PrintString (Utilities|String|BuildString(Float) "" "Time to target: " TimeToTarget "s") true true "(R=0.000000,G=0.660000,B=1.000000,A=1.000000)" 0.0)
    (else
      (Development|PrintString "No valid solution" true true "(R=0.000000,G=0.660000,B=1.000000,A=1.000000)" 0.0))))

(fn GetTargetingSolutionIterative
  (params (TargetActor :type Actor%20Object%20Reference) (Iterations :type Integer))
  (bind _projectiletimetotarget (Variables|Default|GetProjectileTimeToTarget))
  (bind (_predictedaimvector _predictedtargetrelativeposition) (Class|CVectorUtility|GetAimDirectionIterative (Transformation|GetActorLocation) (Transformation|GetActorLocation TargetActor) (- (Transformation|GetVelocity) (Transformation|GetVelocity)) (+ "0, 0, 0" "0, 0, 0") (Variables|Default|GetProjectileSpeed) Iterations _projectiletimetotarget))
  (return _predictedaimvector _predictedtargetrelativeposition _projectiletimetotarget))

(fn TestLineIntersection
  (bind _a1 (LocalVariables|Geta1))
  (bind _a2 (LocalVariables|Geta2))
  (bind _b1 (LocalVariables|Getb1))
  (bind _b2 (LocalVariables|Getb2))
  (bind _intersectionpoint (Class|CVectorUtility|LineLineIntersection _a1 _a2 _b1 _b2))
  (Rendering|Debug|DrawDebugLine (Math|Conversions|ToVector(Vector2D) _a1) (Math|Conversions|ToVector(Vector2D) _a2) "(R=1.000000,G=0.000000,B=0.000000,A=1.000000)" 0.0 5.0)
  (Rendering|Debug|DrawDebugLine (Math|Conversions|ToVector(Vector2D) _b1) (Math|Conversions|ToVector(Vector2D) _b2) "(R=1.000000,G=0.000000,B=0.000000,A=1.000000)" 0.0 5.0)
  (Rendering|Debug|DrawDebugPoint (Math|Conversions|ToVector(Vector2D) _intersectionpoint) 1e+01 "(R=1.000000,G=0.000000,B=0.000000,A=1.000000)" 0.0))

(fn AltFire
  (bind _returnvalue (Game|SpawnActorfromClass "/Game/BP_Projectile_Test.BP_Projectile_Test_C" (Transformation|GetWorldTransform (Variables|Default|GetScene)) "Undefined" 0 self))
  (Default|Launch _returnvalue (+ (Transformation|GetVelocity) (* (+ (Transformation|GetActorForwardVector) (* (Math|Random|RandomUnitVector) 0.03)) 1.55e+03)))
  (return))